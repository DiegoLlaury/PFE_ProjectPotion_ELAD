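; Interactable bed actor that advances the game to the next night once the current one is finished.
; On BeginPlay it caches BP_GameInstance, then either clears NewGame and requests the current night's NPC or, on later loads, resets NightFinished.
; Interacting while NightFinished is set increases CurrentNight in steps of 100, requests that night's NPC and opens a level by object reference.
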(event EventBeginPlay
  (bind _asbp_game_instance (Utilities|Casting|CastToBP_GameInstance (Game|GetGameInstance)))
  (bind _output_get (Variables|Default|SetAs%20BP%20Game%20Instance _asbp_game_instance))
  (if (Variables|/Game/Blueprints/Managers/BP_GameInstance.BP_GameInstance_C|GetNewGame? _output_get)
    (Variables|/Game/Blueprints/Managers/BP_GameInstance.BP_GameInstance_C|SetNewGame? _output_get false)
    (Default|GetNPCforNight (Variables|Default|GetAs%20BP%20Game%20Instance) (Variables|/Game/Blueprints/Managers/BP_GameInstance.BP_GameInstance_C|GetCurrentNight (Variables|Default|GetAs%20BP%20Game%20Instance)))
    (else
      (Variables|/Game/Blueprints/Managers/BP_GameInstance.BP_GameInstance_C|SetNightFinished (Variables|Default|GetAs%20BP%20Game%20Instance) false))))

(event Collision|EventActorBeginOverlap
  (params (OtherActor :type Actor%20Object%20Reference)))

(event EventTick
  (params (DeltaSeconds :type Float%20%28single-precision%29)))

(event EventOnInteract
  (params (ItemSlots :type Array%20of%20S%20Item%20Slot%20Structures))
  (bind _as_bp_game_instance (Variables|Default|GetAs%20BP%20Game%20Instance))
  (if (Variables|/Game/Blueprints/Managers/BP_GameInstance.BP_GameInstance_C|GetNightFinished _as_bp_game_instance)
    (bind _output_get (Variables|/Game/Blueprints/Managers/BP_GameInstance.BP_GameInstance_C|SetCurrentNight _as_bp_game_instance (+ (Variables|/Game/Blueprints/Managers/BP_GameInstance.BP_GameInstance_C|GetCurrentNight _as_bp_game_instance) 100)))
    (Default|GetNPCforNight _as_bp_game_instance _output_get)
    (Game|OpenLevel(byObjectReference) (Variables|Default|GetLevel))))

(fn ConstructionScript)

(fn FocusTarget
  (return ""))