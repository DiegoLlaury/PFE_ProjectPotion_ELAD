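; Cauldron actor for potion crafting that matches held ingredients against recipes in DT_Recipes.
; On BeginPlay it binds to the player's LaunchCauldron dispatcher, which scans recipe rows using CompareMap for identical ingredients and counts.
; A match clears the temporary ingredient map and only prints the resulting potion ID.
; AddIngredientTemp tallies ingredients into that map, but its checks and input are unwired placeholders.
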(event Custom|LaunchCauldron
  ;[0.15 0.15 0.15 0.5] Système de craft de potion
  (bind _outrownames (DataTable|GetDataTableRowNames (Variables|Default|GetDT_Recipes)))
  (bind _array_element (Utilities|Array|ForEachLoopwithBreak _outrownames :!label _label)
    (:LoopBody
      (bind _returnvalue (Utilities|GetDataTableRow "/Game/Data/Datatables/DT_Recipes.DT_Recipes" _array_element)
        (:then
          (if (CallFunction|CompareMap (Variables|Default|GetTempProperty) (.ingredients _returnvalue))
            (Utilities|Map|Clear (Variables|Default|GetTempProperty))
            (Development|PrintString (Utilities|String|ToString(Name) (.idresultingpotion _returnvalue)))
            (goto _label Break)))))))

(event EventBeginPlay
  (bind _asbp_player (Utilities|Casting|CastToBP_Player (Game|Player|GetPlayerPawn 0)))
  (Variables|Default|SetAs%20BP%20Player _asbp_player)
  (EventDispatchers|BindEventtoLaunchCauldron (Variables|Default|GetAs%20BP%20Player) (EventDispatchers|CreateEvent :!event Custom|LaunchCauldron)))

(fn ConstructionScript)

(fn AddIngredientTemp
  (if true
    (if true
      (for _array_element (Utilities|Array|MakeArray "")
        (if (Utilities|Map|Contains (Variables|Default|GetTempProperty) _array_element)
          (bind _result (Math|Integer|IncrementInt (.Value (Utilities|Map|Find (Variables|Default|GetTempProperty) _array_element)))
            (:%20%20
              (Utilities|Map|Add (Variables|Default|GetTempProperty) _array_element _result)))
          (else
            (Utilities|Map|Add (Variables|Default|GetTempProperty) _array_element 1))))
      (bind _output_get (Variables|Default|SetTempProperty (Variables|Default|GetTempProperty)))
      (bind _keys (Utilities|Map|Keys _output_get))
      (for _array_element_2 _keys
        (Development|PrintString _array_element_2))
      (else
        (Development|PrintString "Impossibe ingredient brute")))
    (else
      (Development|PrintString "No Ingredient in inventory"))))

(fn CompareMap
  (params (MapA_Ingredient :type Map%20of%20Strings%20to%20Integers) (MapB_Recipe :type Map%20of%20Strings%20to%20Integers))
  (if (== (Utilities|Map|Length MapA_Ingredient) (Utilities|Map|Length MapB_Recipe))
    (bind _keys (Utilities|Map|Keys MapA_Ingredient))
    (for _array_element _keys
      (if (Utilities|Map|Contains MapB_Recipe _array_element)
        (if (== (.Value (Utilities|Map|Find MapA_Ingredient _array_element)) (.Value (Utilities|Map|Find MapB_Recipe _array_element)))
          (Variables|Default|SetIs%20Matching true)
          (else
            (return false)))
        (else
          (return false))))
    (return true)
    (else
      (return false))))

(fn FocusTarget
  (return ""))