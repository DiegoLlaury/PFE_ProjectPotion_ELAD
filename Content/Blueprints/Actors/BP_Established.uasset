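; Possessable alchemy workbench that turns inventory ingredients into processed items or potions, according to its Method: Cut, Grind or Cauldron.
; Interacting possesses the bench and opens the inventory; the escape input repossesses the player.
; Cut and Grind swap an ingredient for its processed item.
; Cauldron tallies ingredient properties in a map, then, on launch, grants the potion whose DT_Recipes entry matches those counts exactly.
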(event Custom|LaunchCauldron
  ;[0.15 0.15 0.15 0.5] Système de craft de potion
  (if (Utilities|Map|IsNotEmpty (Variables|Default|GetTempProperty))
    (bind _outrownames (DataTable|GetDataTableRowNames (Variables|References|GetDT_Recipes)))
    (bind _array_element (Utilities|Array|ForEachLoopwithBreak _outrownames :!label _label)
      (:LoopBody
        (bind _returnvalue (Utilities|GetDataTableRow "/Game/Data/Datatables/DT_Recipes.DT_Recipes" _array_element)
          (:then
            (if (CallFunction|CompareMap (Variables|Default|GetTempProperty) (.ingredients _returnvalue))
              (Utilities|Map|Clear (Variables|Default|GetTempProperty))
              (Default|Pickup (Variables|/Game/Blueprints/Managers/BP_GameController.BP_GameController_C|GetBPC_Inventory (Variables|References|GetAs%20BP%20My%20Controller)) (.idresultingpotion _returnvalue) 1)
              (goto _label Break))))))
    (else
      (Development|PrintString "No ingredient"))))

(event Custom|ProcessIngredient
  (params (IngredientData :type S%20Ingredient%20Structure) (Index :type Integer))
  (switch Utilities|FlowControl|Switch|SwitchonEProcessingMethod (Variables|Default|GetMethod)
    (:NewEnumerator0
      (CallFunction|ProcessIngredients IngredientData (Variables|Default|GetMethod) Index :!label _label))
    (:NewEnumerator1
      (goto _label))
    (:NewEnumerator2
      (CallFunction|AddIngredientTemp IngredientData Index))))

(event Input|EnhancedActionEvents|EnhancedInputActionIA_EscapeWorkbench
  (params (ActionValue :type Boolean) (ElapsedSeconds :type Float%20%28double-precision%29) (TriggeredSeconds :type Float%20%28double-precision%29) (InputAction :type Input%20Action%20Object%20Reference :default "/Game/FirstPerson/Input/Actions/IA_EscapeWorkbench.IA_EscapeWorkbench"))
  (bind _as_bp_my_controller (Variables|References|GetAs%20BP%20My%20Controller))
  ;[0.15 0.15 0.15 0.5] Fais sortir le joueur de l'établis, et lui fais reprendre le controle de son personnage
  (Variables|/Script/Engine.PlayerController|SetbShowMouseCursor (Variables|References|GetAs%20BP%20My%20Controller) false)
  (EventDispatchers|UnbindEventfromOnUseItem (Variables|/Game/Blueprints/Managers/BP_GameController.BP_GameController_C|GetBPC_Inventory (Variables|References|GetAs%20BP%20My%20Controller)) (EventDispatchers|CreateEvent :!event Custom|ProcessIngredient))
  (Default|RemoveHUD (Variables|/Game/Widgets/HUD/HUDPlayer/WBP_PlayerHUD.WBP_PlayerHUD_C|GetWB_PlayerDisplay (Variables|/Game/Blueprints/Managers/BP_GameController.BP_GameController_C|GetWB_PlayerHUD _as_bp_my_controller)))
  (Utilities|FlowControl|Delay 0.3)
  (Variables|/Game/Blueprints/Managers/BP_GameController.BP_GameController_C|SetIsOnWorkbench _as_bp_my_controller false)
  (switch Utilities|FlowControl|Switch|SwitchonEProcessingMethod (Variables|Default|GetMethod)
    (:NewEnumerator0
      _)
    (:NewEnumerator1
      _)
    (:NewEnumerator2
      (Widget|RemovefromParent (Variables|References|GetWidgetCauldron))))
  (Pawn|Possess (Variables|References|GetAs%20BP%20My%20Controller) (Variables|References|GetAs%20BP%20Player)))

(event EventBeginPlay
  (bind _asbp_player (Utilities|Casting|CastToBP_Player (Game|Player|GetPlayerPawn 0)))
  (Variables|References|SetAs%20BP%20Player _asbp_player)
  (bind _asbp_game_controller (Utilities|Casting|CastToBP_GameController (Game|GetPlayerController 0)))
  (Variables|References|SetAs%20BP%20My%20Controller _asbp_game_controller))

(fn ConstructionScript)

(fn ProcessIngredients
  (params (InIngredient :type S%20Ingredient%20Structure) (Method :type EProcessingMethod%20Enum :default "NewEnumerator0") (Index :type Integer))
  (bind (_name _propertycut _propertygrind _id _finalproperty _mesh _texture _category) (Utilities|Struct|BreakSIngredient InIngredient))
  (bind _as_bp_my_controller (Variables|References|GetAs%20BP%20My%20Controller))
  (bind _as_bp_my_controller_2 (Variables|References|GetAs%20BP%20My%20Controller))
  (bind _bpc_inventory (Variables|/Game/Blueprints/Managers/BP_GameController.BP_GameController_C|GetBPC_Inventory _as_bp_my_controller))
  (bind _bpc_inventory_2 (Variables|/Game/Blueprints/Managers/BP_GameController.BP_GameController_C|GetBPC_Inventory _as_bp_my_controller_2))
  (if (Utilities|Enum|Equal(Enum) _category "NewEnumerator0")
    (switch Utilities|FlowControl|Switch|SwitchonEProcessingMethod Method
      (:NewEnumerator0
        (Default|RemoveItemUsed _bpc_inventory Index)
        (Default|Pickup _bpc_inventory_2 (Utilities|String|StringToName _propertycut) 1))
      (:NewEnumerator1
        (Default|RemoveItemUsed _bpc_inventory Index)
        (Default|Pickup _bpc_inventory_2 (Utilities|String|StringToName _propertygrind) 1)))))

(fn CompareMap
  (params (MapA_Ingredient :type Map%20of%20Strings%20to%20Integers) (MapB_Recipe :type Map%20of%20Strings%20to%20Integers))
  (if (== (Utilities|Map|Length MapA_Ingredient) (Utilities|Map|Length MapB_Recipe))
    (bind _keys (Utilities|Map|Keys MapA_Ingredient))
    (for _array_element _keys
      (if (Utilities|Map|Contains MapB_Recipe _array_element)
        (if (== (.Value (Utilities|Map|Find MapA_Ingredient _array_element)) (.Value (Utilities|Map|Find MapB_Recipe _array_element)))
          (Variables|Default|SetIs%20Matching true)
          (else
            (return false)))
        (else
          (return false))))
    (return true)
    (else
      (return false))))

(fn AddIngredientTemp
  (params (IngredientIn :type S%20Ingredient%20Structure) (Index :type Integer))
  (bind (_name _propertycut _propertygrind _id _finalproperty _mesh _texture _category) (Utilities|Struct|BreakSIngredient IngredientIn))
  (Development|PrintString "Hello")
  (if (Utilities|Enum|Equal(Enum) _category "NewEnumerator1")
    (for _array_element (Utilities|Array|MakeArray (Utilities|String|EnumtoString _finalproperty))
      (if (Utilities|Map|Contains (Variables|Default|GetTempProperty) _array_element)
        (bind _result (Math|Integer|IncrementInt (.Value (Utilities|Map|Find (Variables|Default|GetTempProperty) _array_element)))
          (:%20%20
            (Utilities|Map|Add (Variables|Default|GetTempProperty) _array_element _result)))
        (else
          (Utilities|Map|Add (Variables|Default|GetTempProperty) _array_element 1))))
    (bind _output_get (Variables|Default|SetTempProperty (Variables|Default|GetTempProperty)))
    (bind _keys (Utilities|Map|Keys _output_get))
    (for _array_element_2 _keys
      _)
    (Default|RemoveItemUsed (Variables|/Game/Blueprints/Managers/BP_GameController.BP_GameController_C|GetBPC_Inventory (Variables|References|GetAs%20BP%20My%20Controller)) Index)
    (else
      (Development|PrintString "Impossibe ingredient brute"))))

(fn FocusTarget
  (return ""))

(fn OnInteract
  (params (ItemSlots :type Array%20of%20S%20Item%20Slot%20Structures))
  (bind _as_bp_player (Variables|References|GetAs%20BP%20Player))
  (bind _player_controller_ref (Variables|/Game/Blueprints/Actors/BP_Player.BP_Player_C|GetPlayer_Controller_Ref _as_bp_player))
  (Variables|/Game/Blueprints/Components/BPC_Inventory.BPC_Inventory_C|Set%20Item%20Slots (Variables|/Game/Blueprints/Managers/BP_GameController.BP_GameController_C|GetBPC_Inventory (Variables|References|GetAs%20BP%20My%20Controller)) ItemSlots)
  (Pawn|Possess _player_controller_ref self)
  (Variables|/Script/Engine.PlayerController|SetbShowMouseCursor _player_controller_ref true)
  (EventDispatchers|BindEventtoOnUseItem (Variables|/Game/Blueprints/Managers/BP_GameController.BP_GameController_C|GetBPC_Inventory (Variables|References|GetAs%20BP%20My%20Controller)) (EventDispatchers|CreateEvent :!event Custom|ProcessIngredient))
  (switch Utilities|FlowControl|Switch|SwitchonEProcessingMethod (Variables|Default|GetMethod)
    (:NewEnumerator0
      _)
    (:NewEnumerator1
      _)
    (:NewEnumerator2
      (bind _returnvalue (UserInterface|CreateWidget "/Game/Widgets/HUD/WBP_Caudron.WBP_Caudron_C"))
      (bind _output_get (Variables|References|SetWidgetCauldron _returnvalue))
      (UserInterface|Viewport|AddtoViewport _output_get 0)
      (EventDispatchers|BindEventtoOnClickProcess (Variables|References|GetWidgetCauldron) (EventDispatchers|CreateEvent :!event Custom|LaunchCauldron))))
  (Variables|/Game/Blueprints/Managers/BP_GameController.BP_GameController_C|SetIsOnWorkbench (Variables|References|GetAs%20BP%20My%20Controller) true)
  (Default|AutomaticOpenInventory (Variables|References|GetAs%20BP%20My%20Controller)))