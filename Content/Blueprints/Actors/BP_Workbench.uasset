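; Workbench actor for processing ingredients, which caches the player pawn and controller on BeginPlay.
; ProcessIngredients currently only prints an "already process" message, as its branch condition is always true.
; Disconnected or unreachable logic remains for building cut or ground ingredient variants, swapping inventory items, closing the workbench widget and restoring game input.
; FocusTarget returns an empty string.
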(event EventBeginPlay
  (bind _asbp_player (Utilities|Casting|CastToBP_Player (Game|Player|GetPlayerPawn 0)))
  (Variables|Default|SetAs%20BP%20Player _asbp_player)
  (bind _asbp_my_controller (Utilities|Casting|CastToBP_MyController (Game|GetPlayerController 0)))
  (Variables|Default|SetAs%20BP%20My%20Controller _asbp_my_controller))

(fn ConstructionScript)

(fn ProcessIngredients
  (params (InIngredient :type S%20Ingredient%20Structure) (Method :type EProcessingMethod%20Enum :default "NewEnumerator0"))
  (if true
    (Development|PrintString "Ingredient already process")))

(fn FocusTarget
  (return ""))