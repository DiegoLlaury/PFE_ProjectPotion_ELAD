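; Possessable 3D grimoire for the ending, showing patron text and image pages; the player controller possesses it on BeginPlay.
; Four widget components feed render targets into dynamic materials on the left, center and right page meshes every tick.
; A timeline flips the center page, shifting page indices stored in the GameInstance, and bookmark jumps repeat turns until the target page.
; Page widgets are rebuilt on each update, always with page data 0.
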(event Custom|TurnLeft
  (bind _as_bp_game_instance (Variables|References|GetAs%20BP%20Game%20Instance))
  (bind _as_bp_game_instance_2 (Variables|References|GetAs%20BP%20Game%20Instance))
  (bind _listindexpage_menu (Variables|/Game/Blueprints/Managers/BP_GameInstance.BP_GameInstance_C|GetListIndexPage_Menu _as_bp_game_instance_2))
  (bind _listindexpage_menu_2 (Variables|/Game/Blueprints/Managers/BP_GameInstance.BP_GameInstance_C|GetListIndexPage_Menu _as_bp_game_instance))
  (Variables|Default|SetbPageTurning true)
  (if (> (Utilities|Array|Get(acopy) (Variables|/Game/Blueprints/Managers/BP_GameInstance.BP_GameInstance_C|GetListIndexPage_Menu (Variables|References|GetAs%20BP%20Game%20Instance))) 0)
    (for _index (range 1 3)
      (Utilities|Array|SetArrayElem _listindexpage_menu_2 (- 3 _index) (- (Utilities|Array|Get(acopy) _listindexpage_menu_2 3) _index)))
    (CallFunction|UpdatePage)
    (Utilities|FlowControl|Gate false :!label _label
      (:Exit
        (Utilities|FlowControl|Sequence
          (:then_0
            (goto _label Close))
          (:then_1
            (Utilities|FlowControl|Gate false) ; enters at Close
          )
          (:then_2
            (bind (_direction _alpha) (Timeline|PageTurn ReverseFromEnd)
              (:Update
                (Transformation|SetRelativeTransform (Variables|Default|GetSK_PageCenter) (Math|Transform|Lerp(Transform) (Transformation|GetRelativeTransform (Variables|Default|GetSK_PageRight)) (Transformation|GetRelativeTransform (Variables|Default|GetSK_PageLeft)) _alpha) false false)
                (Transformation|SetRelativeLocationAndRotation (Variables|Default|GetSK_PageCenter) (Math|Vector|Lerp(Vector) "0, 0, 0" "0, 0, 0" _alpha) (Math|Rotator|MakeRotator 9e+01 0.0 (Math|Float|Lerp 1.8e+02 3.6e+02 _alpha)) false false))
              (:Finished
                (Utilities|FlowControl|Sequence
                  (:then_0
                    (Utilities|FlowControl|Gate false) ; enters at Open
                  )
                  (:then_1
                    (goto _label Open))
                  (:then_2
                    (switch Utilities|FlowControl|Switch|SwitchonETimelineDirection _direction
                      (:Forward
                        (Utilities|Array|SetArrayElem _listindexpage_menu 0 (Utilities|Array|Get(acopy) _listindexpage_menu 2)))
                      (:Backward
                        (Utilities|Array|SetArrayElem _listindexpage_menu 3 (Utilities|Array|Get(acopy) _listindexpage_menu 1))))
                    (CallFunction|UpdatePage)
                    (Variables|Default|SetbPageTurning false))
                  (:then_3
                    (if (Variables|Boolean|GetbBookMarkWork)
                      (if (== (Utilities|Array|Get(acopy) (Variables|/Game/Blueprints/Managers/BP_GameInstance.BP_GameInstance_C|GetListIndexPage_Menu (Variables|References|GetAs%20BP%20Game%20Instance)) 3) (Variables|Default|GetTargetPage))
                        (Variables|Boolean|SetbBookMarkWork false)
                        (else
                          (CallFunction|BookmarkLoop))))))))))))))

(event Custom|TurnRight
  (bind _as_bp_game_instance (Variables|References|GetAs%20BP%20Game%20Instance))
  (bind _as_bp_game_instance_2 (Variables|References|GetAs%20BP%20Game%20Instance))
  (bind _listindexpage_menu (Variables|/Game/Blueprints/Managers/BP_GameInstance.BP_GameInstance_C|GetListIndexPage_Menu _as_bp_game_instance_2))
  (bind _listindexpage_menu_2 (Variables|/Game/Blueprints/Managers/BP_GameInstance.BP_GameInstance_C|GetListIndexPage_Menu _as_bp_game_instance))
  (Variables|Default|SetbPageTurning true)
  (bind _outrownames (DataTable|GetDataTableRowNames "/Game/Data/Datatables/DT_PageMenu.DT_PageMenu"))
  (if (< (+ (Utilities|Array|Get(acopy) (Variables|/Game/Blueprints/Managers/BP_GameInstance.BP_GameInstance_C|GetListIndexPage_Menu (Variables|References|GetAs%20BP%20Game%20Instance))) 3) (Utilities|Array|Length _outrownames))
    (for _index (range 1 3)
      (Utilities|Array|SetArrayElem _listindexpage_menu_2 _index (+ (Utilities|Array|Get(acopy) _listindexpage_menu_2) _index)))
    (CallFunction|UpdatePage)
    (Utilities|FlowControl|Gate false :!label _label
      (:Exit
        (Utilities|FlowControl|Sequence
          (:then_0
            (goto _label Close))
          (:then_1
            (Utilities|FlowControl|Gate false) ; enters at Close
          )
          (:then_2
            (bind (_direction _alpha) (Timeline|PageTurn PlayFromStart)
              (:Update
                (Transformation|SetRelativeTransform (Variables|Default|GetSK_PageCenter) (Math|Transform|Lerp(Transform) (Transformation|GetRelativeTransform (Variables|Default|GetSK_PageRight)) (Transformation|GetRelativeTransform (Variables|Default|GetSK_PageLeft)) _alpha) false false)
                (Transformation|SetRelativeLocationAndRotation (Variables|Default|GetSK_PageCenter) (Math|Vector|Lerp(Vector) "0, 0, 0" "0, 0, 0" _alpha) (Math|Rotator|MakeRotator 9e+01 0.0 (Math|Float|Lerp 1.8e+02 3.6e+02 _alpha)) false false))
              (:Finished
                (Utilities|FlowControl|Sequence
                  (:then_0
                    (goto _label Open))
                  (:then_1
                    (Utilities|FlowControl|Gate false) ; enters at Open
                  )
                  (:then_2
                    (switch Utilities|FlowControl|Switch|SwitchonETimelineDirection _direction
                      (:Forward
                        (Utilities|Array|SetArrayElem _listindexpage_menu 0 (Utilities|Array|Get(acopy) _listindexpage_menu 2)))
                      (:Backward
                        (Utilities|Array|SetArrayElem _listindexpage_menu 3 (Utilities|Array|Get(acopy) _listindexpage_menu 1))))
                    (CallFunction|UpdatePage)
                    (Variables|Default|SetbPageTurning false))
                  (:then_3
                    (if (Variables|Boolean|GetbBookMarkWork)
                      (if (== (Utilities|Array|Get(acopy) (Variables|/Game/Blueprints/Managers/BP_GameInstance.BP_GameInstance_C|GetListIndexPage_Menu (Variables|References|GetAs%20BP%20Game%20Instance)) 3) (Variables|Default|GetTargetPage))
                        (Variables|Boolean|SetbBookMarkWork false)
                        (else
                          (CallFunction|BookmarkLoop))))))))))))))

(event Custom|Move%20Camera
  (bind _camera (Variables|Default|GetCamera))
  (Timeline|Timeline PlayFromStart
    (:Update
      (Transformation|SetWorldLocation _camera (Math|Interpolation|VInterpTo (Transformation|GetWorldLocation _camera) (Variables|Default|GetBaseCamPos) (Variables|Default|GetDelta%20Seconds) (Math|Float|MakeLiteralFloat 5.0)) false false))))

(event Custom|ReturnButton
  (bind _as_bp_game_instance (Variables|References|GetAs%20BP%20Game%20Instance))
  (bind _as_bp_game_instance_2 (Variables|References|GetAs%20BP%20Game%20Instance))
  (bind _as_bp_game_instance_3 (Variables|References|GetAs%20BP%20Game%20Instance))
  (bind _as_bp_game_instance_4 (Variables|References|GetAs%20BP%20Game%20Instance))
  (bind _listindexpage_menu (Variables|/Game/Blueprints/Managers/BP_GameInstance.BP_GameInstance_C|GetListIndexPage_Menu _as_bp_game_instance))
  (bind _listindexpage_menu_2 (Variables|/Game/Blueprints/Managers/BP_GameInstance.BP_GameInstance_C|GetListIndexPage_Menu _as_bp_game_instance_4))
  (bind _listindexpage_menu_3 (Variables|/Game/Blueprints/Managers/BP_GameInstance.BP_GameInstance_C|GetListIndexPage_Menu _as_bp_game_instance_2))
  (bind _listindexpage_menu_4 (Variables|/Game/Blueprints/Managers/BP_GameInstance.BP_GameInstance_C|GetListIndexPage_Menu _as_bp_game_instance_3))
  (if (not (== (Utilities|Array|Get(acopy) (Variables|/Game/Blueprints/Managers/BP_GameInstance.BP_GameInstance_C|GetListIndexPage_Menu (Variables|References|GetAs%20BP%20Game%20Instance)) 3) 1))
    (Variables|Default|SetTargetPage 1)
    (Variables|Boolean|SetbBookMarkWork true)
    (if (< (Utilities|Array|Get(acopy) (Variables|/Game/Blueprints/Managers/BP_GameInstance.BP_GameInstance_C|GetListIndexPage_Menu (Variables|References|GetAs%20BP%20Game%20Instance)) 3) (Variables|Default|GetTargetPage))
      (Variables|Default|SetbPageTurning true)
      (bind _outrownames (DataTable|GetDataTableRowNames "/Game/Data/Datatables/DT_PageMenu.DT_PageMenu"))
      (if (< (+ (Utilities|Array|Get(acopy) _listindexpage_menu) 3) (Utilities|Array|Length _outrownames))
        (for _index (range 1 3)
          (Utilities|Array|SetArrayElem _listindexpage_menu_3 _index (+ (Utilities|Array|Get(acopy) _listindexpage_menu_3) _index)))
        (CallFunction|UpdatePage)
        (Utilities|FlowControl|Gate false :!label _label
          (:Exit
            (Utilities|FlowControl|Sequence
              (:then_0
                (goto _label Close))
              (:then_1
                (goto _label_2 Close))
              (:then_2
                (bind (_direction _alpha) (Timeline|PageTurn PlayFromStart)
                  (:Update
                    (Transformation|SetRelativeTransform (Variables|Default|GetSK_PageCenter) (Math|Transform|Lerp(Transform) (Transformation|GetRelativeTransform (Variables|Default|GetSK_PageRight)) (Transformation|GetRelativeTransform (Variables|Default|GetSK_PageLeft)) _alpha) false false)
                    (Transformation|SetRelativeLocationAndRotation (Variables|Default|GetSK_PageCenter) (Math|Vector|Lerp(Vector) "0, 0, 0" "0, 0, 0" _alpha) (Math|Rotator|MakeRotator 9e+01 0.0 (Math|Float|Lerp 1.8e+02 3.6e+02 _alpha)) false false))
                  (:Finished
                    (Utilities|FlowControl|Sequence
                      (:then_0
                        (goto _label Open))
                      (:then_1
                        (goto _label_2 Open))
                      (:then_2
                        (switch Utilities|FlowControl|Switch|SwitchonETimelineDirection _direction
                          (:Forward
                            (Utilities|Array|SetArrayElem _listindexpage_menu_2 0 (Utilities|Array|Get(acopy) _listindexpage_menu_2 2)))
                          (:Backward
                            (Utilities|Array|SetArrayElem _listindexpage_menu_2 3 (Utilities|Array|Get(acopy) _listindexpage_menu_2 1))))
                        (CallFunction|UpdatePage)
                        (Variables|Default|SetbPageTurning false))
                      (:then_3
                        (if (Variables|Boolean|GetbBookMarkWork)
                          (if (== (Utilities|Array|Get(acopy) (Variables|/Game/Blueprints/Managers/BP_GameInstance.BP_GameInstance_C|GetListIndexPage_Menu (Variables|References|GetAs%20BP%20Game%20Instance)) 3) (Variables|Default|GetTargetPage))
                            (Variables|Boolean|SetbBookMarkWork false)
                            (else
                              (CallFunction|BookmarkLoop)))))))))))))
      (else
        (Variables|Default|SetbPageTurning true)
        (if (> (Utilities|Array|Get(acopy) _listindexpage_menu) 0)
          (for _index_2 (range 1 3)
            (Utilities|Array|SetArrayElem _listindexpage_menu_4 (- 3 _index_2) (- (Utilities|Array|Get(acopy) _listindexpage_menu_4 3) _index_2)))
          (CallFunction|UpdatePage)
          (Utilities|FlowControl|Gate false :!label _label_2
            (:Exit
              (Utilities|FlowControl|Sequence
                (:then_0
                  (goto _label_2 Close))
                (:then_1
                  (goto _label Close))
                (:then_2
                  (Timeline|PageTurn ReverseFromEnd))))))))))

(event Custom|Bookmark%20Loop
  (bind _as_bp_game_instance (Variables|References|GetAs%20BP%20Game%20Instance))
  (bind _as_bp_game_instance_2 (Variables|References|GetAs%20BP%20Game%20Instance))
  (bind _as_bp_game_instance_3 (Variables|References|GetAs%20BP%20Game%20Instance))
  (bind _as_bp_game_instance_4 (Variables|References|GetAs%20BP%20Game%20Instance))
  (bind _listindexpage_menu (Variables|/Game/Blueprints/Managers/BP_GameInstance.BP_GameInstance_C|GetListIndexPage_Menu _as_bp_game_instance))
  (bind _listindexpage_menu_2 (Variables|/Game/Blueprints/Managers/BP_GameInstance.BP_GameInstance_C|GetListIndexPage_Menu _as_bp_game_instance_4))
  (bind _listindexpage_menu_3 (Variables|/Game/Blueprints/Managers/BP_GameInstance.BP_GameInstance_C|GetListIndexPage_Menu _as_bp_game_instance_2))
  (bind _listindexpage_menu_4 (Variables|/Game/Blueprints/Managers/BP_GameInstance.BP_GameInstance_C|GetListIndexPage_Menu _as_bp_game_instance_3))
  (if (Variables|Boolean|GetbBookMarkWork)
    (if (< (Utilities|Array|Get(acopy) (Variables|/Game/Blueprints/Managers/BP_GameInstance.BP_GameInstance_C|GetListIndexPage_Menu (Variables|References|GetAs%20BP%20Game%20Instance)) 3) (Variables|Default|GetTargetPage))
      (Variables|Default|SetbPageTurning true)
      (bind _outrownames (DataTable|GetDataTableRowNames "/Game/Data/Datatables/DT_PageMenu.DT_PageMenu"))
      (if (< (+ (Utilities|Array|Get(acopy) _listindexpage_menu) 3) (Utilities|Array|Length _outrownames))
        (for _index (range 1 3)
          (Utilities|Array|SetArrayElem _listindexpage_menu_3 _index (+ (Utilities|Array|Get(acopy) _listindexpage_menu_3) _index)))
        (CallFunction|UpdatePage)
        (Utilities|FlowControl|Gate false :!label _label
          (:Exit
            (Utilities|FlowControl|Sequence
              (:then_0
                (goto _label Close))
              (:then_1
                (goto _label_2 Close))
              (:then_2
                (bind (_direction _alpha) (Timeline|PageTurn PlayFromStart)
                  (:Update
                    (Transformation|SetRelativeTransform (Variables|Default|GetSK_PageCenter) (Math|Transform|Lerp(Transform) (Transformation|GetRelativeTransform (Variables|Default|GetSK_PageRight)) (Transformation|GetRelativeTransform (Variables|Default|GetSK_PageLeft)) _alpha) false false)
                    (Transformation|SetRelativeLocationAndRotation (Variables|Default|GetSK_PageCenter) (Math|Vector|Lerp(Vector) "0, 0, 0" "0, 0, 0" _alpha) (Math|Rotator|MakeRotator 9e+01 0.0 (Math|Float|Lerp 1.8e+02 3.6e+02 _alpha)) false false))
                  (:Finished
                    (Utilities|FlowControl|Sequence
                      (:then_0
                        (goto _label Open))
                      (:then_1
                        (goto _label_2 Open))
                      (:then_2
                        (switch Utilities|FlowControl|Switch|SwitchonETimelineDirection _direction
                          (:Forward
                            (Utilities|Array|SetArrayElem _listindexpage_menu_2 0 (Utilities|Array|Get(acopy) _listindexpage_menu_2 2)))
                          (:Backward
                            (Utilities|Array|SetArrayElem _listindexpage_menu_2 3 (Utilities|Array|Get(acopy) _listindexpage_menu_2 1))))
                        (CallFunction|UpdatePage)
                        (Variables|Default|SetbPageTurning false))
                      (:then_3
                        (if (Variables|Boolean|GetbBookMarkWork)
                          (if (== (Utilities|Array|Get(acopy) (Variables|/Game/Blueprints/Managers/BP_GameInstance.BP_GameInstance_C|GetListIndexPage_Menu (Variables|References|GetAs%20BP%20Game%20Instance)) 3) (Variables|Default|GetTargetPage))
                            (Variables|Boolean|SetbBookMarkWork false)
                            (else
                              (CallFunction|BookmarkLoop)))))))))))))
      (else
        (Variables|Default|SetbPageTurning true)
        (if (> (Utilities|Array|Get(acopy) _listindexpage_menu) 0)
          (for _index_2 (range 1 3)
            (Utilities|Array|SetArrayElem _listindexpage_menu_4 (- 3 _index_2) (- (Utilities|Array|Get(acopy) _listindexpage_menu_4 3) _index_2)))
          (CallFunction|UpdatePage)
          (Utilities|FlowControl|Gate false :!label _label_2
            (:Exit
              (Utilities|FlowControl|Sequence
                (:then_0
                  (goto _label_2 Close))
                (:then_1
                  (goto _label Close))
                (:then_2
                  (Timeline|PageTurn ReverseFromEnd))))))))))

(event Custom|SetTimelineTime
  (bind _as_bp_game_instance (Variables|References|GetAs%20BP%20Game%20Instance))
  (bind _listindexpage_menu (Variables|/Game/Blueprints/Managers/BP_GameInstance.BP_GameInstance_C|GetListIndexPage_Menu _as_bp_game_instance))
  (bind (_direction _alpha) (Timeline|PageTurn SetNewTime)
    (:Update
      (Transformation|SetRelativeTransform (Variables|Default|GetSK_PageCenter) (Math|Transform|Lerp(Transform) (Transformation|GetRelativeTransform (Variables|Default|GetSK_PageRight)) (Transformation|GetRelativeTransform (Variables|Default|GetSK_PageLeft)) _alpha) false false)
      (Transformation|SetRelativeLocationAndRotation (Variables|Default|GetSK_PageCenter) (Math|Vector|Lerp(Vector) "0, 0, 0" "0, 0, 0" _alpha) (Math|Rotator|MakeRotator 9e+01 0.0 (Math|Float|Lerp 1.8e+02 3.6e+02 _alpha)) false false))
    (:Finished
      (Utilities|FlowControl|Sequence
        (:then_0
          (Utilities|FlowControl|Gate false) ; enters at Open
        )
        (:then_1
          (Utilities|FlowControl|Gate false) ; enters at Open
        )
        (:then_2
          (switch Utilities|FlowControl|Switch|SwitchonETimelineDirection _direction
            (:Forward
              (Utilities|Array|SetArrayElem _listindexpage_menu 0 (Utilities|Array|Get(acopy) _listindexpage_menu 2)))
            (:Backward
              (Utilities|Array|SetArrayElem _listindexpage_menu 3 (Utilities|Array|Get(acopy) _listindexpage_menu 1))))
          (CallFunction|UpdatePage)
          (Variables|Default|SetbPageTurning false))
        (:then_3
          (if (Variables|Boolean|GetbBookMarkWork)
            (if (== (Utilities|Array|Get(acopy) (Variables|/Game/Blueprints/Managers/BP_GameInstance.BP_GameInstance_C|GetListIndexPage_Menu (Variables|References|GetAs%20BP%20Game%20Instance)) 3) (Variables|Default|GetTargetPage))
              (Variables|Boolean|SetbBookMarkWork false)
              (else
                (CallFunction|BookmarkLoop)))))))))

(event Custom|GoToOption
  (bind _as_bp_game_instance (Variables|References|GetAs%20BP%20Game%20Instance))
  (bind _as_bp_game_instance_2 (Variables|References|GetAs%20BP%20Game%20Instance))
  (bind _as_bp_game_instance_3 (Variables|References|GetAs%20BP%20Game%20Instance))
  (bind _as_bp_game_instance_4 (Variables|References|GetAs%20BP%20Game%20Instance))
  (bind _listindexpage_menu (Variables|/Game/Blueprints/Managers/BP_GameInstance.BP_GameInstance_C|GetListIndexPage_Menu _as_bp_game_instance))
  (bind _listindexpage_menu_2 (Variables|/Game/Blueprints/Managers/BP_GameInstance.BP_GameInstance_C|GetListIndexPage_Menu _as_bp_game_instance_4))
  (bind _listindexpage_menu_3 (Variables|/Game/Blueprints/Managers/BP_GameInstance.BP_GameInstance_C|GetListIndexPage_Menu _as_bp_game_instance_2))
  (bind _listindexpage_menu_4 (Variables|/Game/Blueprints/Managers/BP_GameInstance.BP_GameInstance_C|GetListIndexPage_Menu _as_bp_game_instance_3))
  (if (not (== (Utilities|Array|Get(acopy) (Variables|/Game/Blueprints/Managers/BP_GameInstance.BP_GameInstance_C|GetListIndexPage_Menu (Variables|References|GetAs%20BP%20Game%20Instance)) 3) 3))
    (Variables|Default|SetTargetPage 5)
    (Variables|Boolean|SetbBookMarkWork true)
    (if (< (Utilities|Array|Get(acopy) (Variables|/Game/Blueprints/Managers/BP_GameInstance.BP_GameInstance_C|GetListIndexPage_Menu (Variables|References|GetAs%20BP%20Game%20Instance)) 3) (Variables|Default|GetTargetPage))
      (Variables|Default|SetbPageTurning true)
      (bind _outrownames (DataTable|GetDataTableRowNames "/Game/Data/Datatables/DT_PageMenu.DT_PageMenu"))
      (if (< (+ (Utilities|Array|Get(acopy) _listindexpage_menu) 3) (Utilities|Array|Length _outrownames))
        (for _index (range 1 3)
          (Utilities|Array|SetArrayElem _listindexpage_menu_3 _index (+ (Utilities|Array|Get(acopy) _listindexpage_menu_3) _index)))
        (CallFunction|UpdatePage)
        (Utilities|FlowControl|Gate false :!label _label
          (:Exit
            (Utilities|FlowControl|Sequence
              (:then_0
                (goto _label Close))
              (:then_1
                (goto _label_2 Close))
              (:then_2
                (bind (_direction _alpha) (Timeline|PageTurn PlayFromStart)
                  (:Update
                    (Transformation|SetRelativeTransform (Variables|Default|GetSK_PageCenter) (Math|Transform|Lerp(Transform) (Transformation|GetRelativeTransform (Variables|Default|GetSK_PageRight)) (Transformation|GetRelativeTransform (Variables|Default|GetSK_PageLeft)) _alpha) false false)
                    (Transformation|SetRelativeLocationAndRotation (Variables|Default|GetSK_PageCenter) (Math|Vector|Lerp(Vector) "0, 0, 0" "0, 0, 0" _alpha) (Math|Rotator|MakeRotator 9e+01 0.0 (Math|Float|Lerp 1.8e+02 3.6e+02 _alpha)) false false))
                  (:Finished
                    (Utilities|FlowControl|Sequence
                      (:then_0
                        (goto _label Open))
                      (:then_1
                        (goto _label_2 Open))
                      (:then_2
                        (switch Utilities|FlowControl|Switch|SwitchonETimelineDirection _direction
                          (:Forward
                            (Utilities|Array|SetArrayElem _listindexpage_menu_2 0 (Utilities|Array|Get(acopy) _listindexpage_menu_2 2)))
                          (:Backward
                            (Utilities|Array|SetArrayElem _listindexpage_menu_2 3 (Utilities|Array|Get(acopy) _listindexpage_menu_2 1))))
                        (CallFunction|UpdatePage)
                        (Variables|Default|SetbPageTurning false))
                      (:then_3
                        (if (Variables|Boolean|GetbBookMarkWork)
                          (if (== (Utilities|Array|Get(acopy) (Variables|/Game/Blueprints/Managers/BP_GameInstance.BP_GameInstance_C|GetListIndexPage_Menu (Variables|References|GetAs%20BP%20Game%20Instance)) 3) (Variables|Default|GetTargetPage))
                            (Variables|Boolean|SetbBookMarkWork false)
                            (else
                              (CallFunction|BookmarkLoop)))))))))))))
      (else
        (Variables|Default|SetbPageTurning true)
        (if (> (Utilities|Array|Get(acopy) _listindexpage_menu) 0)
          (for _index_2 (range 1 3)
            (Utilities|Array|SetArrayElem _listindexpage_menu_4 (- 3 _index_2) (- (Utilities|Array|Get(acopy) _listindexpage_menu_4 3) _index_2)))
          (CallFunction|UpdatePage)
          (Utilities|FlowControl|Gate false :!label _label_2
            (:Exit
              (Utilities|FlowControl|Sequence
                (:then_0
                  (goto _label_2 Close))
                (:then_1
                  (goto _label Close))
                (:then_2
                  (Timeline|PageTurn ReverseFromEnd))))))))))

(event EventBeginPlay
  (Audio|PushSoundMixModifier "/Game/SoundEffect/SM_MainMix.SM_MainMix")
  (Utilities|FlowControl|Delay 0.2)
  (bind _asbp_game_controller (Utilities|Casting|CastToBP_GameController (Game|GetPlayerController 0)))
  (Variables|References|SetAs%20BP%20Game%20Controller _asbp_game_controller)
  (bind _asbp_player (Utilities|Casting|CastToBP_Player (Game|Player|GetPlayerPawn 0)))
  (Variables|References|SetAs%20BP%20Player _asbp_player)
  (bind _asbp_game_instance (Utilities|Casting|CastToBP_GameInstance (Game|GetGameInstance)))
  (Variables|References|SetAs%20BP%20Game%20Instance _asbp_game_instance)
  (Variables|Default|SetCurrentIndexButton 0)
  (Pawn|Possess (Variables|References|GetAs%20BP%20Game%20Controller) self)
  (bind _returnvalue (Rendering|Material|CreateDynamicMaterialInstance (Variables|Default|GetSK_PageCenter) 0 0 "None" :!class /Script/Engine.PrimitiveComponent))
  (Variables|References|SetDIM_Center _returnvalue)
  (bind _returnvalue_2 (Rendering|Material|CreateDynamicMaterialInstance (Variables|Default|GetSK_PageLeft) 0 0 "None" :!class /Script/Engine.PrimitiveComponent))
  (Variables|References|SetDIM_Left _returnvalue_2)
  (bind _returnvalue_3 (Rendering|Material|CreateDynamicMaterialInstance (Variables|Default|GetSK_PageRight) 0 0 "None" :!class /Script/Engine.PrimitiveComponent))
  (Variables|References|SetDIMRight _returnvalue_3)
  (Variables|Default|SetListWidgetComponent (Utilities|Array|MakeArray (Variables|Default|GetLeft) (Variables|Default|GetMidRight) (Variables|Default|GetMidLeft) (Variables|Default|GetRight)))
  (CallFunction|UpdatePage)
  (Variables|Default|SetBaseCamPos (Transformation|GetWorldLocation (Variables|Default|GetCamera))))

(event EventTick
  (params (DeltaSeconds :type Float%20%28single-precision%29))
  (Variables|Default|SetDelta%20Seconds DeltaSeconds)
  (Variables|Default|SetTimer (* (Variables|Default|GetDelta%20Seconds) (- (Variables|Default|GetTimer) (Variables|Default|GetDelta%20Seconds))))
  (Utilities|FlowControl|Sequence
    (:then_0
      (bind _dim_center (Variables|References|GetDIM_Center)
        (:then
          (Rendering|Material|SetTextureParameterValue _dim_center "TextFront" (Class|WidgetComponent|GetRenderTarget (Variables|Default|GetMidLeft)))
          (Rendering|Material|SetTextureParameterValue (Variables|References|GetDIM_Center) "TextBack" (Class|WidgetComponent|GetRenderTarget (Variables|Default|GetMidRight)))
          (Rendering|Material|SetTextureParameterValue (Variables|References|GetDIM_Left) "TextFront" (Class|WidgetComponent|GetRenderTarget (Variables|Default|GetLeft)))
          (Rendering|Material|SetTextureParameterValue (Variables|References|GetDIMRight) "TextBack" (Class|WidgetComponent|GetRenderTarget (Variables|Default|GetRight))))
        (:else)))))

(fn ConstructionScript)

(fn UpdatePage
  (for (_array_element _array_index) (Variables|/Game/Blueprints/Managers/BP_GameInstance.BP_GameInstance_C|GetListIndexPage_Menu (Variables|References|GetAs%20BP%20Game%20Instance))
    (CallFunction|CreateWidget _array_element _array_index)))

(fn CreateWidget
  (params (PageIndex :type Integer) (ArrayIndex :type Integer))
  (bind _listwidgetcomponent (Variables|Default|GetListWidgetComponent))
  (bind _output (Utilities|Array|Get(acopy) _listwidgetcomponent ArrayIndex))
  (if (== ArrayIndex 0)
    (bind _returnvalue (UserInterface|CreateWidget "/Game/Widgets/HUD/HUDGrimoire/WBP_PagePatronEnding_Txt.WBP_PagePatronEnding_Txt_C" 0 (Variables|References|GetAs%20BP%20Game%20Instance)))
    (Default|SetPageData _returnvalue)
    (UserInterface|SetWidget _output _returnvalue)
    (else
      (bind _returnvalue_2 (UserInterface|CreateWidget "/Game/Widgets/HUD/HUDGrimoire/WBP_PagePatronEnding_Img.WBP_PagePatronEnding_Img_C" 0 (Variables|References|GetAs%20BP%20Game%20Instance)))
      (Default|SetPageData _returnvalue_2)
      (UserInterface|SetWidget _output _returnvalue_2))))

(fn MoveUp)

(fn TeleportCursortoButton)

(fn FocusTarget
  (return ""))