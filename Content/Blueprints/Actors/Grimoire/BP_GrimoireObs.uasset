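; Interactable grimoire actor that opens the grimoire UI when the player interacts with it.
; On interact it creates a new WBP_Grimoire widget, calls its tutorial page update, adds it to the viewport and flags it as visible.
; BeginPlay caches the BP_GameController, though these graphs do not use it further.
; FocusTarget returns an empty string, and nothing here closes the widget.
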(event EventBeginPlay
  (bind _asbp_game_controller (Utilities|Casting|CastToBP_GameController (Game|GetPlayerController 0)))
  (Variables|Default|SetAs%20BP%20Game%20Controller _asbp_game_controller))

(event Collision|EventActorBeginOverlap
  (params (OtherActor :type Actor%20Object%20Reference)))

(event EventTick
  (params (DeltaSeconds :type Float%20%28single-precision%29)))

(event EventOnInteract
  (params (ItemSlots :type Array%20of%20S%20Item%20Slot%20Structures))
  (bind _returnvalue (UserInterface|CreateWidget "/Game/Widgets/HUD/HUDGrimoire/WBP_Grimoire.WBP_Grimoire_C"))
  (Default|UpdatePageTuto _returnvalue)
  (bind _output_get (Variables|Default|SetRef_WBP_Grimoire _returnvalue))
  (UserInterface|Viewport|AddtoViewport _output_get 0)
  (Variables|Default|SetIsWidgetVisible true))

(fn ConstructionScript)

(fn FocusTarget
  (return ""))