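; Main-menu grimoire pawn, possessed on BeginPlay: a 3D book whose pages host menu widgets for play, options, credits and quit.
; UpdatePage builds four page widgets from DT_PageMenu using GameInstance indices and binds the active side's buttons for stick navigation.
; Widget render targets feed dynamic page materials every Tick, while a timeline animates page turns, repeating toward bookmarked pages.
; Sound buttons switch the stick to adjusting sound-class volumes.
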(event Custom|TurnLeft
  (bind _as_bp_game_instance (Variables|References|GetAs%20BP%20Game%20Instance))
  (bind _as_bp_game_instance_2 (Variables|References|GetAs%20BP%20Game%20Instance))
  (bind _listindexpage_menu (Variables|/Game/Blueprints/Managers/BP_GameInstance.BP_GameInstance_C|GetListIndexPage_Menu _as_bp_game_instance_2))
  (bind _listindexpage_menu_2 (Variables|/Game/Blueprints/Managers/BP_GameInstance.BP_GameInstance_C|GetListIndexPage_Menu _as_bp_game_instance))
  (Variables|Default|SetbPageTurning true)
  (if (> (Utilities|Array|Get(acopy) (Variables|/Game/Blueprints/Managers/BP_GameInstance.BP_GameInstance_C|GetListIndexPage_Menu (Variables|References|GetAs%20BP%20Game%20Instance))) 0)
    (for _index (range 1 3)
      (Utilities|Array|SetArrayElem _listindexpage_menu_2 (- 3 _index) (- (Utilities|Array|Get(acopy) _listindexpage_menu_2 3) _index)))
    (CallFunction|UpdatePage)
    (Utilities|FlowControl|Gate false :!label _label
      (:Exit
        (Utilities|FlowControl|Sequence
          (:then_0
            (goto _label Close))
          (:then_1
            (Utilities|FlowControl|Gate false) ; enters at Close
          )
          (:then_2
            (bind (_direction _alpha _pagealpha) (Timeline|Timeline_0 ReverseFromEnd)
              (:Update
                (Rendering|Material|SetScalarParameterValue (Variables|References|GetDIM_Center) "Alpha" (* _pagealpha (Utilities|Select :Index _direction :Forward 1.0 :Backward -1.0)) :!class /Script/Engine.MaterialInstanceDynamic)
                (Transformation|SetRelativeTransform (Variables|Default|GetSK_PageCenter) (Math|Transform|Lerp(Transform) (Transformation|GetRelativeTransform (Variables|Default|GetSK_PageRight)) (Transformation|GetRelativeTransform (Variables|Default|GetSK_PageLeft)) _alpha) false false)
                (Transformation|SetRelativeLocationAndRotation (Variables|Default|GetSK_PageCenter) (Math|Vector|Lerp(Vector) "0, 0, 0" "0, 0, 0" _alpha) (Math|Rotator|MakeRotator 9e+01 0.0 (Math|Float|Lerp 1.8e+02 3.6e+02 _alpha)) false false))
              (:Finished
                (Utilities|FlowControl|Sequence
                  (:then_0
                    (Utilities|FlowControl|Gate false) ; enters at Open
                  )
                  (:then_1
                    (goto _label Open))
                  (:then_2
                    (switch Utilities|FlowControl|Switch|SwitchonETimelineDirection _direction
                      (:Forward
                        (Utilities|Array|SetArrayElem _listindexpage_menu 0 (Utilities|Array|Get(acopy) _listindexpage_menu 2)))
                      (:Backward
                        (Utilities|Array|SetArrayElem _listindexpage_menu 3 (Utilities|Array|Get(acopy) _listindexpage_menu 1))))
                    (CallFunction|UpdatePage)
                    (Variables|Default|SetbPageTurning false))
                  (:then_3
                    (if (Variables|Boolean|GetbBookMarkWork)
                      (if (== (Utilities|Array|Get(acopy) (Variables|/Game/Blueprints/Managers/BP_GameInstance.BP_GameInstance_C|GetListIndexPage_Menu (Variables|References|GetAs%20BP%20Game%20Instance)) 3) (Variables|Default|GetTargetPage))
                        (Variables|Boolean|SetbBookMarkWork false)
                        (else
                          (CallFunction|BookmarkLoop))))))))))))))

(event Custom|TurnRight
  (bind _as_bp_game_instance (Variables|References|GetAs%20BP%20Game%20Instance))
  (bind _as_bp_game_instance_2 (Variables|References|GetAs%20BP%20Game%20Instance))
  (bind _listindexpage_menu (Variables|/Game/Blueprints/Managers/BP_GameInstance.BP_GameInstance_C|GetListIndexPage_Menu _as_bp_game_instance_2))
  (bind _listindexpage_menu_2 (Variables|/Game/Blueprints/Managers/BP_GameInstance.BP_GameInstance_C|GetListIndexPage_Menu _as_bp_game_instance))
  (Variables|Default|SetbPageTurning true)
  (bind _outrownames (DataTable|GetDataTableRowNames "/Game/Data/Datatables/DT_PageMenu.DT_PageMenu"))
  (if (< (+ (Utilities|Array|Get(acopy) (Variables|/Game/Blueprints/Managers/BP_GameInstance.BP_GameInstance_C|GetListIndexPage_Menu (Variables|References|GetAs%20BP%20Game%20Instance))) 3) (Utilities|Array|Length _outrownames))
    (for _index (range 1 3)
      (Utilities|Array|SetArrayElem _listindexpage_menu_2 _index (+ (Utilities|Array|Get(acopy) _listindexpage_menu_2) _index)))
    (CallFunction|UpdatePage)
    (Utilities|FlowControl|Gate false :!label _label
      (:Exit
        (Utilities|FlowControl|Sequence
          (:then_0
            (goto _label Close))
          (:then_1
            (Utilities|FlowControl|Gate false) ; enters at Close
          )
          (:then_2
            (bind (_direction _alpha _pagealpha) (Timeline|Timeline_0 PlayFromStart)
              (:Update
                (Rendering|Material|SetScalarParameterValue (Variables|References|GetDIM_Center) "Alpha" (* _pagealpha (Utilities|Select :Index _direction :Forward 1.0 :Backward -1.0)) :!class /Script/Engine.MaterialInstanceDynamic)
                (Transformation|SetRelativeTransform (Variables|Default|GetSK_PageCenter) (Math|Transform|Lerp(Transform) (Transformation|GetRelativeTransform (Variables|Default|GetSK_PageRight)) (Transformation|GetRelativeTransform (Variables|Default|GetSK_PageLeft)) _alpha) false false)
                (Transformation|SetRelativeLocationAndRotation (Variables|Default|GetSK_PageCenter) (Math|Vector|Lerp(Vector) "0, 0, 0" "0, 0, 0" _alpha) (Math|Rotator|MakeRotator 9e+01 0.0 (Math|Float|Lerp 1.8e+02 3.6e+02 _alpha)) false false))
              (:Finished
                (Utilities|FlowControl|Sequence
                  (:then_0
                    (goto _label Open))
                  (:then_1
                    (Utilities|FlowControl|Gate false) ; enters at Open
                  )
                  (:then_2
                    (switch Utilities|FlowControl|Switch|SwitchonETimelineDirection _direction
                      (:Forward
                        (Utilities|Array|SetArrayElem _listindexpage_menu 0 (Utilities|Array|Get(acopy) _listindexpage_menu 2)))
                      (:Backward
                        (Utilities|Array|SetArrayElem _listindexpage_menu 3 (Utilities|Array|Get(acopy) _listindexpage_menu 1))))
                    (CallFunction|UpdatePage)
                    (Variables|Default|SetbPageTurning false))
                  (:then_3
                    (if (Variables|Boolean|GetbBookMarkWork)
                      (if (== (Utilities|Array|Get(acopy) (Variables|/Game/Blueprints/Managers/BP_GameInstance.BP_GameInstance_C|GetListIndexPage_Menu (Variables|References|GetAs%20BP%20Game%20Instance)) 3) (Variables|Default|GetTargetPage))
                        (Variables|Boolean|SetbBookMarkWork false)
                        (else
                          (CallFunction|BookmarkLoop))))))))))))))

(event Custom|ChooseButtonUp
  (bind _listwidgetbutton (Variables|Default|GetListWidgetButton))
  (bind _returnvalue (Utilities|Array|Length _listwidgetbutton))
  (bind _returnvalue_2 (- _returnvalue 1))
  (if (== (Variables|Default|GetCurrentIndexButton) 0)
    (Variables|Default|SetCurrentIndexButton _returnvalue_2)
    (else
      (bind _result (Math|Integer|DecrementInt (Variables|Default|GetCurrentIndexButton))
        (:%20%20
          (Variables|Default|SetCurrentIndexButton (Math|Integer|Clamp(Integer) _result 0 _returnvalue_2))))))
  (Utilities|IsValid (Utilities|Array|Get(acopy) (Variables|Default|GetListWidgetButton) (Variables|Default|GetCurrentIndexButton))
    (:Is%20Valid
      (Default|SetFocused (Utilities|Array|Get(acopy) (Variables|Default|GetListWidgetButton) (Variables|Default|GetCurrentIndexButton)))
      (Development|PrintString (Utilities|String|Append (Utilities|GetDisplayName (Utilities|Array|Get(acopy) (Variables|Default|GetListWidgetButton) (Variables|Default|GetCurrentIndexButton))) "_" (Utilities|String|ToString(Integer) (Variables|Default|GetCurrentIndexButton))))
      (Variables|Temporary|SetTempNavButton (Utilities|Array|Get(acopy) (Variables|Default|GetListWidgetButton) (Variables|Default|GetCurrentIndexButton))))))

(event Custom|ChooseButtonDown
  (bind _listwidgetbutton (Variables|Default|GetListWidgetButton))
  (bind _returnvalue (Utilities|Array|Length _listwidgetbutton))
  (bind _returnvalue_2 (- _returnvalue 1))
  (if (== _returnvalue_2 (Variables|Default|GetCurrentIndexButton))
    (Variables|Default|SetCurrentIndexButton 0)
    (else
      (bind _result (Math|Integer|IncrementInt (Variables|Default|GetCurrentIndexButton))
        (:%20%20
          (Variables|Default|SetCurrentIndexButton (Math|Integer|Clamp(Integer) _result 0 _returnvalue_2))))))
  (Utilities|IsValid (Utilities|Array|Get(acopy) (Variables|Default|GetListWidgetButton) (Variables|Default|GetCurrentIndexButton))
    (:Is%20Valid
      (Default|SetFocused (Utilities|Array|Get(acopy) (Variables|Default|GetListWidgetButton) (Variables|Default|GetCurrentIndexButton)))
      (Development|PrintString (Utilities|String|Append (Utilities|GetDisplayName (Utilities|Array|Get(acopy) (Variables|Default|GetListWidgetButton) (Variables|Default|GetCurrentIndexButton))) "_" (Utilities|String|ToString(Integer) (Variables|Default|GetCurrentIndexButton))))
      (Variables|Temporary|SetTempNavButton (Utilities|Array|Get(acopy) (Variables|Default|GetListWidgetButton) (Variables|Default|GetCurrentIndexButton))))))

(event Custom|Move%20Camera
  (bind _camera (Variables|Default|GetCamera))
  (Timeline|Timeline PlayFromStart
    (:Update
      (Transformation|SetWorldLocation _camera (Math|Interpolation|VInterpTo (Transformation|GetWorldLocation _camera) (Variables|Default|GetBaseCamPos) (Variables|Default|GetDelta%20Seconds) (Math|Float|MakeLiteralFloat 5.0)) false false))))

(event Custom|MoveDown)

(event Custom|OnButtonActivated
  (params (ButtonType :type EButtonMenu%20Enum :default "NewEnumerator0") (ButtonRef :type WBP%20Nav%20Button%20Object%20Reference))
  (bind _as_bp_game_instance (Variables|References|GetAs%20BP%20Game%20Instance))
  (bind _tempnavbutton (Variables|Temporary|GetTempNavButton))
  (if (not (Variables|Default|GetbPageTurning))
    (switch Utilities|FlowControl|Switch|SwitchonEButtonMenu (Variables|/Game/Widgets/HUD/HUDGrimoire/Menu/WBP_NavButton.WBP_NavButton_C|GetButtonType ButtonRef)
      (:NewEnumerator0
        (Default|ShowLoadingScreen _as_bp_game_instance)
        (Variables|/Game/Blueprints/Managers/BP_GameInstance.BP_GameInstance_C|SetbIsOnMenu _as_bp_game_instance false)
        (Class|GameplayStatics|LoadStreamLevelbySoftObjectPtr "/Game/Levels/Arenas/L_WitchHouse.L_WitchHouse" false false)
        (Game|OpenLevel(byObjectReference) "/Game/Levels/Arenas/L_WitchHouse.L_WitchHouse"))
      (:NewEnumerator1
        (Default|SetUnfocused (Variables|Temporary|GetTempNavButton))
        (Variables|Default|SetGrimoireSide "NewEnumerator1")
        (CallFunction|TurnRight))
      (:NewEnumerator2
        (Default|SetUnfocused (Variables|Temporary|GetTempNavButton))
        (Variables|Default|SetGrimoireSide "NewEnumerator1")
        (CallFunction|GotoOption))
      (:NewEnumerator3
        (Game|QuitGame 0 "Quit" false))
      (:NewEnumerator4
        (Default|SetUnfocused (Variables|Temporary|GetTempNavButton))
        (Variables|Default|SetGrimoireSide "NewEnumerator0")
        (CallFunction|ReturnButton))
      (:NewEnumerator5
        (Variables|Default|SetbParameterFocus true :!label _label)
        (Default|Unselect _tempnavbutton)
        (Default|ShowArrow _tempnavbutton "Visible"))
      (:NewEnumerator6
        (goto _label))
      (:NewEnumerator7
        (goto _label)))))

(event Custom|ReturnButton
  (bind _as_bp_game_instance (Variables|References|GetAs%20BP%20Game%20Instance))
  (bind _as_bp_game_instance_2 (Variables|References|GetAs%20BP%20Game%20Instance))
  (bind _as_bp_game_instance_3 (Variables|References|GetAs%20BP%20Game%20Instance))
  (bind _as_bp_game_instance_4 (Variables|References|GetAs%20BP%20Game%20Instance))
  (bind _listindexpage_menu (Variables|/Game/Blueprints/Managers/BP_GameInstance.BP_GameInstance_C|GetListIndexPage_Menu _as_bp_game_instance))
  (bind _listindexpage_menu_2 (Variables|/Game/Blueprints/Managers/BP_GameInstance.BP_GameInstance_C|GetListIndexPage_Menu _as_bp_game_instance_4))
  (bind _listindexpage_menu_3 (Variables|/Game/Blueprints/Managers/BP_GameInstance.BP_GameInstance_C|GetListIndexPage_Menu _as_bp_game_instance_2))
  (bind _listindexpage_menu_4 (Variables|/Game/Blueprints/Managers/BP_GameInstance.BP_GameInstance_C|GetListIndexPage_Menu _as_bp_game_instance_3))
  (if (not (== (Utilities|Array|Get(acopy) (Variables|/Game/Blueprints/Managers/BP_GameInstance.BP_GameInstance_C|GetListIndexPage_Menu (Variables|References|GetAs%20BP%20Game%20Instance)) 3) 1))
    (Variables|Default|SetTargetPage 1)
    (Variables|Boolean|SetbBookMarkWork true)
    (if (< (Utilities|Array|Get(acopy) (Variables|/Game/Blueprints/Managers/BP_GameInstance.BP_GameInstance_C|GetListIndexPage_Menu (Variables|References|GetAs%20BP%20Game%20Instance)) 3) (Variables|Default|GetTargetPage))
      (Variables|Default|SetbPageTurning true)
      (bind _outrownames (DataTable|GetDataTableRowNames "/Game/Data/Datatables/DT_PageMenu.DT_PageMenu"))
      (if (< (+ (Utilities|Array|Get(acopy) _listindexpage_menu) 3) (Utilities|Array|Length _outrownames))
        (for _index (range 1 3)
          (Utilities|Array|SetArrayElem _listindexpage_menu_3 _index (+ (Utilities|Array|Get(acopy) _listindexpage_menu_3) _index)))
        (CallFunction|UpdatePage)
        (Utilities|FlowControl|Gate false :!label _label
          (:Exit
            (Utilities|FlowControl|Sequence
              (:then_0
                (goto _label Close))
              (:then_1
                (goto _label_2 Close))
              (:then_2
                (bind (_direction _alpha _pagealpha) (Timeline|Timeline_0 PlayFromStart)
                  (:Update
                    (Rendering|Material|SetScalarParameterValue (Variables|References|GetDIM_Center) "Alpha" (* _pagealpha (Utilities|Select :Index _direction :Forward 1.0 :Backward -1.0)) :!class /Script/Engine.MaterialInstanceDynamic)
                    (Transformation|SetRelativeTransform (Variables|Default|GetSK_PageCenter) (Math|Transform|Lerp(Transform) (Transformation|GetRelativeTransform (Variables|Default|GetSK_PageRight)) (Transformation|GetRelativeTransform (Variables|Default|GetSK_PageLeft)) _alpha) false false)
                    (Transformation|SetRelativeLocationAndRotation (Variables|Default|GetSK_PageCenter) (Math|Vector|Lerp(Vector) "0, 0, 0" "0, 0, 0" _alpha) (Math|Rotator|MakeRotator 9e+01 0.0 (Math|Float|Lerp 1.8e+02 3.6e+02 _alpha)) false false))
                  (:Finished
                    (Utilities|FlowControl|Sequence
                      (:then_0
                        (goto _label Open))
                      (:then_1
                        (goto _label_2 Open))
                      (:then_2
                        (switch Utilities|FlowControl|Switch|SwitchonETimelineDirection _direction
                          (:Forward
                            (Utilities|Array|SetArrayElem _listindexpage_menu_2 0 (Utilities|Array|Get(acopy) _listindexpage_menu_2 2)))
                          (:Backward
                            (Utilities|Array|SetArrayElem _listindexpage_menu_2 3 (Utilities|Array|Get(acopy) _listindexpage_menu_2 1))))
                        (CallFunction|UpdatePage)
                        (Variables|Default|SetbPageTurning false))
                      (:then_3
                        (if (Variables|Boolean|GetbBookMarkWork)
                          (if (== (Utilities|Array|Get(acopy) (Variables|/Game/Blueprints/Managers/BP_GameInstance.BP_GameInstance_C|GetListIndexPage_Menu (Variables|References|GetAs%20BP%20Game%20Instance)) 3) (Variables|Default|GetTargetPage))
                            (Variables|Boolean|SetbBookMarkWork false)
                            (else
                              (CallFunction|BookmarkLoop)))))))))))))
      (else
        (Variables|Default|SetbPageTurning true)
        (if (> (Utilities|Array|Get(acopy) _listindexpage_menu) 0)
          (for _index_2 (range 1 3)
            (Utilities|Array|SetArrayElem _listindexpage_menu_4 (- 3 _index_2) (- (Utilities|Array|Get(acopy) _listindexpage_menu_4 3) _index_2)))
          (CallFunction|UpdatePage)
          (Utilities|FlowControl|Gate false :!label _label_2
            (:Exit
              (Utilities|FlowControl|Sequence
                (:then_0
                  (goto _label_2 Close))
                (:then_1
                  (goto _label Close))
                (:then_2
                  (Timeline|Timeline_0 ReverseFromEnd))))))))))

(event Custom|Bookmark%20Loop
  (bind _as_bp_game_instance (Variables|References|GetAs%20BP%20Game%20Instance))
  (bind _as_bp_game_instance_2 (Variables|References|GetAs%20BP%20Game%20Instance))
  (bind _as_bp_game_instance_3 (Variables|References|GetAs%20BP%20Game%20Instance))
  (bind _as_bp_game_instance_4 (Variables|References|GetAs%20BP%20Game%20Instance))
  (bind _listindexpage_menu (Variables|/Game/Blueprints/Managers/BP_GameInstance.BP_GameInstance_C|GetListIndexPage_Menu _as_bp_game_instance))
  (bind _listindexpage_menu_2 (Variables|/Game/Blueprints/Managers/BP_GameInstance.BP_GameInstance_C|GetListIndexPage_Menu _as_bp_game_instance_4))
  (bind _listindexpage_menu_3 (Variables|/Game/Blueprints/Managers/BP_GameInstance.BP_GameInstance_C|GetListIndexPage_Menu _as_bp_game_instance_2))
  (bind _listindexpage_menu_4 (Variables|/Game/Blueprints/Managers/BP_GameInstance.BP_GameInstance_C|GetListIndexPage_Menu _as_bp_game_instance_3))
  (if (Variables|Boolean|GetbBookMarkWork)
    (if (< (Utilities|Array|Get(acopy) (Variables|/Game/Blueprints/Managers/BP_GameInstance.BP_GameInstance_C|GetListIndexPage_Menu (Variables|References|GetAs%20BP%20Game%20Instance)) 3) (Variables|Default|GetTargetPage))
      (Variables|Default|SetbPageTurning true)
      (bind _outrownames (DataTable|GetDataTableRowNames "/Game/Data/Datatables/DT_PageMenu.DT_PageMenu"))
      (if (< (+ (Utilities|Array|Get(acopy) _listindexpage_menu) 3) (Utilities|Array|Length _outrownames))
        (for _index (range 1 3)
          (Utilities|Array|SetArrayElem _listindexpage_menu_3 _index (+ (Utilities|Array|Get(acopy) _listindexpage_menu_3) _index)))
        (CallFunction|UpdatePage)
        (Utilities|FlowControl|Gate false :!label _label
          (:Exit
            (Utilities|FlowControl|Sequence
              (:then_0
                (goto _label Close))
              (:then_1
                (goto _label_2 Close))
              (:then_2
                (bind (_direction _alpha _pagealpha) (Timeline|Timeline_0 PlayFromStart)
                  (:Update
                    (Rendering|Material|SetScalarParameterValue (Variables|References|GetDIM_Center) "Alpha" (* _pagealpha (Utilities|Select :Index _direction :Forward 1.0 :Backward -1.0)) :!class /Script/Engine.MaterialInstanceDynamic)
                    (Transformation|SetRelativeTransform (Variables|Default|GetSK_PageCenter) (Math|Transform|Lerp(Transform) (Transformation|GetRelativeTransform (Variables|Default|GetSK_PageRight)) (Transformation|GetRelativeTransform (Variables|Default|GetSK_PageLeft)) _alpha) false false)
                    (Transformation|SetRelativeLocationAndRotation (Variables|Default|GetSK_PageCenter) (Math|Vector|Lerp(Vector) "0, 0, 0" "0, 0, 0" _alpha) (Math|Rotator|MakeRotator 9e+01 0.0 (Math|Float|Lerp 1.8e+02 3.6e+02 _alpha)) false false))
                  (:Finished
                    (Utilities|FlowControl|Sequence
                      (:then_0
                        (goto _label Open))
                      (:then_1
                        (goto _label_2 Open))
                      (:then_2
                        (switch Utilities|FlowControl|Switch|SwitchonETimelineDirection _direction
                          (:Forward
                            (Utilities|Array|SetArrayElem _listindexpage_menu_2 0 (Utilities|Array|Get(acopy) _listindexpage_menu_2 2)))
                          (:Backward
                            (Utilities|Array|SetArrayElem _listindexpage_menu_2 3 (Utilities|Array|Get(acopy) _listindexpage_menu_2 1))))
                        (CallFunction|UpdatePage)
                        (Variables|Default|SetbPageTurning false))
                      (:then_3
                        (if (Variables|Boolean|GetbBookMarkWork)
                          (if (== (Utilities|Array|Get(acopy) (Variables|/Game/Blueprints/Managers/BP_GameInstance.BP_GameInstance_C|GetListIndexPage_Menu (Variables|References|GetAs%20BP%20Game%20Instance)) 3) (Variables|Default|GetTargetPage))
                            (Variables|Boolean|SetbBookMarkWork false)
                            (else
                              (CallFunction|BookmarkLoop)))))))))))))
      (else
        (Variables|Default|SetbPageTurning true)
        (if (> (Utilities|Array|Get(acopy) _listindexpage_menu) 0)
          (for _index_2 (range 1 3)
            (Utilities|Array|SetArrayElem _listindexpage_menu_4 (- 3 _index_2) (- (Utilities|Array|Get(acopy) _listindexpage_menu_4 3) _index_2)))
          (CallFunction|UpdatePage)
          (Utilities|FlowControl|Gate false :!label _label_2
            (:Exit
              (Utilities|FlowControl|Sequence
                (:then_0
                  (goto _label_2 Close))
                (:then_1
                  (goto _label Close))
                (:then_2
                  (Timeline|Timeline_0 ReverseFromEnd))))))))))

(event Custom|SetTimelineTime)

(event Custom|GoToOption
  (bind _as_bp_game_instance (Variables|References|GetAs%20BP%20Game%20Instance))
  (bind _as_bp_game_instance_2 (Variables|References|GetAs%20BP%20Game%20Instance))
  (bind _as_bp_game_instance_3 (Variables|References|GetAs%20BP%20Game%20Instance))
  (bind _as_bp_game_instance_4 (Variables|References|GetAs%20BP%20Game%20Instance))
  (bind _listindexpage_menu (Variables|/Game/Blueprints/Managers/BP_GameInstance.BP_GameInstance_C|GetListIndexPage_Menu _as_bp_game_instance))
  (bind _listindexpage_menu_2 (Variables|/Game/Blueprints/Managers/BP_GameInstance.BP_GameInstance_C|GetListIndexPage_Menu _as_bp_game_instance_4))
  (bind _listindexpage_menu_3 (Variables|/Game/Blueprints/Managers/BP_GameInstance.BP_GameInstance_C|GetListIndexPage_Menu _as_bp_game_instance_2))
  (bind _listindexpage_menu_4 (Variables|/Game/Blueprints/Managers/BP_GameInstance.BP_GameInstance_C|GetListIndexPage_Menu _as_bp_game_instance_3))
  (if (not (== (Utilities|Array|Get(acopy) (Variables|/Game/Blueprints/Managers/BP_GameInstance.BP_GameInstance_C|GetListIndexPage_Menu (Variables|References|GetAs%20BP%20Game%20Instance)) 3) 3))
    (Variables|Default|SetTargetPage 5)
    (Variables|Boolean|SetbBookMarkWork true)
    (if (< (Utilities|Array|Get(acopy) (Variables|/Game/Blueprints/Managers/BP_GameInstance.BP_GameInstance_C|GetListIndexPage_Menu (Variables|References|GetAs%20BP%20Game%20Instance)) 3) (Variables|Default|GetTargetPage))
      (Variables|Default|SetbPageTurning true)
      (bind _outrownames (DataTable|GetDataTableRowNames "/Game/Data/Datatables/DT_PageMenu.DT_PageMenu"))
      (if (< (+ (Utilities|Array|Get(acopy) _listindexpage_menu) 3) (Utilities|Array|Length _outrownames))
        (for _index (range 1 3)
          (Utilities|Array|SetArrayElem _listindexpage_menu_3 _index (+ (Utilities|Array|Get(acopy) _listindexpage_menu_3) _index)))
        (CallFunction|UpdatePage)
        (Utilities|FlowControl|Gate false :!label _label
          (:Exit
            (Utilities|FlowControl|Sequence
              (:then_0
                (goto _label Close))
              (:then_1
                (goto _label_2 Close))
              (:then_2
                (bind (_direction _alpha _pagealpha) (Timeline|Timeline_0 PlayFromStart)
                  (:Update
                    (Rendering|Material|SetScalarParameterValue (Variables|References|GetDIM_Center) "Alpha" (* _pagealpha (Utilities|Select :Index _direction :Forward 1.0 :Backward -1.0)) :!class /Script/Engine.MaterialInstanceDynamic)
                    (Transformation|SetRelativeTransform (Variables|Default|GetSK_PageCenter) (Math|Transform|Lerp(Transform) (Transformation|GetRelativeTransform (Variables|Default|GetSK_PageRight)) (Transformation|GetRelativeTransform (Variables|Default|GetSK_PageLeft)) _alpha) false false)
                    (Transformation|SetRelativeLocationAndRotation (Variables|Default|GetSK_PageCenter) (Math|Vector|Lerp(Vector) "0, 0, 0" "0, 0, 0" _alpha) (Math|Rotator|MakeRotator 9e+01 0.0 (Math|Float|Lerp 1.8e+02 3.6e+02 _alpha)) false false))
                  (:Finished
                    (Utilities|FlowControl|Sequence
                      (:then_0
                        (goto _label Open))
                      (:then_1
                        (goto _label_2 Open))
                      (:then_2
                        (switch Utilities|FlowControl|Switch|SwitchonETimelineDirection _direction
                          (:Forward
                            (Utilities|Array|SetArrayElem _listindexpage_menu_2 0 (Utilities|Array|Get(acopy) _listindexpage_menu_2 2)))
                          (:Backward
                            (Utilities|Array|SetArrayElem _listindexpage_menu_2 3 (Utilities|Array|Get(acopy) _listindexpage_menu_2 1))))
                        (CallFunction|UpdatePage)
                        (Variables|Default|SetbPageTurning false))
                      (:then_3
                        (if (Variables|Boolean|GetbBookMarkWork)
                          (if (== (Utilities|Array|Get(acopy) (Variables|/Game/Blueprints/Managers/BP_GameInstance.BP_GameInstance_C|GetListIndexPage_Menu (Variables|References|GetAs%20BP%20Game%20Instance)) 3) (Variables|Default|GetTargetPage))
                            (Variables|Boolean|SetbBookMarkWork false)
                            (else
                              (CallFunction|BookmarkLoop)))))))))))))
      (else
        (Variables|Default|SetbPageTurning true)
        (if (> (Utilities|Array|Get(acopy) _listindexpage_menu) 0)
          (for _index_2 (range 1 3)
            (Utilities|Array|SetArrayElem _listindexpage_menu_4 (- 3 _index_2) (- (Utilities|Array|Get(acopy) _listindexpage_menu_4 3) _index_2)))
          (CallFunction|UpdatePage)
          (Utilities|FlowControl|Gate false :!label _label_2
            (:Exit
              (Utilities|FlowControl|Sequence
                (:then_0
                  (goto _label_2 Close))
                (:then_1
                  (goto _label Close))
                (:then_2
                  (Timeline|Timeline_0 ReverseFromEnd))))))))))

(event Input|EnhancedActionEvents|EnhancedInputActionIA_Interact
  (params (ActionValue :type Boolean) (ElapsedSeconds :type Float%20%28double-precision%29) (TriggeredSeconds :type Float%20%28double-precision%29) (InputAction :type Input%20Action%20Object%20Reference :default "/Game/FirstPerson/Input/Actions/IA_Interact.IA_Interact"))
  (:Started
    (bind _tempnavbutton (Variables|Temporary|GetTempNavButton)
      (:then
        (Default|OnInteract _tempnavbutton))
      (:else))))

(event Input|EnhancedActionEvents|EnhancedInputActionIA_EscapeWorkbench
  (params (ActionValue :type Boolean) (ElapsedSeconds :type Float%20%28double-precision%29) (TriggeredSeconds :type Float%20%28double-precision%29) (InputAction :type Input%20Action%20Object%20Reference :default "/Game/FirstPerson/Input/Actions/IA_EscapeWorkbench.IA_EscapeWorkbench"))
  (bind _tempnavbutton (Variables|Temporary|GetTempNavButton))
  (:Started
    (switch Utilities|FlowControl|Switch|SwitchonEButtonMenu (Variables|/Game/Widgets/HUD/HUDGrimoire/Menu/WBP_NavButton.WBP_NavButton_C|GetButtonType (Variables|Temporary|GetTempNavButton))
      (:NewEnumerator5
        _)
      (:NewEnumerator6
        _)
      (:NewEnumerator7
        _))
    (Variables|Default|SetbParameterFocus false)
    (Default|Select _tempnavbutton)
    (Default|ShowArrow _tempnavbutton "Hidden")))

(event Input|EnhancedActionEvents|EnhancedInputActionIA_JoystickRSelect
  (params (ActionValue :type Float%20%28double-precision%29) (ElapsedSeconds :type Float%20%28double-precision%29) (TriggeredSeconds :type Float%20%28double-precision%29) (InputAction :type Input%20Action%20Object%20Reference :default "/Game/FirstPerson/Input/Actions/IA_JoystickRSelect.IA_JoystickRSelect"))
  (bind _tempnavbutton (Variables|Temporary|GetTempNavButton))
  (bind _tempnavbutton_2 (Variables|Temporary|GetTempNavButton))
  (:Triggered
    (if (Variables|Default|GetbParameterFocus)
      (if (and (< ActionValue -0.5) (not (Variables|Boolean|GetbJoystickConsumed)))
        (bind _numberparameter (Default|ChangeDownSound _tempnavbutton))
        (Variables|Default|SetNumber%20Parameter _numberparameter)
        (switch Utilities|FlowControl|Switch|SwitchonEButtonMenu (Variables|/Game/Widgets/HUD/HUDGrimoire/Menu/WBP_NavButton.WBP_NavButton_C|GetButtonType _tempnavbutton) :!label _label
          (:NewEnumerator5
            (bind _output_get (Variables|/Game/Blueprints/Managers/BP_GameInstance.BP_GameInstance_C|SetSoundValue_Voice (Variables|References|GetAs%20BP%20Game%20Instance) (Variables|Default|GetNumber%20Parameter)))
            (Audio|SetSoundMixClassOverride "/Game/SoundEffect/SM_MainMix.SM_MainMix" "/Game/SoundEffect/SC_Voice.SC_Voice" (/ (Math|Conversions|ToFloat(Integer) _output_get) 1e+02) 1.0 0.2 true))
          (:NewEnumerator6
            (bind _output_get_2 (Variables|/Game/Blueprints/Managers/BP_GameInstance.BP_GameInstance_C|SetSoundValue_Ambiant (Variables|References|GetAs%20BP%20Game%20Instance) (Variables|Default|GetNumber%20Parameter)))
            (Audio|SetSoundMixClassOverride "/Game/SoundEffect/SM_MainMix.SM_MainMix" "/Game/SoundEffect/SC_Ambiant.SC_Ambiant" (/ (Math|Conversions|ToFloat(Integer) _output_get_2) 1e+02) 1.0 0.2 true))
          (:NewEnumerator7
            (bind _output_get_3 (Variables|/Game/Blueprints/Managers/BP_GameInstance.BP_GameInstance_C|SetSoundValue_Music (Variables|References|GetAs%20BP%20Game%20Instance) (Variables|Default|GetNumber%20Parameter)))
            (Audio|SetSoundMixClassOverride "/Game/SoundEffect/SM_MainMix.SM_MainMix" "/Game/SoundEffect/SC_Music.SC_Music" (/ (Math|Conversions|ToFloat(Integer) _output_get_3) 1e+02) 1.0 0.2 true)))
        (elif (and (> ActionValue 0.5) (not (Variables|Boolean|GetbJoystickConsumed)))
          (bind _numberparameter_2 (Default|ChangeUpSound _tempnavbutton))
          (Variables|Default|SetNumber%20Parameter _numberparameter_2)
          (goto _label)))
      (elif (and (< ActionValue -0.5) (not (Variables|Boolean|GetbJoystickConsumed)))
        (Default|SetUnfocused _tempnavbutton_2)
        (CallFunction|ChooseButtonDown)
        (Variables|Boolean|SetbJoystickConsumed true)
        (elif (and (> ActionValue 0.5) (not (Variables|Boolean|GetbJoystickConsumed)))
          (Default|SetUnfocused _tempnavbutton_2)
          (CallFunction|ChooseButtonUP)
          (Variables|Boolean|SetbJoystickConsumed true)))))
  (:Completed
    (Variables|Boolean|SetbJoystickConsumed false)))

(event EventBeginPlay
  (Audio|PushSoundMixModifier "/Game/SoundEffect/SM_MainMix.SM_MainMix")
  (Utilities|FlowControl|Delay 0.2)
  (bind _asbp_game_controller (Utilities|Casting|CastToBP_GameController (Game|GetPlayerController 0)))
  (Variables|References|SetAs%20BP%20Game%20Controller _asbp_game_controller)
  (bind _asbp_player (Utilities|Casting|CastToBP_Player (Game|Player|GetPlayerPawn 0)))
  (Variables|References|SetAs%20BP%20Player _asbp_player)
  (bind _asbp_game_instance (Utilities|Casting|CastToBP_GameInstance (Game|GetGameInstance)))
  (Variables|References|SetAs%20BP%20Game%20Instance _asbp_game_instance)
  (Variables|Default|SetCurrentIndexButton 0)
  (Pawn|Possess (Variables|References|GetAs%20BP%20Game%20Controller) self)
  (bind _returnvalue (Rendering|Material|CreateDynamicMaterialInstance (Variables|Default|GetSK_PageCenter) 0 0 "None" :!class /Script/Engine.PrimitiveComponent))
  (Variables|References|SetDIM_Center _returnvalue)
  (bind _returnvalue_2 (Rendering|Material|CreateDynamicMaterialInstance (Variables|Default|GetSK_PageLeft) 0 0 "None" :!class /Script/Engine.PrimitiveComponent))
  (Variables|References|SetDIM_Left _returnvalue_2)
  (bind _returnvalue_3 (Rendering|Material|CreateDynamicMaterialInstance (Variables|Default|GetSK_PageRight) 0 0 "None" :!class /Script/Engine.PrimitiveComponent))
  (Variables|References|SetDIMRight _returnvalue_3)
  (Variables|Default|SetListWidgetComponent (Utilities|Array|MakeArray (Variables|Default|GetLeft) (Variables|Default|GetMidRight) (Variables|Default|GetMidLeft) (Variables|Default|GetRight)))
  (CallFunction|UpdatePage)
  (Variables|Default|SetBaseCamPos (Transformation|GetWorldLocation (Variables|Default|GetCamera))))

(event EventTick
  (params (DeltaSeconds :type Float%20%28single-precision%29))
  (Variables|Default|SetDelta%20Seconds DeltaSeconds)
  (Variables|Default|SetTimer (* (Variables|Default|GetDelta%20Seconds) (- (Variables|Default|GetTimer) (Variables|Default|GetDelta%20Seconds))))
  (Utilities|FlowControl|Sequence
    (:then_0
      (bind _dim_center (Variables|References|GetDIM_Center)
        (:then
          (Rendering|Material|SetTextureParameterValue _dim_center "TextFront" (Class|WidgetComponent|GetRenderTarget (Variables|Default|GetMidLeft)))
          (Rendering|Material|SetTextureParameterValue (Variables|References|GetDIM_Center) "TextBack" (Class|WidgetComponent|GetRenderTarget (Variables|Default|GetMidRight)))
          (Rendering|Material|SetTextureParameterValue (Variables|References|GetDIM_Left) "TextFront" (Class|WidgetComponent|GetRenderTarget (Variables|Default|GetLeft)))
          (Rendering|Material|SetTextureParameterValue (Variables|References|GetDIMRight) "TextBack" (Class|WidgetComponent|GetRenderTarget (Variables|Default|GetRight))))
        (:else)))))

(fn ConstructionScript)

(fn UpdatePage
  (for _array_element (Variables|Default|GetListWidgetButton)
    (EventDispatchers|UnbindEventfromOnButtonActived _array_element (EventDispatchers|CreateEvent :!event Custom|OnButtonActivated)))
  (Utilities|Array|Clear (Variables|Default|GetListWidgetButton))
  (for (_array_element_2 _array_index) (Variables|/Game/Blueprints/Managers/BP_GameInstance.BP_GameInstance_C|GetListIndexPage_Menu (Variables|References|GetAs%20BP%20Game%20Instance))
    (CallFunction|CreateWidget _array_element_2 _array_index))
  (switch Utilities|FlowControl|Switch|SwitchonESideGrimoire (Variables|Default|GetGrimoireSide)
    (:NewEnumerator0
      (for (_array_element_3 _array_index_2) (Variables|Default|GetListWidgetComponent)
        (if (< _array_index_2 2)
          (bind _navbuttons (Class|BPIGrimoirePage|GetNavigationButton(Message) (UserInterface|GetWidget _array_element_3)))
          (Class|BPIGrimoirePage|OnPageFocused(Message) (Variables|Temporary|GetTempWidgetMenu))
          (if (Utilities|Array|IsEmpty _navbuttons)
            (Development|PrintString "No Button")
            (else
              (for _array_element_4 _navbuttons
                (EventDispatchers|BindEventtoOnButtonActived _array_element_4 (EventDispatchers|CreateEvent :!event Custom|OnButtonActivated))
                (Utilities|Array|Add (Variables|Default|GetListWidgetButton) _array_element_4))
              (Variables|Temporary|SetTempNavButton (Utilities|Array|Get(acopy) (Variables|Default|GetListWidgetButton)))
              (bind _tempnavbutton (Variables|Temporary|GetTempNavButton)
                (:then
                  (Default|SetFocused _tempnavbutton))
                (:else
                  (Development|PrintString "TempNavButton not Valid"))))))))
    (:NewEnumerator1
      (for (_array_element_5 _array_index_3) (Variables|Default|GetListWidgetComponent)
        (if (or (== _array_index_3 2) (== _array_index_3 3))
          (bind _navbuttons_2 (Class|BPIGrimoirePage|GetNavigationButton(Message) (UserInterface|GetWidget _array_element_5)))
          (Class|BPIGrimoirePage|OnPageFocused(Message) (Variables|Temporary|GetTempWidgetMenu))
          (if (Utilities|Array|IsEmpty _navbuttons_2)
            (Development|PrintString "No Button")
            (else
              (for _array_element_6 _navbuttons_2
                (EventDispatchers|BindEventtoOnButtonActived _array_element_6 (EventDispatchers|CreateEvent :!event Custom|OnButtonActivated))
                (Utilities|Array|Add (Variables|Default|GetListWidgetButton) _array_element_6))
              (bind _output_get (Variables|Temporary|SetTempNavButton (Utilities|Array|Get(acopy) (Variables|Default|GetListWidgetButton))))
              (Default|SetFocused _output_get))))))))

(fn CreateWidget
  (params (PageIndex :type Integer) (ArrayIndex :type Integer))
  (bind _listwidgetcomponent (Variables|Default|GetListWidgetComponent))
  (bind _output (Utilities|Array|Get(acopy) _listwidgetcomponent ArrayIndex))
  (bind _outrownames (DataTable|GetDataTableRowNames "/Game/Data/Datatables/DT_PageMenu.DT_PageMenu"))
  (bind _returnvalue (Utilities|GetDataTableRow "/Game/Data/Datatables/DT_PageMenu.DT_PageMenu" (Utilities|Array|Get(acopy) _outrownames PageIndex))
    (:then
      (switch Utilities|FlowControl|Switch|SwitchonEGrimoirePageType (.PageType (Utilities|Struct|BreakSPageData _returnvalue))
        (:NewEnumerator5
          (bind _returnvalue_2 (UserInterface|CreateWidget (.WidgetClass (Utilities|Struct|BreakSPageData _returnvalue))))
          (Variables|Temporary|SetTempWidgetMenu _returnvalue_2)
          (if (Class|KismetSystemLibrary|DoesClassImplementInterface (.WidgetClass (Utilities|Struct|BreakSPageData _returnvalue)) "/Game/Blueprints/Interfaces/BPI_GrimoirePage.BPI_GrimoirePage_C")
            (bind _tempwidgetmenu (Variables|Temporary|GetTempWidgetMenu)
              (:then
                (UserInterface|SetWidget _output _tempwidgetmenu))
              (:else))
            (else
              (Development|PrintString "Interface problem"))))
        (:NewEnumerator0
          (bind _returnvalue_3 (UserInterface|CreateWidget "/Game/Widgets/HUD/HUDGrimoire/WBP_PagePatronFrontPage.WBP_PagePatronFrontPage_C"))
          (bind _output_get (Variables|References|SetTempWidgetChapter _returnvalue_3))
          (Default|SetPageData _output_get PageIndex)
          (UserInterface|SetWidget _output (Variables|References|GetTempWidgetChapter)))
        (:NewEnumerator2
          (bind _returnvalue_4 (UserInterface|CreateWidget "/Game/Widgets/HUD/HUDGrimoire/WBP_PagePatronIngredient.WBP_PagePatronIngredient_C"))
          (bind _output_get_2 (Variables|References|SetTempWidgetIngredient _returnvalue_4))
          (Default|SetPageData _output_get_2 PageIndex)
          (UserInterface|SetWidget _output (Variables|References|GetTempWidgetIngredient)))
        (:NewEnumerator3
          (bind _returnvalue_5 (UserInterface|CreateWidget "/Game/Widgets/HUD/HUDGrimoire/WBP_PagePatronPotion.WBP_PagePatronPotion_C" 0 (Variables|References|GetAs%20BP%20Game%20Instance)))
          (bind _output_get_3 (Variables|References|SetTempWidgetPotion _returnvalue_5))
          (Default|SetPageData _output_get_3 PageIndex)
          (UserInterface|SetWidget _output (Variables|References|GetTempWidgetPotion)))
        (:NewEnumerator4
          (bind _returnvalue_6 (UserInterface|CreateWidget "/Game/Widgets/HUD/HUDGrimoire/WBP_PagePatronBlank.WBP_PagePatronBlank_C"))
          (bind _output_get_4 (Variables|References|SetTempWidgetBlank _returnvalue_6))
          (UserInterface|SetWidget _output _output_get_4))))))

(fn MoveUp)

(fn TeleportCursortoButton)

(fn FocusTarget
  (return ""))