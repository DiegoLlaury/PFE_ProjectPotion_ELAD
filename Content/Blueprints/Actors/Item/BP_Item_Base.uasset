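; Base actor for ingredient items, which shows a "Prendre {Item}" focus prompt and an outline highlight.
; The construction script sets mesh, scale and optional material from the item's DT_Ingredients row, which also supplies the prompt name.
; On BeginPlay it copies its unique instance ID into BPCItemData and destroys itself if the GameInstance lists it as collected.
; UIInteract applies the outline overlay, and a delayed event clears it once the Tick-updated Timer is negative.
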(event Custom|OutlineDelay
  (if (< (Variables|Default|GetTimer) 0.0)
    (Rendering|Material|SetOverlayMaterial (Variables|Default|GetCube) "/Game/Materials/MI_ObjectOutlineFalse.MI_ObjectOutlineFalse" :!class /Script/Engine.MeshComponent)))

(event EventBeginPlay
  (bind _asbp_game_instance (Utilities|Casting|CastToBP_GameInstance (Game|GetGameInstance)))
  (Variables|Default|SetAs%20BP%20Game%20Instance _asbp_game_instance)
  (bind _output_get (Variables|/Game/Blueprints/Components/BPC_ItemData.BPC_ItemData_C|SetUniqueItemID (Variables|Default|GetBPC_ItemData) (Utilities|String|StringToName (Variables|Default|GetUniqueInstanceID))))
  (if (Utilities|Set|Contains (Variables|/Game/Blueprints/Managers/BP_GameInstance.BP_GameInstance_C|GetCollectedItems (Variables|Default|GetAs%20BP%20Game%20Instance)) _output_get)
    (Actor|DestroyActor)))

(event EventUIInteract
  (Rendering|Material|SetOverlayMaterial (Variables|Default|GetCube) "/Game/Materials/MI_ObjectOutline.MI_ObjectOutline" :!class /Script/Engine.MeshComponent)
  (Variables|Default|SetTimer 0.1)
  (Utilities|Time|SetTimerbyEvent (delegate Custom|OutlineDelay) 0.2))

(event EventTick
  (params (DeltaSeconds :type Float%20%28single-precision%29))
  (Variables|Default|SetDelta%20Seconds DeltaSeconds)
  (Variables|Default|SetTimer (* (Variables|Default|GetDelta%20Seconds) (- (Variables|Default|GetTimer) (Variables|Default|GetDelta%20Seconds)))))

(fn ConstructionScript
  (bind _cube (Variables|Default|GetCube))
  (bind _returnvalue (Utilities|GetDataTableRow "/Game/Data/Datatables/DT_Ingredients.DT_Ingredients" (.rowname (Variables|/Game/Blueprints/Components/BPC_ItemData.BPC_ItemData_C|GetGetItemData (Variables|Default|GetBPC_ItemData))))
    (:then
      (Components|StaticMesh|SetStaticMesh _cube (.mesh _returnvalue))
      (Transformation|SetRelativeScale3D _cube (.scaleobject _returnvalue))
      (Utilities|IsValid (.texture _returnvalue)
        (:Is%20Valid
          (Rendering|Material|SetMaterial (Variables|Default|GetCube) 0 (.texture _returnvalue)))))))

(fn FocusTarget
  (bind _returnvalue (Utilities|GetDataTableRow "/Game/Data/Datatables/DT_Ingredients.DT_Ingredients" (.RowName (Utilities|Struct|BreakDataTableRowHandle (Variables|/Game/Blueprints/Components/BPC_ItemData.BPC_ItemData_C|GetGetItemData (Variables|Default|GetBPC_ItemData)))))
    (:then
      (return (Utilities|Text|FormatText "Prendre {Item}" (.Name (Utilities|Struct|BreakSIngredient _returnvalue)))))))