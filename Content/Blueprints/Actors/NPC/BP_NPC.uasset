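; NPC actor that the player can interact with to open a world-space dialogue driven by BPCDialogueManager, unless the game instance flags NpcDispawn.
; Each tick eases the dialogue widget toward the player's side, rotating and distance-scaling it and the key prompt toward the camera.
; Leaving DetectPlayer mid-talk hides the dialogue, and the next interaction replays its opening animation.
; StartWalkAnim picks animations by NPC type; idle, turn and grab functions are stubs.
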(event OnComponentBeginOverlap(DetectPlayer)
  (params (OverlappedComponent :type Primitive%20Component%20Object%20Reference) (OtherActor :type Actor%20Object%20Reference) (OtherComp :type Primitive%20Component%20Object%20Reference) (OtherBodyIndex :type Integer) (bFromSweep :type Boolean) (SweepResult :type Hit%20Result%20Structure%20%28by%20ref%29))
  (if (== OtherActor (Game|GetPlayerCharacter 0))
    _))

(event OnComponentEndOverlap(DetectPlayer)
  (params (OverlappedComponent :type Primitive%20Component%20Object%20Reference) (OtherActor :type Actor%20Object%20Reference) (OtherComp :type Primitive%20Component%20Object%20Reference) (OtherBodyIndex :type Integer))
  (if (and (== OtherActor (Game|GetPlayerCharacter 0)) (Variables|/Game/Blueprints/Components/BPC_DialogueManager.BPC_DialogueManager_C|GetIsTalking? (Variables|Default|GetBPC_DialogueManager)))
    (Default|DialogueReversAnim (Variables|/Game/Blueprints/Components/BPC_DialogueManager.BPC_DialogueManager_C|GetWB_UIDialogue (Variables|Default|GetBPC_DialogueManager)))
    (Utilities|FlowControl|Delay 0.25)
    (Rendering|SetVisibility (Variables|Default|GetWB_Dialogue) false false)
    (Variables|Default|SetEndTalk true)
    (Rendering|SetVisibility (Variables|Default|GetBPW_AKey) false false)))

(event Custom|Hide%20UI
  (if (< (Variables|Default|GetTimer) 0.0)
    (Rendering|SetVisibility (Variables|Default|GetBPW_AKey) false false)))

(event EventBeginPlay
  (bind _asbp_game_instance (Utilities|Casting|CastToBP_GameInstance (Game|GetGameInstance)))
  (Variables|References|SetAs%20BP%20Game%20Instance _asbp_game_instance)
  (Utilities|FlowControl|Delay 0.1)
  (UserInterface|SetWidget (Variables|Default|GetWB_Dialogue) (Variables|/Game/Blueprints/Components/BPC_DialogueManager.BPC_DialogueManager_C|GetWB_UIDialogue (Variables|Default|GetBPC_DialogueManager))))

(event EventUIInteract
  (Rendering|SetVisibility (Variables|Default|GetBPW_AKey) true false)
  (Variables|Default|SetTimer 0.1)
  (Utilities|Time|SetTimerbyEvent (delegate Custom|Hide%20UI) 0.2 true))

(event EventTick
  (params (DeltaSeconds :type Float%20%28single-precision%29))
  (bind _returnvalue (Game|GetPlayerCharacter 0))
  (bind _returnvalue_2 (Game|GetPlayerCameraManager 0))
  (bind _wb_dialogue (Variables|Default|GetWB_Dialogue))
  (bind _returnvalue_3 (Transformation|GetWorldLocation _wb_dialogue))
  (bind _returnvalue_4 (Camera|GetCameraLocation _returnvalue_2))
  ;[0.15 0.15 0.15 0.5] Le Widget de diaglogue du PNJ tourne par rapport au joueur
  (Variables|Default|SetDeltatime DeltaSeconds)
  (Utilities|IsValid _returnvalue
    (:Is%20Valid
      (Variables|Default|SetTimer (* (Variables|Default|GetDeltatime) (- (Variables|Default|GetTimer) (Variables|Default|GetDeltatime))))
      (Transformation|SetWorldLocation (Variables|Default|GetWB_Dialogue) (Math|Interpolation|VInterpTo (Transformation|GetWorldLocation (Variables|Default|GetWB_Dialogue)) (+ (Transformation|GetActorLocation) (* (Math|Vector|Normalize (- (Transformation|GetActorLocation _returnvalue) (Transformation|GetActorLocation))) (Variables|Default|GetDistance))) (Variables|Default|GetDeltatime) 3.0) false false)
      (Transformation|SetWorldRotation (Variables|Default|GetWB_Dialogue) (Math|Rotator|FindLookatRotation _returnvalue_3 (- _returnvalue_4 "0.000000,0.000000,10.000000")) false false)
      (Transformation|SetWorldScale3D (Variables|Default|GetWB_Dialogue) (Math|Conversions|ToVector(Float) (Math|Float|Clamp(Float) (/ (Math|Vector|Distance(Vector) _returnvalue_4 _returnvalue_3) 1e+03) 0.2 0.5))))))

(event EventOnInteract
  (params (ItemSlots :type Array%20of%20S%20Item%20Slot%20Structures) (PlayerRef :type BP%20Player%20Object%20Reference))
  ;[0.15 0.15 0.15 0.5] Quand le joueur intéragit avec le PNJ lance le dialogue et fait apparaitre le widget
  (if (not (Variables|/Game/Blueprints/Managers/BP_GameInstance.BP_GameInstance_C|GetNpcDispawn (Variables|References|GetAs%20BP%20Game%20Instance)))
    (if (Variables|Default|GetEndTalk)
      (Variables|Default|SetEndTalk false)
      (Default|DialogueAnim (Variables|/Game/Blueprints/Components/BPC_DialogueManager.BPC_DialogueManager_C|GetWB_UIDialogue (Variables|Default|GetBPC_DialogueManager)))
      (else
        (Default|OnInteract (Variables|Default|GetBPC_DialogueManager))))
    (Utilities|FlowControl|Delay 0.1)
    (Rendering|SetVisibility (Variables|Default|GetWB_Dialogue) true false)))

(fn ConstructionScript)

(fn StartWalkAnim
  (bind _mesh (Variables|Character|GetMesh))
  (switch Utilities|FlowControl|Switch|SwitchonENPC (Variables|Default|GetENPCType)
    (:NewEnumerator0
      (Components|Animation|PlayAnimation _mesh "/Game/Characters/Mannequins/Animations/Manny/Anim_Walking_Hunter.Anim_Walking_Hunter" true))
    (:NewEnumerator1
      (Components|Animation|PlayAnimation _mesh "/Game/Characters/Mannequins/Animations/Manny/Anim_Walking_Thieft.Anim_Walking_Thieft" true :!label _label))
    (:NewEnumerator2
      (Components|Animation|PlayAnimation _mesh "/Game/Characters/Mannequins/Animations/Manny/Anim_Female_Walk.Anim_Female_Walk" true))
    (:NewEnumerator3
      (goto _label))
    (:NewEnumerator4
      (Components|Animation|PlayAnimation _mesh "/Game/Characters/Mannequins/Animations/Manny/Anim_Walking_AnimLady.Anim_Walking_AnimLady" true))))

(fn StartIdleAnim)

(fn StartTurnAnim)

(fn StartGrabAnim)

(fn FocusTarget
  (return ""))