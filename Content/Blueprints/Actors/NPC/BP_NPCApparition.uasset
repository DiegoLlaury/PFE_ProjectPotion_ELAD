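; BP_NPCApparition spawns a Jester NPC near a door and walks it in along a spline on BeginPlay.
; The NPCAnim timeline advances spline distance by speed and delta time, moving the NPC's capsule with hard-coded offsets.
; EndAnim reverses the timeline with negative speed and a half-turn yaw to walk the NPC back.
; BeginPlay also binds to the NPC dialogue's EndQuestPotion event.
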(event Custom|PlayAnim
  (Variables|Default|SetSplineSpeed 3e+02)
  (Timeline|NPCAnim Play
    (:Update
      (Variables|Default|SetDistanceAlongSpline (+ (* (stale EventTick DeltaSeconds) (Variables|Default|GetSplineSpeed)) (Variables|Default|GetDistanceAlongSpline)))
      (Transformation|SetRelativeTransform (Variables|/Script/Engine.Character|GetCapsuleComponent (Variables|Default|GetCurrentNPC)) (Math|Transform|MakeTransform (Math|Vector|MakeVector (- (.x (.location (Spline|GetTransformatDistanceAlongSpline (Variables|Default|GetSpline) (Variables|Default|GetDistanceAlongSpline) "Local" false))) 9e+02) (- (.y (.location (Spline|GetTransformatDistanceAlongSpline (Variables|Default|GetSpline) (Variables|Default|GetDistanceAlongSpline) "Local" false))) 5e+02) (+ (.z (.location (Spline|GetTransformatDistanceAlongSpline (Variables|Default|GetSpline) (Variables|Default|GetDistanceAlongSpline) "Local" false))) 4e+01)) (Math|Rotator|MakeRotator (.roll (.rotation (Spline|GetTransformatDistanceAlongSpline (Variables|Default|GetSpline) (Variables|Default|GetDistanceAlongSpline) "Local" false))) (.pitch (.rotation (Spline|GetTransformatDistanceAlongSpline (Variables|Default|GetSpline) (Variables|Default|GetDistanceAlongSpline) "Local" false))) (+ (.yaw (.rotation (Spline|GetTransformatDistanceAlongSpline (Variables|Default|GetSpline) (Variables|Default|GetDistanceAlongSpline) "Local" false))) (Variables|Default|GetRotationCharac))) (Variables|/Script/Engine.SceneComponent|GetRelativeScale3D (Variables|Default|GetBP_NPC))) false false))))

(event Custom|EndAnim
  (Variables|Default|SetSplineSpeed -3e+02)
  (Variables|Default|SetRotationCharac 1.8e+02)
  (Timeline|NPCAnim ReverseFromEnd
    (:Update
      (Variables|Default|SetDistanceAlongSpline (+ (* (stale EventTick DeltaSeconds) (Variables|Default|GetSplineSpeed)) (Variables|Default|GetDistanceAlongSpline)))
      (Transformation|SetRelativeTransform (Variables|/Script/Engine.Character|GetCapsuleComponent (Variables|Default|GetCurrentNPC)) (Math|Transform|MakeTransform (Math|Vector|MakeVector (- (.x (.location (Spline|GetTransformatDistanceAlongSpline (Variables|Default|GetSpline) (Variables|Default|GetDistanceAlongSpline) "Local" false))) 9e+02) (- (.y (.location (Spline|GetTransformatDistanceAlongSpline (Variables|Default|GetSpline) (Variables|Default|GetDistanceAlongSpline) "Local" false))) 5e+02) (+ (.z (.location (Spline|GetTransformatDistanceAlongSpline (Variables|Default|GetSpline) (Variables|Default|GetDistanceAlongSpline) "Local" false))) 4e+01)) (Math|Rotator|MakeRotator (.roll (.rotation (Spline|GetTransformatDistanceAlongSpline (Variables|Default|GetSpline) (Variables|Default|GetDistanceAlongSpline) "Local" false))) (.pitch (.rotation (Spline|GetTransformatDistanceAlongSpline (Variables|Default|GetSpline) (Variables|Default|GetDistanceAlongSpline) "Local" false))) (+ (.yaw (.rotation (Spline|GetTransformatDistanceAlongSpline (Variables|Default|GetSpline) (Variables|Default|GetDistanceAlongSpline) "Local" false))) (Variables|Default|GetRotationCharac))) (Variables|/Script/Engine.SceneComponent|GetRelativeScale3D (Variables|Default|GetBP_NPC))) false false))))

(event EventBeginPlay
  (bind _door (Variables|Default|GetDoor))
  (bind _returnvalue (Transformation|GetRelativeTransform _door))
  (bind _returnvalue_2 (Game|SpawnActorfromClass "/Game/Blueprints/Actors/NPC/BP_NPC_Jester.BP_NPC_Jester_C" (Math|Transform|MakeTransform (Math|Vector|MakeVector (.x (.location _returnvalue)) (- (.y (.location _returnvalue)) 1e+02) (.z (.location _returnvalue))) "0, 0, 0" "1.000000,1.000000,1.000000") "Undefined" "MultiplyWithRoot" 0 0))
  (Variables|Default|SetCurrentNPC _returnvalue_2)
  (EventDispatchers|BindEventtoEndQuestPotion (Variables|/Game/Blueprints/Actors/NPC/BP_NPC.BP_NPC_C|GetBPC_Dialogue (Variables|Default|GetCurrentNPC)) (EventDispatchers|CreateEvent :!event Custom|EndAnim))
  (CallFunction|PlayAnim))

(event Collision|EventActorBeginOverlap
  (params (OtherActor :type Actor%20Object%20Reference)))

(event EventTick
  (params (DeltaSeconds :type Float%20%28single-precision%29)))

(fn ConstructionScript)