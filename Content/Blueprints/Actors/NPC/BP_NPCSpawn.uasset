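; Shop NPC spawner that brings the night's characters in and out one at a time, in GameInstance list order.
; It spawns each from DT_NPCData, configuring dialogue and reaction.
; A timeline advances the NPC along a spline using speed and Tick delta, then reverses for departure, alongside interpolated door animations.
; After departure it destroys the NPC and spawns the next, triggering end-of-night HUD and blink when none remain.
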(event Custom|PlayAnim
  (bind _bp_game_instance_ref (Variables|References|GetBP_Game_Instance_Ref))
  (bind _current_npc_ref (Variables|References|GetCurrent_NPC_Ref))
  (bind _current_npc_ref_2 (Variables|References|GetCurrent_NPC_Ref))
  (bind _bp_game_instance_ref_2 (Variables|References|GetBP_Game_Instance_Ref))
  ;[0.15 0.15 0.15 0.5] Gère l'activation de l'animation
  (Variables|Value|SetSplineSpeed 2.5e+02)
  (if (Variables|/Game/Blueprints/Managers/BP_GameInstance.BP_GameInstance_C|GetIsNPCInShop _bp_game_instance_ref)
    (Default|StartIdleAnim _current_npc_ref)
    (Variables|Value|SetDistanceAlongSpline 1e+03)
    ;[0.15 0.15 0.15 0.5] Réalise l'animation du PNJ entrant et sortant de la boutique
    (Transformation|SetRelativeTransform (Variables|/Script/Engine.Character|GetCapsuleComponent (Variables|References|GetCurrent_NPC_Ref)) (Math|Transform|MakeTransform (Math|Vector|MakeVector (.x (.location (Spline|GetTransformatDistanceAlongSpline (Variables|Default|GetSpline) (Variables|Value|GetDistanceAlongSpline) "World" false))) (.y (.location (Spline|GetTransformatDistanceAlongSpline (Variables|Default|GetSpline) (Variables|Value|GetDistanceAlongSpline) "World" false))) (- (.z (.location (Spline|GetTransformatDistanceAlongSpline (Variables|Default|GetSpline) (Variables|Value|GetDistanceAlongSpline) "World" false))) 2e+01)) (Math|Rotator|MakeRotator (.roll (.rotation (Spline|GetTransformatDistanceAlongSpline (Variables|Default|GetSpline) (Variables|Value|GetDistanceAlongSpline) "World" false))) (.pitch (.rotation (Spline|GetTransformatDistanceAlongSpline (Variables|Default|GetSpline) (Variables|Value|GetDistanceAlongSpline) "World" false))) (+ (.yaw (.rotation (Spline|GetTransformatDistanceAlongSpline (Variables|Default|GetSpline) (Variables|Value|GetDistanceAlongSpline) "World" false))) (Variables|Value|GetRotationCharac))) "1.000000,1.000000,1.000000") false false :!label _label)
    (else
      (Default|StartWalkAnim _current_npc_ref)
      (Variables|/Game/Blueprints/Managers/BP_GameInstance.BP_GameInstance_C|SetIsNPCInShop _bp_game_instance_ref true)
      (Variables|Value|SetDistanceAlongSpline 0.0)
      (CallFunction|AnimDoorOpen)
      (Timeline|NPCAnim Play
        (:Update
          (Variables|Value|SetDistanceAlongSpline (+ (* (stale EventTick DeltaSeconds) (Variables|Value|GetSplineSpeed)) (Variables|Value|GetDistanceAlongSpline)))
          (goto _label))
        (:Finished
          ;[0.15 0.15 0.15 0.5] Fait disparaitre le PNJ et réapparaitre le suivant
          (if (Variables|/Game/Blueprints/Managers/BP_GameInstance.BP_GameInstance_C|GetNpcDispawn (Variables|References|GetBP_Game_Instance_Ref))
            (Actor|DestroyActor _current_npc_ref_2)
            (Math|Integer|IncrementInt (Variables|/Game/Blueprints/Managers/BP_GameInstance.BP_GameInstance_C|GetCurrentNPC (Variables|References|GetBP_Game_Instance_Ref))
              (:%20%20
                (Variables|Value|SetRotationCharac 0.0)
                (Variables|/Game/Blueprints/Managers/BP_GameInstance.BP_GameInstance_C|SetNpcDispawn _bp_game_instance_ref_2 false)
                (Variables|/Game/Blueprints/Managers/BP_GameInstance.BP_GameInstance_C|SetIsNPCInShop _bp_game_instance_ref_2 false)
                (Variables|/Game/Blueprints/Managers/BP_GameInstance.BP_GameInstance_C|SetNightFinished _bp_game_instance_ref_2 true)
                (Utilities|FlowControl|Delay 1.0)
                (CallFunction|SpawnNextNPC)))
            (else
              (Default|StartIdleAnim _current_npc_ref_2))))))))

(event Custom|EndAnim
  (bind _current_npc_ref (Variables|References|GetCurrent_NPC_Ref))
  (bind _bp_game_instance_ref (Variables|References|GetBP_Game_Instance_Ref))
  ;[0.15 0.15 0.15 0.5] Gère l'activation de l'animation
  (Default|StartWalkAnim (Variables|References|GetCurrent_NPC_Ref))
  (Variables|Value|SetSplineSpeed -2.5e+02)
  (Variables|Value|SetRotationCharac 1.8e+02)
  (Variables|/Game/Blueprints/Managers/BP_GameInstance.BP_GameInstance_C|SetIsNPCInShop (Variables|References|GetBP_Game_Instance_Ref) false)
  (Variables|/Game/Blueprints/Managers/BP_GameInstance.BP_GameInstance_C|SetNpcDispawn (Variables|References|GetBP_Game_Instance_Ref) true)
  (Utilities|FlowControl|Sequence
    (:then_0
      ;[0.15 0.15 0.15 0.5] Réalise l'animation du PNJ entrant et sortant de la boutique
      (Timeline|NPCAnim ReverseFromEnd
        (:Update
          (Variables|Value|SetDistanceAlongSpline (+ (* (stale EventTick DeltaSeconds) (Variables|Value|GetSplineSpeed)) (Variables|Value|GetDistanceAlongSpline)))
          (Transformation|SetRelativeTransform (Variables|/Script/Engine.Character|GetCapsuleComponent (Variables|References|GetCurrent_NPC_Ref)) (Math|Transform|MakeTransform (Math|Vector|MakeVector (.x (.location (Spline|GetTransformatDistanceAlongSpline (Variables|Default|GetSpline) (Variables|Value|GetDistanceAlongSpline) "World" false))) (.y (.location (Spline|GetTransformatDistanceAlongSpline (Variables|Default|GetSpline) (Variables|Value|GetDistanceAlongSpline) "World" false))) (- (.z (.location (Spline|GetTransformatDistanceAlongSpline (Variables|Default|GetSpline) (Variables|Value|GetDistanceAlongSpline) "World" false))) 2e+01)) (Math|Rotator|MakeRotator (.roll (.rotation (Spline|GetTransformatDistanceAlongSpline (Variables|Default|GetSpline) (Variables|Value|GetDistanceAlongSpline) "World" false))) (.pitch (.rotation (Spline|GetTransformatDistanceAlongSpline (Variables|Default|GetSpline) (Variables|Value|GetDistanceAlongSpline) "World" false))) (+ (.yaw (.rotation (Spline|GetTransformatDistanceAlongSpline (Variables|Default|GetSpline) (Variables|Value|GetDistanceAlongSpline) "World" false))) (Variables|Value|GetRotationCharac))) "1.000000,1.000000,1.000000") false false))
        (:Finished
          ;[0.15 0.15 0.15 0.5] Fait disparaitre le PNJ et réapparaitre le suivant
          (if (Variables|/Game/Blueprints/Managers/BP_GameInstance.BP_GameInstance_C|GetNpcDispawn (Variables|References|GetBP_Game_Instance_Ref))
            (Actor|DestroyActor _current_npc_ref)
            (Math|Integer|IncrementInt (Variables|/Game/Blueprints/Managers/BP_GameInstance.BP_GameInstance_C|GetCurrentNPC (Variables|References|GetBP_Game_Instance_Ref))
              (:%20%20
                (Variables|Value|SetRotationCharac 0.0)
                (Variables|/Game/Blueprints/Managers/BP_GameInstance.BP_GameInstance_C|SetNpcDispawn _bp_game_instance_ref false)
                (Variables|/Game/Blueprints/Managers/BP_GameInstance.BP_GameInstance_C|SetIsNPCInShop _bp_game_instance_ref false)
                (Variables|/Game/Blueprints/Managers/BP_GameInstance.BP_GameInstance_C|SetNightFinished _bp_game_instance_ref true)
                (Utilities|FlowControl|Delay 1.0)
                (CallFunction|SpawnNextNPC)))
            (else
              (Default|StartIdleAnim _current_npc_ref))))))
    (:then_1
      (Default|RemoveReaction (Variables|References|GetCurrent_NPC_Ref))
      (Utilities|FlowControl|Delay 1.25)
      (CallFunction|AnimDoorOpen))))

(event Custom|AnimDoorOpen
  (bind _door (Variables|Default|GetDoor))
  (Variables|Default|SetDoorOpen true)
  (Timeline|AnimDoorTM PlayFromStart
    (:Update
      (Transformation|SetRelativeRotation _door (Math|Interpolation|RInterpTo (Variables|/Script/Engine.SceneComponent|GetRelativeRotation _door) "0, 0, 0" (Variables|Value|GetDelta%20Seconds) (Math|Float|MakeLiteralFloat 2.0)) false false))
    (:Finished
      (if (Variables|Default|GetDoorOpen)
        (Utilities|FlowControl|Delay 0.75)
        (Variables|Default|SetDoorOpen false)
        (CallFunction|AnimDoorShut)))))

(event Custom|AnimDoorShut
  (Timeline|Timeline PlayFromStart
    (:Update
      (Transformation|SetRelativeRotation (Variables|Default|GetDoor) (Math|Interpolation|RInterpTo (Variables|/Script/Engine.SceneComponent|GetRelativeRotation (Variables|Default|GetDoor)) "0.000000,-90.000000,0.000000" (Variables|Value|GetDelta%20Seconds) (Math|Float|MakeLiteralFloat 2.0)) false false))
    (:Finished
      (if (Variables|Default|GetDoorOpen)
        (Utilities|FlowControl|Delay 0.75)
        (CallFunction|AnimDoorOpen)
        (Variables|Default|SetDoorOpen false)))))

(event EventBeginPlay
  (bind _asbp_game_instance (Utilities|Casting|CastToBP_GameInstance (Game|GetGameInstance)))
  (Variables|References|SetBP_Game_Instance_Ref _asbp_game_instance)
  (bind _asbp_game_controller (Utilities|Casting|CastToBP_GameController (Game|GetPlayerController 0)))
  (Variables|References|SetAs%20BP%20Game%20Controller _asbp_game_controller)
  (bind _asbp_player (Utilities|Casting|CastToBP_Player (Game|Player|GetPlayerPawn 0)))
  (Variables|References|SetAs%20BP%20Player _asbp_player)
  (Utilities|FlowControl|Delay 0.1)
  (Variables|Default|SetRelative%20Rotation%20Door (Variables|/Script/Engine.SceneComponent|GetRelativeRotation (Variables|Default|GetDoor)))
  (CallFunction|SpawnNextNPC))

(event EventTick
  (params (DeltaSeconds :type Float%20%28single-precision%29))
  (Variables|Value|SetDelta%20Seconds DeltaSeconds))

(fn ConstructionScript)

(fn SpawnNextNPC
  (bind _bp_game_instance_ref (Variables|References|GetBP_Game_Instance_Ref))
  (bind _bp_game_instance_ref_2 (Variables|References|GetBP_Game_Instance_Ref))
  (bind _door (Variables|Default|GetDoor))
  (bind _bp_game_instance_ref_3 (Variables|References|GetBP_Game_Instance_Ref))
  (bind _returnvalue (Transformation|GetRelativeTransform _door))
  (bind _npcfornight_ (Variables|/Game/Blueprints/Managers/BP_GameInstance.BP_GameInstance_C|GetNPCForNight%20 _bp_game_instance_ref))
  (bind _ereaction (Variables|/Game/Blueprints/Managers/BP_GameInstance.BP_GameInstance_C|GetEReaction _bp_game_instance_ref_2))
  (bind _currentnpc (Variables|/Game/Blueprints/Managers/BP_GameInstance.BP_GameInstance_C|GetCurrentNPC _bp_game_instance_ref))
  ;[0.15 0.15 0.15 0.5] Permet de faire apparaitre les PNJ automatiquement par rapport à la liste donné par la game instance
  (if (>= (Utilities|Array|Length _npcfornight_) (+ _currentnpc 1))
    (bind _returnvalue_2 (Utilities|GetDataTableRow "/Game/Data/Datatables/DT_NPCData.DT_NPCData" (Utilities|String|StringToName (Utilities|String|ToString(Integer) (Utilities|Array|Get(acopy) _npcfornight_ _currentnpc))))
      (:then
        (bind _returnvalue_3 (Game|SpawnActorfromClass (.NPC_BP (Utilities|Struct|BreakSNPCData _returnvalue_2)) (Math|Transform|MakeTransform (Math|Vector|MakeVector (.x (.location _returnvalue)) (- (.y (.location _returnvalue)) 1e+02) (.z (.location _returnvalue))) "0, 0, 0" "1.000000,1.000000,1.000000") "Undefined" "MultiplyWithRoot" 0 0))
        (Variables|References|SetCurrent_NPC_Ref _returnvalue_3)
        (Utilities|FlowControl|Sequence
          (:then_0
            (Variables|/Game/Blueprints/Components/BPC_DialogueManager.BPC_DialogueManager_C|SetGetDialogueData (Variables|/Game/Blueprints/Actors/NPC/BP_NPC.BP_NPC_C|GetBPC_DialogueManager (Variables|References|GetCurrent_NPC_Ref)) (.DataTableDialogue (Utilities|Struct|BreakSNPCData _returnvalue_2)))
            (Variables|/Game/Blueprints/Components/BPC_DialogueManager.BPC_DialogueManager_C|SetCharacter%20Index (Variables|/Game/Blueprints/Actors/NPC/BP_NPC.BP_NPC_C|GetBPC_DialogueManager (Variables|References|GetCurrent_NPC_Ref)) (.Index (Utilities|Struct|BreakSNPCData _returnvalue_2)))
            (Variables|/Game/Blueprints/Components/BPC_DialogueManager.BPC_DialogueManager_C|SetCurrentReaction (Variables|/Game/Blueprints/Actors/NPC/BP_NPC.BP_NPC_C|GetBPC_DialogueManager (Variables|References|GetCurrent_NPC_Ref)) (Variables|/Game/Blueprints/Managers/BP_GameInstance.BP_GameInstance_C|GetCurrentNPCReaction _bp_game_instance_ref_2))
            (Variables|/Game/Blueprints/Components/BPC_DialogueManager.BPC_DialogueManager_C|SetCurrentEnumReaction (Variables|/Game/Blueprints/Actors/NPC/BP_NPC.BP_NPC_C|GetBPC_DialogueManager (Variables|References|GetCurrent_NPC_Ref)) _ereaction)
            (bind _dialogueindex (Default|SetupNPCLine (Variables|References|GetBP_Game_Instance_Ref) (.Index (Utilities|Struct|BreakSNPCData _returnvalue_2))))
            (bind _getnpcdialogue (Default|GetSDialogueData (Variables|/Game/Blueprints/Actors/NPC/BP_NPC.BP_NPC_C|GetBPC_DialogueManager (Variables|References|GetCurrent_NPC_Ref)) _dialogueindex))
            (if (.bIsReacting (Utilities|Struct|BreakSNPCDialogue _getnpcdialogue))
              (Variables|/Game/Blueprints/Managers/BP_GameInstance.BP_GameInstance_C|SetNPCIsReacting (Variables|References|GetBP_Game_Instance_Ref) true)))
          (:then_1
            (EventDispatchers|BindEventtoEndQuestPotion (Variables|/Game/Blueprints/Actors/NPC/BP_NPC.BP_NPC_C|GetBPC_DialogueManager (Variables|References|GetCurrent_NPC_Ref)) (EventDispatchers|CreateEvent :!event DispawnCurrentNPC))
            (CallFunction|PlayAnim)
            (if (Variables|/Game/Blueprints/Managers/BP_GameInstance.BP_GameInstance_C|GetNPCIsReacting (Variables|References|GetBP_Game_Instance_Ref))
              (Default|SetReaction (Variables|References|GetCurrent_NPC_Ref) _ereaction))))))
    (else
      (Development|PrintString "End of Night")
      (Variables|/Game/Blueprints/Managers/BP_GameInstance.BP_GameInstance_C|SetNightFinished _bp_game_instance_ref_3 true)
      (Variables|/Game/Blueprints/Managers/BP_GameInstance.BP_GameInstance_C|SetNpcDispawn _bp_game_instance_ref_3 false)
      (Default|BlinkEffect (Variables|References|GetAs%20BP%20Player))
      (Default|EndOfNight (Variables|/Game/Blueprints/Managers/BP_GameController.BP_GameController_C|GetWB_InfoHUD (Variables|References|GetAs%20BP%20Game%20Controller))))))

(fn DispawnCurrentNPC
  ;[0.15 0.15 0.15 0.5] Fait disparaitre le PNJ
  (CallFunction|EndAnim))