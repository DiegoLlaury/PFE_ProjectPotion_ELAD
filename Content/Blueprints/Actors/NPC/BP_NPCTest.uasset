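; BP_NPCTest is a test NPC that shows dialogue when interacted with.
; The first Interact creates a WB_DataTableDialogue widget, adds it to the viewport and sets a Talking flag, so later interactions reuse that widget.
; Each interaction calls the widget's Talk and then increments its DialogueIndex.
; Talking is never cleared here, and FocusTarget returns an empty string.
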(event Custom|Talk
  (bind _ui (Variables|Default|GetUI))
  (Default|Talk _ui)
  (Math|Integer|IncrementInt (Variables|/Game/Blueprints/Actors/NPC/WB_DataTableDialogue.WB_DataTableDialogue_C|GetDialogueIndex _ui)))

(event EventInteract
  (params (Interactor :type BP%20My%20Controller%20Object%20Reference))
  (if (Variables|Default|GetTalking?)
    (CallFunction|Talk)
    (else
      (bind _returnvalue (UserInterface|CreateWidget "/Game/Blueprints/Actors/NPC/WB_DataTableDialogue.WB_DataTableDialogue_C"))
      (bind _output_get (Variables|Default|SetUI _returnvalue))
      (UserInterface|Viewport|AddtoViewport _output_get 0)
      (Variables|Default|SetTalking? true)
      (CallFunction|Talk))))

(fn ConstructionScript)

(fn FocusTarget
  (return ""))