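; Base NPC actor that shows data-table dialogue in a widget and can ask the player for an item.
; Each interaction advances the row index until a row needs a potion, after which interacting opens the player's inventory.
; While the player is in range of an already talking NPC, it binds to item use.
; Item detection matches ingredient IDs to dialogue options, jumps to that row and removes the item.
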(event OnComponentEndOverlap(DetectPlayer)
  (params (OverlappedComponent :type Primitive%20Component%20Object%20Reference) (OtherActor :type Actor%20Object%20Reference) (OtherComp :type Primitive%20Component%20Object%20Reference) (OtherBodyIndex :type Integer))
  (Variables|/Game/Blueprints/Components/BPC_Inventory.BPC_Inventory_C|SetIsaPNJ (Variables|/Game/Blueprints/Managers/BP_MyController.BP_MyController_C|GetBPC_Inventory (Variables|Default|GetAs%20BP%20My%20Controller)) false)
  (EventDispatchers|UnbindEventfromOnUseItem (Variables|/Game/Blueprints/Managers/BP_MyController.BP_MyController_C|GetBPC_Inventory (Variables|Default|GetAs%20BP%20My%20Controller)) (EventDispatchers|CreateEvent :!event Custom|ItemDetection))
  (Rendering|SetVisibility (Variables|Default|GetDialogue) false false))

(event OnComponentBeginOverlap(DetectPlayer)
  (params (OverlappedComponent :type Primitive%20Component%20Object%20Reference) (OtherActor :type Actor%20Object%20Reference) (OtherComp :type Primitive%20Component%20Object%20Reference) (OtherBodyIndex :type Integer) (bFromSweep :type Boolean) (SweepResult :type Hit%20Result%20Structure%20%28by%20ref%29))
  (if (Variables|Default|GetTalking?)
    (Variables|/Game/Blueprints/Components/BPC_Inventory.BPC_Inventory_C|SetIsaPNJ (Variables|/Game/Blueprints/Managers/BP_MyController.BP_MyController_C|GetBPC_Inventory (Variables|Default|GetAs%20BP%20My%20Controller)) true)
    (EventDispatchers|BindEventtoOnUseItem (Variables|/Game/Blueprints/Managers/BP_MyController.BP_MyController_C|GetBPC_Inventory (Variables|Default|GetAs%20BP%20My%20Controller)) (EventDispatchers|CreateEvent :!event Custom|ItemDetection))
    (Rendering|SetVisibility (Variables|Default|GetDialogue) true false)))

(event Custom|UpdateTalk
  (params (LineNumber :type Name))
  (bind _out_row_need_potion_ (Default|NextTalk (Variables|Default|GetUI) LineNumber))
  (if _out_row_need_potion_
    (Variables|/Game/Blueprints/Components/BPC_Inventory.BPC_Inventory_C|SetNeedObject%20 (Variables|/Game/Blueprints/Managers/BP_MyController.BP_MyController_C|GetBPC_Inventory (Variables|Default|GetAs%20BP%20My%20Controller)) true)
    (elif (not (Variables|/Game/Blueprints/Components/BPC_Inventory.BPC_Inventory_C|GetNeedObject%20 (Variables|/Game/Blueprints/Managers/BP_MyController.BP_MyController_C|GetBPC_Inventory (Variables|Default|GetAs%20BP%20My%20Controller))))
      (Math|Integer|IncrementInt (Variables|Default|GetDialogueIndex)))))

(event Custom|ItemDetection
  (params (IngredientData :type S%20Ingredient%20Structure) (Index :type Integer))
  (bind _as_bp_my_controller (Variables|Default|GetAs%20BP%20My%20Controller))
  (bind _bpc_inventory (Variables|/Game/Blueprints/Managers/BP_MyController.BP_MyController_C|GetBPC_Inventory _as_bp_my_controller))
  (bind _returnvalue (Utilities|GetDataTableRow "/Game/Data/Datatables/DT_Dialogue.DT_Dialogue" (Utilities|Array|Get(acopy) (Variables|Default|GetLines) (Variables|Default|GetDialogueIndex)))
    (:then
      (for _array_element (.opendialogueoptions _returnvalue)
        (if (== (.ingredientneed _array_element) (.ID (Utilities|Struct|BreakSIngredient IngredientData)))
          (CallFunction|UpdateTalk (.row _array_element))
          (Variables|/Game/Blueprints/Components/BPC_Inventory.BPC_Inventory_C|SetNeedObject%20 _bpc_inventory false)
          (Default|RemoveItemUsed _bpc_inventory Index)
          (else
            (Development|PrintString "N'est pas pareil")))))))

(event EventOnInteract
  (params (ItemSlots :type Array%20of%20S%20Item%20Slot%20Structures))
  (if (Variables|/Game/Blueprints/Components/BPC_Inventory.BPC_Inventory_C|GetNeedObject%20 (Variables|/Game/Blueprints/Managers/BP_MyController.BP_MyController_C|GetBPC_Inventory (Variables|Default|GetAs%20BP%20My%20Controller)))
    (Default|AutomaticOpenInventory (Variables|Default|GetAs%20BP%20My%20Controller))
    (elif (Variables|Default|GetTalking?)
      (CallFunction|UpdateTalk (Utilities|Array|Get(acopy) (Variables|Default|GetLines) (Variables|Default|GetDialogueIndex)))
      (else
        (Variables|Default|SetTalking? true)
        (Rendering|SetVisibility (Variables|Default|GetDialogue) true false)
        (CallFunction|UpdateTalk (Utilities|Array|Get(acopy) (Variables|Default|GetLines) (Variables|Default|GetDialogueIndex)))))))

(event EventBeginPlay
  (bind _asbp_my_controller (Utilities|Casting|CastToBP_MyController (Game|GetPlayerController 0)))
  (Variables|Default|SetAs%20BP%20My%20Controller _asbp_my_controller)
  (bind _returnvalue (UserInterface|CreateWidget "/Game/Widgets/HUD/WB_DataTableDialogue.WB_DataTableDialogue_C"))
  (bind _output_get (Variables|Default|SetUI _returnvalue))
  (UserInterface|SetWidget (Variables|Default|GetDialogue) _output_get)
  (bind _outrownames (DataTable|GetDataTableRowNames (.datatable (Variables|/Game/Blueprints/Components/BPC_Dialogue.BPC_Dialogue_C|GetDialogueData (Variables|Default|GetBPC_Dialogue)))))
  (Variables|Default|SetLines _outrownames)
  (Variables|Default|SetDialogueIndex (Utilities|Array|FindItem (Variables|Default|GetLines) (.rowname (Variables|/Game/Blueprints/Components/BPC_Dialogue.BPC_Dialogue_C|GetDialogueData (Variables|Default|GetBPC_Dialogue))))))

(fn ConstructionScript)

(fn FocusTarget
  (return ""))