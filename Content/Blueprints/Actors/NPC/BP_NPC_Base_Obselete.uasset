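; Base NPC actor, named as obsolete, that offers dialogue and reacts to inventory items the player uses nearby.
; BPCDialogue handles interaction and supplies the world-space dialogue widget, which turns to the camera and scales with distance within clamped limits each tick.
; Entering the detection volume mid-conversation shows the widget and binds the player inventory's use-item event, passing ingredients to the dialogue component; leaving hides and unbinds it.
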(event OnComponentEndOverlap(DetectPlayer)
  (params (OverlappedComponent :type Primitive%20Component%20Object%20Reference) (OtherActor :type Actor%20Object%20Reference) (OtherComp :type Primitive%20Component%20Object%20Reference) (OtherBodyIndex :type Integer))
  (Variables|/Game/Blueprints/Components/BPC_Inventory.BPC_Inventory_C|SetIsANPC? (Variables|/Game/Blueprints/Managers/BP_MyController.BP_MyController_C|GetBPC_Inventory (Variables|Default|GetAs%20BP%20My%20Controller)) false)
  (EventDispatchers|UnbindEventfromOnUseItem (Variables|/Game/Blueprints/Managers/BP_MyController.BP_MyController_C|GetBPC_Inventory (Variables|Default|GetAs%20BP%20My%20Controller)) (EventDispatchers|CreateEvent :!event Custom|ItemDetection))
  (Rendering|SetVisibility (Variables|Default|GetWB_Dialogue) false false))

(event OnComponentBeginOverlap(DetectPlayer)
  (params (OverlappedComponent :type Primitive%20Component%20Object%20Reference) (OtherActor :type Actor%20Object%20Reference) (OtherComp :type Primitive%20Component%20Object%20Reference) (OtherBodyIndex :type Integer) (bFromSweep :type Boolean) (SweepResult :type Hit%20Result%20Structure%20%28by%20ref%29))
  (if (Variables|/Game/Blueprints/Components/BPC_DialogueManager.BPC_DialogueManager_C|GetIsTalking? (Variables|Default|GetBPC_Dialogue))
    (Variables|/Game/Blueprints/Components/BPC_Inventory.BPC_Inventory_C|SetIsANPC? (Variables|/Game/Blueprints/Managers/BP_MyController.BP_MyController_C|GetBPC_Inventory (Variables|Default|GetAs%20BP%20My%20Controller)) true)
    (EventDispatchers|BindEventtoOnUseItem (Variables|/Game/Blueprints/Managers/BP_MyController.BP_MyController_C|GetBPC_Inventory (Variables|Default|GetAs%20BP%20My%20Controller)) (EventDispatchers|CreateEvent :!event Custom|ItemDetection))
    (Rendering|SetVisibility (Variables|Default|GetWB_Dialogue) true false)))

(event Custom|ItemDetection
  (params (IngredientData :type S%20Ingredient%20Structure) (Index :type Integer))
  (Default|ItemDetection (Variables|Default|GetBPC_Dialogue) IngredientData Index))

(event EventOnInteract
  (params (ItemSlots :type Array%20of%20S%20Item%20Slot%20Structures))
  (bind _talking_ (Default|OnInteract (Variables|Default|GetBPC_Dialogue)))
  (if _talking_
    (Rendering|SetVisibility (Variables|Default|GetWB_Dialogue) true false)))

(event EventTick
  (params (DeltaSeconds :type Float%20%28single-precision%29))
  (bind _returnvalue (Game|GetPlayerCameraManager 0))
  (bind _wb_dialogue (Variables|Default|GetWB_Dialogue))
  (bind _returnvalue_2 (Camera|GetCameraLocation _returnvalue))
  (bind _returnvalue_3 (Transformation|GetWorldLocation _wb_dialogue))
  (Transformation|SetWorldRotation (Variables|Default|GetWB_Dialogue) (Math|Rotator|FindLookatRotation _returnvalue_3 _returnvalue_2) false false)
  (Transformation|SetWorldScale3D (Variables|Default|GetWB_Dialogue) (Math|Conversions|ToVector(Float) (Math|Float|Clamp(Float) (/ (Math|Vector|Distance(Vector) _returnvalue_2 _returnvalue_3) 1e+03) 0.5 1.5))))

(event EventBeginPlay
  (bind _asbp_my_controller (Utilities|Casting|CastToBP_MyController (Game|GetPlayerController 0)))
  (Variables|Default|SetAs%20BP%20My%20Controller _asbp_my_controller)
  (UserInterface|SetWidget (Variables|Default|GetWB_Dialogue) (Variables|/Game/Blueprints/Components/BPC_DialogueManager.BPC_DialogueManager_C|GetWB_UIDialogue (Variables|Default|GetBPC_Dialogue))))

(fn ConstructionScript)

(fn FocusTarget
  (return ""))