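; Cauldron workbench where the player brews potions from inventory ingredients.
; Interacting possesses the bench, swaps HUD and binds item use; added ingredients tally property counts and can be returned.
; Brewing eases the camera over the cauldron and opens a QTE widget.
; ProcessPotion matches the tally exactly against DT_Recipes, falls back to Random_Potion, then adds the potion to inventory and shows a result popup.
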(event Custom|LaunchCauldron
  (CallFunction|MoveCamera)
  (Default|RemoveHUD (Variables|Default|GetAs%20BP%20My%20Controller))
  (Utilities|FlowControl|Delay 0.3)
  (Variables|Default|SetQTEOn true)
  (bind _returnvalue (UserInterface|CreateWidget "/Game/Widgets/HUD/HUDWorkbench/WBP_QTEPotion.WBP_QTEPotion_C" 0 self))
  (bind _output_get (Variables|Default|SetQTEPotion _returnvalue))
  (UserInterface|Viewport|AddtoViewport _output_get 0))

(event Custom|OutlineDelay
  (if (< (Variables|Default|GetTimer) 0.0)
    (Default|ButtonDisappear (Variables|/Game/Blueprints/Managers/BP_GameController.BP_GameController_C|GetWB_InfoHUD (Variables|Reference|GetAs%20BP%20Game%20Controller)))
    (Rendering|Material|SetOverlayMaterial (Variables|Default|GetCauldron) "/Game/Materials/MI_ObjectOutlineFalse.MI_ObjectOutlineFalse" :!class /Script/Engine.MeshComponent)))

(event Custom|MoveCamera
  (bind _camera (Variables|Default|GetCamera))
  (Timeline|Timeline Play
    (:Update
      (Transformation|SetWorldLocation _camera (Math|Interpolation|VInterpTo (Transformation|GetWorldLocation _camera) (+ (Transformation|GetWorldLocation (Variables|Default|GetCauldron)) "0.000000,0.000000,200.000000") (Variables|Default|GetDelta%20Seconds) (Math|Float|MakeLiteralFloat 1e+01)) false false))))

(event Custom|ProcessPotion
  (bind _wbp_cauldron (Variables|Reference|GetWBP_Cauldron))
  (bind _wbp_cauldron_2 (Variables|Reference|GetWBP_Cauldron))
  ;[0.15 0.15 0.15 0.5] Systeme de Craft de Potion
  (Default|AutomaticHUDWorkbench (Variables|Default|GetAs%20BP%20My%20Controller) "NewEnumerator2")
  (Variables|Default|SetQTEOn false)
  (if (Utilities|Map|IsNotEmpty (Variables|Default|GetTempProperty))
    (Components|Activation|SetActive (Variables|Default|GetSmokePotion) false false)
    (bind _outrownames (DataTable|GetDataTableRowNames (Variables|Default|GetDT_Recipes)))
    (bind _array_element (Utilities|Array|ForEachLoopwithBreak _outrownames :!label _label)
      (:LoopBody
        (bind _returnvalue (Utilities|GetDataTableRow "/Game/Data/Datatables/DT_Recipes.DT_Recipes" _array_element)
          (:then
            (if (CallFunction|CompareMap (Variables|Default|GetTempProperty) (.ingredients _returnvalue))
              (Utilities|Map|Clear (Variables|Default|GetTempProperty))
              (Utilities|Array|Clear (Variables|Default|GetTempListSlot))
              (CallFunction|CreatePotionUI (.idresultingpotion _returnvalue))
              (Default|Pickup (Variables|/Game/Blueprints/Managers/BP_GameController.BP_GameController_C|GetBPC_Inventory (Variables|Default|GetAs%20BP%20My%20Controller)) (.idresultingpotion _returnvalue) 1 (Variables|/Game/Blueprints/Managers/BP_GameInstance.BP_GameInstance_C|GetInventorySlotsSave (Variables|Reference|GetAs%20BP%20Game%20Instance)))
              (Variables|Default|SetSuccessPotion true)
              (CallFunction|MoveCameraBase)
              (Default|RemoveImage _wbp_cauldron_2)
              (UserInterface|Viewport|AddtoViewport _wbp_cauldron_2 0)
              (goto _label Break)))))
      (:Completed
        (if (not (Variables|Default|GetSuccessPotion))
          (Utilities|Map|Clear (Variables|Default|GetTempProperty))
          (Utilities|Array|Clear (Variables|Default|GetTempListSlot))
          (Development|PrintString "Random Potion")
          (CallFunction|CreatePotionUI "Random_Potion")
          (Default|Pickup (Variables|/Game/Blueprints/Managers/BP_GameController.BP_GameController_C|GetBPC_Inventory (Variables|Default|GetAs%20BP%20My%20Controller)) "Random_Potion" 1 (Variables|/Game/Blueprints/Managers/BP_GameInstance.BP_GameInstance_C|GetInventorySlotsSave (Variables|Reference|GetAs%20BP%20Game%20Instance)))
          (Variables|Default|SetSuccessPotion false)
          (CallFunction|MoveCameraBase)
          (Default|RemoveImage _wbp_cauldron)
          (UserInterface|Viewport|AddtoViewport _wbp_cauldron 0))))))

(event Custom|MoveCameraBase
  (bind _camera (Variables|Default|GetCamera))
  (Timeline|Timeline_0 PlayFromStart
    (:Update
      (Transformation|SetWorldLocation _camera (Math|Interpolation|VInterpTo (Transformation|GetWorldLocation _camera) (Variables|Default|GetBaseCamPos) (Variables|Default|GetDelta%20Seconds) (Math|Float|MakeLiteralFloat 5.0)) false false))))

(event Input|EnhancedActionEvents|EnhancedInputActionIA_ActiveCauldron
  (params (ActionValue :type Boolean) (ElapsedSeconds :type Float%20%28double-precision%29) (TriggeredSeconds :type Float%20%28double-precision%29) (InputAction :type Input%20Action%20Object%20Reference :default "/Game/FirstPerson/Input/Actions/IA_ActiveCauldron.IA_ActiveCauldron"))
  (:Started
    (Variables|Default|SetTotalElement 0)
    (bind _values (Utilities|Map|Values (Variables|Default|GetTempProperty)))
    (for _array_element _values
      (Variables|Default|SetTotalElement (+ _array_element (Variables|Default|GetTotalElement))))
    (if (not (Variables|Default|GetQTEOn))
      (if (> (Variables|Default|GetTotalElement) 1)
        (Components|Activation|SetActive (Variables|Default|GetSmokePotion) true false)
        (CallFunction|LaunchCauldron)
        (Widget|RemovefromParent (Variables|Reference|GetWBP_Cauldron))))))

(event Input|EnhancedActionEvents|EnhancedInputActionIA_EscapeWorkbench
  (params (ActionValue :type Boolean) (ElapsedSeconds :type Float%20%28double-precision%29) (TriggeredSeconds :type Float%20%28double-precision%29) (InputAction :type Input%20Action%20Object%20Reference :default "/Game/FirstPerson/Input/Actions/IA_EscapeWorkbench.IA_EscapeWorkbench"))
  (bind _as_bp_my_controller (Variables|Default|GetAs%20BP%20My%20Controller))
  (:Started
    (if (Variables|Default|GetPotionUIIsOn)
      (Default|LeaveWidget (Variables|Default|GetWBP_PotionCreate))
      (Variables|Default|SetPotionUIIsOn false)
      (elif (not (Variables|Default|GetQTEOn))
        (CallFunction|QuitWorkbenchs)
        (Utilities|FlowControl|Delay 0.2)
        (EventDispatchers|UnbindEventfromOnUseItem (Variables|/Game/Blueprints/Managers/BP_GameController.BP_GameController_C|GetBPC_Inventory (Variables|Default|GetAs%20BP%20My%20Controller)) (EventDispatchers|CreateEvent :!event AddIngredientTemp))
        (Transformation|SetWorldLocation (Variables|Default|GetCamera) (Variables|Default|GetBaseCamPos) false false)
        (Pawn|Possess (Variables|Default|GetAs%20BP%20My%20Controller) (Variables|Default|GetAs%20BP%20Player))
        (Variables|/Game/Blueprints/Managers/BP_GameController.BP_GameController_C|SetIsOnWorkbench _as_bp_my_controller false)
        (Default|RemoveHUDTest _as_bp_my_controller)
        (Widget|RemovefromParent (Variables|Reference|GetWBP_Cauldron))))))

(event Input|EnhancedActionEvents|EnhancedInputActionIA_RemoveItemFromCauldron
  (params (ActionValue :type Boolean) (ElapsedSeconds :type Float%20%28double-precision%29) (TriggeredSeconds :type Float%20%28double-precision%29) (InputAction :type Input%20Action%20Object%20Reference :default "/Game/FirstPerson/Input/Actions/IA_RemoveItemFromCauldron.IA_RemoveItemFromCauldron"))
  (:Started
    (if (not (Variables|Default|GetQTEOn))
      (CallFunction|GivebackItem)
      (Default|RemoveImage (Variables|Reference|GetWBP_Cauldron)))))

(event EventBeginPlay
  (|CallParentFunction)
  (Variables|Default|SetBaseCamPos (Transformation|GetWorldLocation (Variables|Default|GetCamera)))
  (bind _asbp_game_controller (Utilities|Casting|CastToBP_GameController (Game|GetPlayerController 0)))
  (Variables|Reference|SetAs%20BP%20Game%20Controller _asbp_game_controller)
  (bind _asbp_game_instance (Utilities|Casting|CastToBP_GameInstance (Game|GetGameInstance)))
  (Variables|Reference|SetAs%20BP%20Game%20Instance _asbp_game_instance)
  (bind _returnvalue (UserInterface|CreateWidget "/Game/Widgets/HUD/HUDWorkbench/WBP_CauldronUX.WBP_CauldronUX_C"))
  (Variables|Reference|SetWBP_Cauldron _returnvalue))

(event Collision|EventActorBeginOverlap
  (params (OtherActor :type Actor%20Object%20Reference))
  (|CallParentFunction OtherActor) ; This node is disabled and will not be called.\nDrag off pins to build functionality.
)

(event EventOnInteract
  (params (ItemSlots :type Array%20of%20S%20Item%20Slot%20Structures) (PlayerRef :type BP%20Player%20Object%20Reference))
  (bind _as_bp_my_controller (Variables|Default|GetAs%20BP%20My%20Controller))
  ;[0.15 0.15 0.15 0.5] Interact with cauldron
  (EventDispatchers|BindEventtoOnUseItem (Variables|/Game/Blueprints/Managers/BP_GameController.BP_GameController_C|GetBPC_Inventory (Variables|Default|GetAs%20BP%20My%20Controller)) (EventDispatchers|CreateEvent :!event AddIngredientTemp))
  (Variables|/Game/Blueprints/Managers/BP_GameController.BP_GameController_C|SetIsOnWorkbench _as_bp_my_controller true)
  (Pawn|Possess _as_bp_my_controller self)
  (Default|AutomaticHUDWorkbench _as_bp_my_controller "NewEnumerator2")
  (Default|ChangeUX (Variables|/Game/Widgets/HUD/HUDPlayer/WBP_PlayerHUD.WBP_PlayerHUD_C|GetWB_PlayerDisplay (Variables|/Game/Blueprints/Managers/BP_GameController.BP_GameController_C|GetWB_PlayerHUD (Variables|Reference|GetAs%20BP%20Game%20Controller))) "NewEnumerator2")
  (UserInterface|Viewport|AddtoViewport (Variables|Reference|GetWBP_Cauldron) 0)
  (Rendering|Material|SetOverlayMaterial (Variables|Default|GetCauldron) "/Game/Materials/MI_ObjectOutlineFalse.MI_ObjectOutlineFalse" :!class /Script/Engine.MeshComponent)
  (Transformation|SetWorldLocation (Variables|Default|GetCamera) (Transformation|GetWorldLocation (Variables|/Game/Blueprints/Actors/BP_Player.BP_Player_C|GetFirstPersonCamera (Variables|Default|GetAs%20BP%20Player))) false false)
  (CallFunction|MoveCameraBase))

(event EventUIInteract
  (if (not (Variables|/Game/Blueprints/Managers/BP_GameController.BP_GameController_C|GetIsOnWorkbench (Variables|Reference|GetAs%20BP%20Game%20Controller)))
    (Rendering|Material|SetOverlayMaterial (Variables|Default|GetCauldron) "/Game/Materials/MI_ObjectOutline.MI_ObjectOutline" :!class /Script/Engine.MeshComponent)
    (Default|ButtonAppear (Variables|/Game/Blueprints/Managers/BP_GameController.BP_GameController_C|GetWB_InfoHUD (Variables|Reference|GetAs%20BP%20Game%20Controller)))
    (Variables|Default|SetTimer 0.1)
    (Utilities|Time|SetTimerbyEvent (delegate Custom|OutlineDelay) 0.1)))

(event EventTick
  (params (DeltaSeconds :type Float%20%28single-precision%29))
  (Variables|Default|SetDelta%20Seconds DeltaSeconds)
  (Variables|Default|SetTimer (* (Variables|Default|GetDelta%20Seconds) (- (Variables|Default|GetTimer) (Variables|Default|GetDelta%20Seconds)))))

(fn ConstructionScript
  (|CallParentFunction))

(fn AddIngredientTemp
  (params (IngredientIn :type S%20Ingredient%20Structure) (Index :type Integer) (ItemID :type Name))
  (bind (_name _propertycut _propertygrind _id _finalproperty _mesh _texture _category _class _image) (Utilities|Struct|BreakSIngredient IngredientIn))
  (if (Utilities|Enum|Equal(Enum) _category "NewEnumerator1")
    (Default|AddSlot (Variables|Reference|GetWBP_Cauldron) _image)
    (Utilities|Array|Add (Variables|Default|GetTempListSlot) ItemID)
    (for _array_element (Utilities|Array|MakeArray (Utilities|String|EnumtoString _finalproperty))
      (if (Utilities|Map|Contains (Variables|Default|GetTempProperty) _array_element)
        (bind _result (Math|Integer|IncrementInt (.Value (Utilities|Map|Find (Variables|Default|GetTempProperty) _array_element)))
          (:%20%20
            (Utilities|Map|Add (Variables|Default|GetTempProperty) _array_element _result)))
        (else
          (Utilities|Map|Add (Variables|Default|GetTempProperty) _array_element 1))))
    (bind _output_get (Variables|Default|SetTempProperty (Variables|Default|GetTempProperty)))
    (bind _keys (Utilities|Map|Keys _output_get))
    (for _array_element_2 _keys
      (Development|PrintString _array_element_2))
    (Default|RemoveItemUsed (Variables|/Game/Blueprints/Managers/BP_GameController.BP_GameController_C|GetBPC_Inventory (Variables|Default|GetAs%20BP%20My%20Controller)) Index)
    (else
      (Development|PrintString "Impossible ingredient brute"))))

(fn CompareMap
  (params (MapA_Ingredient :type Map%20of%20Strings%20to%20Integers) (MapB_Recipe :type Map%20of%20Strings%20to%20Integers))
  (if (== (Utilities|Map|Length MapA_Ingredient) (Utilities|Map|Length MapB_Recipe))
    (bind _keys (Utilities|Map|Keys MapA_Ingredient))
    (for _array_element _keys
      (if (Utilities|Map|Contains MapB_Recipe _array_element)
        (if (== (.Value (Utilities|Map|Find MapA_Ingredient _array_element)) (.Value (Utilities|Map|Find MapB_Recipe _array_element)))
          (Variables|Default|SetIs%20Matching true)
          (else
            (return false)))
        (else
          (return false))))
    (return true)
    (else
      (return false))))

(fn GivebackItem
  (bind _templistslot (Variables|Default|GetTempListSlot))
  (if (Utilities|Array|IsNotEmpty _templistslot)
    (for _array_element _templistslot
      (Default|Pickup (Variables|/Game/Blueprints/Managers/BP_GameController.BP_GameController_C|GetBPC_Inventory (Variables|Reference|GetAs%20BP%20Game%20Controller)) _array_element 1 (Variables|/Game/Blueprints/Managers/BP_GameInstance.BP_GameInstance_C|GetInventorySlotsSave (Variables|Reference|GetAs%20BP%20Game%20Instance))))
    (Utilities|Array|Clear _templistslot)
    (Utilities|Map|Clear (Variables|Default|GetTempProperty))))

(fn CreatePotionUI
  (params (ItemID :type Name))
  (bind _as_bp_my_controller (Variables|Default|GetAs%20BP%20My%20Controller))
  (bind _returnvalue (UserInterface|CreateWidget "/Game/Widgets/HUD/HUDWorkbench/WBP_PotionCreate.WBP_PotionCreate_C" _as_bp_my_controller _as_bp_my_controller))
  (bind _output_get (Variables|Default|SetWBP_PotionCreate _returnvalue))
  (UserInterface|Viewport|AddtoViewport _output_get 0)
  (Variables|Default|SetPotionUIIsOn true)
  (bind _returnvalue_2 (Utilities|GetDataTableRow "/Game/Data/Datatables/DT_Ingredients.DT_Ingredients" ItemID)
    (:then
      (Variables|Default|SetWidgetIsOn true)
      (Default|SetPotionImage&Text _output_get (.Image (Utilities|Struct|BreakSIngredient _returnvalue_2)) (.Name (Utilities|Struct|BreakSIngredient _returnvalue_2)))
      (Default|AnimationPlay _output_get))))