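; BP_Workbench_Cut is the cutting workbench actor, handling the player's switch away from it toward the grind workbench view.
; On BeginPlay it runs parent logic and caches the player's BP_GameController.
; The IA_ChangeWorkbench input removes the HUD through the controller's player display widget, then uses MoveComponentTo to move the Camera to the controller's stored grind-workbench position, keeping its relative rotation.
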(event Input|EnhancedActionEvents|EnhancedInputActionIA_ChangeWorkbench
  (params (ActionValue :type Boolean) (ElapsedSeconds :type Float%20%28double-precision%29) (TriggeredSeconds :type Float%20%28double-precision%29) (InputAction :type Input%20Action%20Object%20Reference :default "/Game/FirstPerson/Input/Actions/IA_ChangeWorkbench.IA_ChangeWorkbench"))
  (bind _camera (Variables|Default|GetCamera))
  (:Started
    (Default|RemoveHUD (Variables|/Game/Widgets/HUD/HUDPlayer/WBP_PlayerHUD.WBP_PlayerHUD_C|GetWB_PlayerDisplay (Variables|/Game/Blueprints/Managers/BP_GameController.BP_GameController_C|GetWB_PlayerHUD (Variables|Default|GetBP_MyController))))
    (Components|MoveComponentTo _camera (Variables|/Game/Blueprints/Managers/BP_GameController.BP_GameController_C|GetCamPosWorkbench_Grind (stale EventBeginPlay _output_get)) (Variables|/Script/Engine.SceneComponent|GetRelativeRotation _camera) false false 0.2 false)))

(event EventBeginPlay
  (|CallParentFunction)
  (bind _asbp_game_controller (Utilities|Casting|CastToBP_GameController (Game|GetPlayerController 0)))
  (bind _output_get (Variables|Default|SetBP_MyController _asbp_game_controller)))

(event Collision|EventActorBeginOverlap
  (params (OtherActor :type Actor%20Object%20Reference)))

(event EventTick
  (params (DeltaSeconds :type Float%20%28single-precision%29)))

(fn ConstructionScript
  (|CallParentFunction))