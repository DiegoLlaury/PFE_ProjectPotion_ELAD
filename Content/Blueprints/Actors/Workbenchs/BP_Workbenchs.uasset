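; BP_Workbenchs is an interactable workbench actor that opens a crafting-method HUD, with only the Cauldron method handled so far.
; BeginPlay caches the player pawn and game controller.
; OnInteract passes the incoming item slots to the controller's inventory component, flags the workbench state and requests the HUD matching MethodProcess.
; QuitWorkbenchs removes the HUD and clears the flag, while FocusTarget returns empty text.
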(event EventBeginPlay
  (bind _asbp_player (Utilities|Casting|CastToBP_Player (Game|Player|GetPlayerPawn 0)))
  (Variables|Default|SetAs%20BP%20Player _asbp_player)
  (bind _asbp_game_controller (Utilities|Casting|CastToBP_GameController (Game|GetPlayerController 0)))
  (Variables|Default|SetAs%20BP%20My%20Controller _asbp_game_controller))

(event EventTick
  (params (DeltaSeconds :type Float%20%28single-precision%29)))

(event EventOnInteract
  (params (ItemSlots :type Array%20of%20S%20Item%20Slot%20Structures))
  (bind _as_bp_my_controller (Variables|Default|GetAs%20BP%20My%20Controller))
  (Variables|/Game/Blueprints/Components/BPC_Inventory.BPC_Inventory_C|Set%20Item%20Slots (Variables|/Game/Blueprints/Managers/BP_GameController.BP_GameController_C|GetBPC_Inventory (Variables|Default|GetAs%20BP%20My%20Controller)) ItemSlots)
  (Variables|/Game/Blueprints/Managers/BP_GameController.BP_GameController_C|SetIsOnWorkbench _as_bp_my_controller true)
  (switch Utilities|FlowControl|Switch|SwitchonEProcessingMethod (Variables|Default|GetMethodProcess)
    (:NewEnumerator2
      (Default|AutomaticHUDWorkbench _as_bp_my_controller "NewEnumerator2"))))

(fn ConstructionScript)

(fn NewFunction)

(fn QuitWorkbenchs
  (bind _as_bp_my_controller (Variables|Default|GetAs%20BP%20My%20Controller))
  (Default|RemoveHUD _as_bp_my_controller)
  (Variables|/Game/Blueprints/Managers/BP_GameController.BP_GameController_C|SetIsOnWorkbench _as_bp_my_controller false))

(fn FocusTarget
  (return ""))