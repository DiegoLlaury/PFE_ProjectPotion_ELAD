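; Possessable crafting workbench (OldSystem) where the player cuts or grinds ingredients or brews potions, depending on its Method.
; On interact the controller possesses it and binds inventory item use; escape, blocked during QTEs, repossesses the player.
; Cut and Grind swap raw items for processed variants.
; Cauldron tallies processed ingredients' properties in a map, launches a QTE widget, and ProcessPotion grants the potion whose DT_Recipes entry matches exactly.
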(event Custom|LaunchCauldron
  ;[0.15 0.15 0.15 0.5] Système de craft de potion
  (if (not (<= (Utilities|Map|Length (Variables|Default|GetTempProperty)) 1))
    (CallFunction|MoveCamera)
    (Default|RemoveHUD (Variables|/Game/Widgets/HUD/HUDPlayer/WBP_PlayerHUD.WBP_PlayerHUD_C|GetWB_PlayerDisplay (Variables|/Game/Blueprints/Managers/BP_GameController.BP_GameController_C|GetWB_PlayerHUD (Variables|References|GetAs%20BP%20My%20Controller))))
    (Utilities|FlowControl|Delay 0.3)
    (Variables|Default|SetQTEOn true)
    (bind _returnvalue (UserInterface|CreateWidget "/Game/Widgets/HUD/HUDWorkbench/WBP_QTEPotion.WBP_QTEPotion_C" 0 0))
    (bind _output_get (Variables|References|SetQTEPotion _returnvalue))
    (UserInterface|Viewport|AddtoViewport _output_get 0)))

(event Custom|ProcessIngredient
  (params (IngredientData :type S%20Ingredient%20Structure) (Index :type Integer))
  (if (Utilities|Enum|Equal(Enum) (.Category (Utilities|Struct|BreakSIngredient IngredientData)) "NewEnumerator0")
    (Variables|Default|SetIngredient%20Data IngredientData)
    (Variables|Default|SetIndex Index)
    (switch Utilities|FlowControl|Switch|SwitchonEProcessingMethod (Variables|Default|GetMethod)
      (:NewEnumerator0
        (Default|RemoveHUD (Variables|/Game/Widgets/HUD/HUDPlayer/WBP_PlayerHUD.WBP_PlayerHUD_C|GetWB_PlayerDisplay (Variables|/Game/Blueprints/Managers/BP_GameController.BP_GameController_C|GetWB_PlayerHUD (Variables|References|GetAs%20BP%20My%20Controller))))
        (Utilities|FlowControl|Delay 0.3)
        (Variables|Default|SetQTEOn true))
      (:NewEnumerator1
        (Default|RemoveHUD (Variables|/Game/Widgets/HUD/HUDPlayer/WBP_PlayerHUD.WBP_PlayerHUD_C|GetWB_PlayerDisplay (Variables|/Game/Blueprints/Managers/BP_GameController.BP_GameController_C|GetWB_PlayerHUD (Variables|References|GetAs%20BP%20My%20Controller))))
        (Utilities|FlowControl|Delay 0.3)
        (Variables|Default|SetQTEOn true)))
    (else
      (Variables|Default|SetIngredient%20Data IngredientData)
      (Variables|Default|SetIndex Index)
      (switch Utilities|FlowControl|Switch|SwitchonEProcessingMethod (Variables|Default|GetMethod)
        (:NewEnumerator2
          (CallFunction|AddIngredientTemp (Variables|Default|GetIngredient%20Data) (Variables|Default|GetIndex)))))))

(event Custom|ProcessToIngredient
  (CallFunction|ProcessIngredients (Variables|Default|GetIngredient%20Data) (Variables|Default|GetMethod) (Variables|Default|GetIndex)))

(event Custom|ProcessPotion
  ;[0.15 0.15 0.15 0.5] Système de craft de potion
  (Default|AutomaticHUDWorkbench (Variables|References|GetAs%20BP%20My%20Controller) "NewEnumerator0")
  (Variables|Default|SetQTEOn false)
  (if (Utilities|Map|IsNotEmpty (Variables|Default|GetTempProperty))
    (bind _outrownames (DataTable|GetDataTableRowNames (Variables|References|GetDT_Recipes)))
    (bind _array_element (Utilities|Array|ForEachLoopwithBreak _outrownames :!label _label)
      (:LoopBody
        (bind _returnvalue (Utilities|GetDataTableRow "/Game/Data/Datatables/DT_Recipes.DT_Recipes" _array_element)
          (:then
            (if (CallFunction|CompareMap (Variables|Default|GetTempProperty) (.ingredients _returnvalue))
              (Utilities|Map|Clear (Variables|Default|GetTempProperty))
              (Default|Pickup (Variables|/Game/Blueprints/Managers/BP_GameController.BP_GameController_C|GetBPC_Inventory (Variables|References|GetAs%20BP%20My%20Controller)) (.idresultingpotion _returnvalue) 1)
              (Transformation|SetRelativeLocation (Variables|Default|GetCamera) (Variables|Default|GetBaseCamPos) false false)
              (goto _label Break))))))))

(event Custom|MoveCamera
  (Timeline|CamMovement Play
    (:Update
      (Transformation|SetRelativeLocation (Variables|Default|GetCamera) (- (Variables|Default|GetBaseCamPos) "40.000000,0.000000,20.000000") false false))))

(event Input|EnhancedActionEvents|EnhancedInputActionIA_EscapeWorkbench
  (params (ActionValue :type Boolean) (ElapsedSeconds :type Float%20%28double-precision%29) (TriggeredSeconds :type Float%20%28double-precision%29) (InputAction :type Input%20Action%20Object%20Reference :default "/Game/FirstPerson/Input/Actions/IA_EscapeWorkbench.IA_EscapeWorkbench"))
  (bind _as_bp_my_controller (Variables|References|GetAs%20BP%20My%20Controller))
  ;[0.15 0.15 0.15 0.5] Fais sortir le joueur de l'établis, et lui fais reprendre le controle de son personnage
  (:Started
    (if (not (Variables|Default|GetQTEOn))
      (EventDispatchers|UnbindEventfromOnUseItem (Variables|/Game/Blueprints/Managers/BP_GameController.BP_GameController_C|GetBPC_Inventory (Variables|References|GetAs%20BP%20My%20Controller)) (EventDispatchers|CreateEvent :!event Custom|ProcessIngredient))
      (Default|RemoveHUD (Variables|/Game/Widgets/HUD/HUDPlayer/WBP_PlayerHUD.WBP_PlayerHUD_C|GetWB_PlayerDisplay (Variables|/Game/Blueprints/Managers/BP_GameController.BP_GameController_C|GetWB_PlayerHUD _as_bp_my_controller)))
      (Utilities|FlowControl|Delay 0.2)
      (Variables|/Game/Blueprints/Managers/BP_GameController.BP_GameController_C|SetIsOnWorkbench _as_bp_my_controller false)
      (switch Utilities|FlowControl|Switch|SwitchonEProcessingMethod (Variables|Default|GetMethod)
        (:NewEnumerator0
          _)
        (:NewEnumerator1
          _)
        (:NewEnumerator2
          (Widget|RemovefromParent (Variables|References|GetWidgetCauldron))))
      (Pawn|Possess (Variables|References|GetAs%20BP%20My%20Controller) (Variables|References|GetAs%20BP%20Player)))))

(event EventBeginPlay
  (bind _asbp_player (Utilities|Casting|CastToBP_Player (Game|Player|GetPlayerPawn 0)))
  (Variables|References|SetAs%20BP%20Player _asbp_player)
  (bind _asbp_game_controller (Utilities|Casting|CastToBP_GameController (Game|GetPlayerController 0)))
  (Variables|References|SetAs%20BP%20My%20Controller _asbp_game_controller)
  (Variables|Default|SetBaseCamPos (Variables|/Script/Engine.SceneComponent|GetRelativeLocation (Variables|Default|GetCamera))))

(fn ConstructionScript)

(fn ProcessIngredients
  (params (InIngredient :type S%20Ingredient%20Structure) (Method :type EProcessingMethod%20Enum :default "NewEnumerator0") (Index :type Integer))
  (bind (_name _propertycut _propertygrind) (Utilities|Struct|BreakSIngredient InIngredient))
  (bind _as_bp_my_controller (Variables|References|GetAs%20BP%20My%20Controller))
  (bind _as_bp_my_controller_2 (Variables|References|GetAs%20BP%20My%20Controller))
  (bind _bpc_inventory (Variables|/Game/Blueprints/Managers/BP_GameController.BP_GameController_C|GetBPC_Inventory _as_bp_my_controller))
  (bind _bpc_inventory_2 (Variables|/Game/Blueprints/Managers/BP_GameController.BP_GameController_C|GetBPC_Inventory _as_bp_my_controller_2))
  (switch Utilities|FlowControl|Switch|SwitchonEProcessingMethod Method
    (:NewEnumerator0
      (Default|RemoveItemUsed _bpc_inventory Index)
      (Default|Pickup _bpc_inventory_2 (Utilities|String|StringToName _propertycut) 1))
    (:NewEnumerator1
      (Default|RemoveItemUsed _bpc_inventory Index)
      (Default|Pickup _bpc_inventory_2 (Utilities|String|StringToName _propertygrind) 1)))
  (Default|AutomaticHUDWorkbench (Variables|References|GetAs%20BP%20My%20Controller) "NewEnumerator0")
  (Variables|Default|SetQTEOn false))

(fn CompareMap
  (params (MapA_Ingredient :type Map%20of%20Strings%20to%20Integers) (MapB_Recipe :type Map%20of%20Strings%20to%20Integers))
  (if (== (Utilities|Map|Length MapA_Ingredient) (Utilities|Map|Length MapB_Recipe))
    (bind _keys (Utilities|Map|Keys MapA_Ingredient))
    (for _array_element _keys
      (if (Utilities|Map|Contains MapB_Recipe _array_element)
        (if (== (.Value (Utilities|Map|Find MapA_Ingredient _array_element)) (.Value (Utilities|Map|Find MapB_Recipe _array_element)))
          (Variables|Default|SetIs%20Matching true)
          (else
            (return false)))
        (else
          (return false))))
    (return true)
    (else
      (return false))))

(fn AddIngredientTemp
  (params (IngredientIn :type S%20Ingredient%20Structure) (Index :type Integer))
  (bind (_name _propertycut _propertygrind _id _finalproperty _mesh _texture _category) (Utilities|Struct|BreakSIngredient IngredientIn))
  (Development|PrintString (Utilities|String|EnumtoString _finalproperty))
  (if (Utilities|Enum|Equal(Enum) _category "NewEnumerator1")
    (for _array_element (Utilities|Array|MakeArray (Utilities|String|EnumtoString _finalproperty))
      (if (Utilities|Map|Contains (Variables|Default|GetTempProperty) _array_element)
        (bind _result (Math|Integer|IncrementInt (.Value (Utilities|Map|Find (Variables|Default|GetTempProperty) _array_element)))
          (:%20%20
            (Utilities|Map|Add (Variables|Default|GetTempProperty) _array_element _result)))
        (else
          (Utilities|Map|Add (Variables|Default|GetTempProperty) _array_element 1))))
    (bind _output_get (Variables|Default|SetTempProperty (Variables|Default|GetTempProperty)))
    (bind _keys (Utilities|Map|Keys _output_get))
    (for _array_element_2 _keys
      _)
    (Default|RemoveItemUsed (Variables|/Game/Blueprints/Managers/BP_GameController.BP_GameController_C|GetBPC_Inventory (Variables|References|GetAs%20BP%20My%20Controller)) Index)
    (else
      (Development|PrintString "Impossible ingredient brute"))))

(fn FocusTarget
  (return ""))

(fn OnInteract
  (params (ItemSlots :type Array%20of%20S%20Item%20Slot%20Structures))
  (Variables|/Game/Blueprints/Components/BPC_Inventory.BPC_Inventory_C|Set%20Item%20Slots (Variables|/Game/Blueprints/Managers/BP_GameController.BP_GameController_C|GetBPC_Inventory (Variables|References|GetAs%20BP%20My%20Controller)) ItemSlots)
  (Pawn|Possess (Variables|References|GetAs%20BP%20My%20Controller) self)
  (EventDispatchers|BindEventtoOnUseItem (Variables|/Game/Blueprints/Managers/BP_GameController.BP_GameController_C|GetBPC_Inventory (Variables|References|GetAs%20BP%20My%20Controller)) (EventDispatchers|CreateEvent :!event Custom|ProcessIngredient))
  (switch Utilities|FlowControl|Switch|SwitchonEProcessingMethod (Variables|Default|GetMethod)
    (:NewEnumerator0
      _)
    (:NewEnumerator1
      _)
    (:NewEnumerator2
      _))
  (Variables|/Game/Blueprints/Managers/BP_GameController.BP_GameController_C|SetIsOnWorkbench (Variables|References|GetAs%20BP%20My%20Controller) true)
  (Default|AutomaticHUDWorkbench (Variables|References|GetAs%20BP%20My%20Controller) "NewEnumerator0"))