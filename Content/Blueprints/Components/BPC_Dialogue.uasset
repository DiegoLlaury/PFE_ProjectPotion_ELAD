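; Dialogue component for NPC conversations, including steps that require the player to hand over a potion or ingredient.
; It walks DataTable rows using an index stored in the GameInstance, displaying each through a dialogue widget that flags potion requests and quest end.
; When an item is needed, interacting opens the inventory.
; ItemDetection matches the item's ID against the row's options, jumps to that option's row and consumes the item.
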(event EventBeginPlay
  (bind _asbp_my_controller (Utilities|Casting|CastToBP_MyController (Game|GetPlayerController 0)))
  (Variables|Default|SetBP%20My%20Controller _asbp_my_controller)
  (bind _returnvalue (UserInterface|CreateWidget "/Game/Widgets/HUD/WB_DataTableDialogue.WB_DataTableDialogue_C"))
  (bind _output_get (Variables|Default|SetUIDialogue _returnvalue))
  (Widget|SetVisibility _output_get "Hidden")
  (bind _asbp_game_instance (Utilities|Casting|CastToBP_GameInstance (Game|GetGameInstance)))
  (Variables|Default|SetBP%20Game%20Instance _asbp_game_instance)
  (bind _outrownames (DataTable|GetDataTableRowNames (.datatable (Variables|Default|GetDialogueData))))
  (Variables|Default|SetLines _outrownames)
  (Variables|/Game/Blueprints/Managers/BP_GameInstance.BP_GameInstance_C|SetIndexDialogueGI (Variables|Default|GetBP%20Game%20Instance) (Utilities|Array|FindItem (Variables|Default|GetLines) (.rowname (Variables|Default|GetDialogueData)))))

(event EventTick
  (params (DeltaSeconds :type Float%20%28single-precision%29)))

(fn UpdateTalk
  (params (LineNumber :type Name))
  (bind _bp_my_controller (Variables|Default|GetBP%20My%20Controller))
  (bind _bpc_inventory (Variables|/Game/Blueprints/Managers/BP_MyController.BP_MyController_C|GetBPC_Inventory _bp_my_controller))
  (bind (_out_row_need_potion_ _out_row_open_dialogue_options _out_row_end_dialogue_) (Default|NextTalk (Variables|Default|GetUIDialogue) LineNumber))
  (if _out_row_end_dialogue_
    (Default|CallEndQuestPotion)
    (elif _out_row_need_potion_
      (Variables|/Game/Blueprints/Components/BPC_Inventory.BPC_Inventory_C|SetNeedObject%20 _bpc_inventory true)
      (elif (not (Variables|/Game/Blueprints/Components/BPC_Inventory.BPC_Inventory_C|GetNeedObject%20 _bpc_inventory))
        (Math|Integer|IncrementInt (Variables|/Game/Blueprints/Managers/BP_GameInstance.BP_GameInstance_C|GetIndexDialogueGI (Variables|Default|GetBP%20Game%20Instance)))))))

(fn OnInteract
  (bind _bp_game_instance (Variables|Default|GetBP%20Game%20Instance))
  (bind _indexdialoguegi (Variables|/Game/Blueprints/Managers/BP_GameInstance.BP_GameInstance_C|GetIndexDialogueGI _bp_game_instance))
  (if (Variables|/Game/Blueprints/Components/BPC_Inventory.BPC_Inventory_C|GetNeedObject%20 (Variables|/Game/Blueprints/Managers/BP_MyController.BP_MyController_C|GetBPC_Inventory (Variables|Default|GetBP%20My%20Controller)))
    (Variables|Default|SetTalking? true)
    (Variables|/Game/Blueprints/Components/BPC_Inventory.BPC_Inventory_C|SetIsaPNJ (Variables|/Game/Blueprints/Managers/BP_MyController.BP_MyController_C|GetBPC_Inventory (Variables|Default|GetBP%20My%20Controller)) true)
    (Default|AutomaticOpenInventory (Variables|Default|GetBP%20My%20Controller))
    (elif (Variables|Default|GetTalking?)
      (CallFunction|UpdateTalk (Utilities|Array|Get(acopy) (Variables|Default|GetLines) _indexdialoguegi))
      (return false)
      (else
        (bind _output_get (Variables|Default|SetTalking? true))
        (CallFunction|UpdateTalk (Utilities|Array|Get(acopy) (Variables|Default|GetLines) _indexdialoguegi))
        (return _output_get)))))

(fn ItemDetection
  (params (IngredientData :type S%20Ingredient%20Structure) (Index :type Integer))
  (bind _bp_my_controller (Variables|Default|GetBP%20My%20Controller))
  (bind _bpc_inventory (Variables|/Game/Blueprints/Managers/BP_MyController.BP_MyController_C|GetBPC_Inventory _bp_my_controller))
  (bind _returnvalue (Utilities|GetDataTableRow "/Game/Data/Datatables/DT_Dialogue.DT_Dialogue" (Utilities|Array|Get(acopy) (Variables|Default|GetLines) (Variables|/Game/Blueprints/Managers/BP_GameInstance.BP_GameInstance_C|GetIndexDialogueGI (Variables|Default|GetBP%20Game%20Instance))))
    (:then
      (for _array_element (.opendialogueoptions _returnvalue)
        (bind _array_element_2 (Utilities|Array|ForEachLoopwithBreak (.ingredientneed _array_element) :!label _label)
          (:LoopBody
            (if (== _array_element_2 (.ID (Utilities|Struct|BreakSIngredient IngredientData)))
              (CallFunction|UpdateTalk (.row _array_element))
              (Variables|/Game/Blueprints/Components/BPC_Inventory.BPC_Inventory_C|SetNeedObject%20 _bpc_inventory false)
              (Default|RemoveItemUsed _bpc_inventory Index)
              (goto _label Break)))
          (:Completed
            (Development|PrintString "N'est pas pareil"))))
      (Development|PrintString "N'a pas trouver la potion"))
    (:RowNotFound
      (Development|PrintString "Dialogue non trouver"))))