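; Dialogue manager component that runs an NPC's data-table conversations, including potion requests that branch the NPC's reply.
; Interaction reads the character's line index from the game instance, and UpdateTalk feeds the matching row to a dialogue widget or completes its text.
; When a potion is needed, it opens the inventory and binds item use to pick a reaction by item ID.
; Progress and reactions are saved to the game instance.
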(event Custom|ItemDetection
  (params (IngredientData :type S%20Ingredient%20Structure) (Index :type Integer))
  (CallFunction|FindGivenPotion IngredientData Index))

(event EventBeginPlay
  (bind _asbp_game_controller (Utilities|Casting|CastToBP_GameController (Game|GetPlayerController 0)))
  (Variables|References|SetBP_My_Controller _asbp_game_controller)
  (bind _returnvalue (UserInterface|CreateWidget "/Game/Widgets/HUD/WB_DataTableDialogue.WB_DataTableDialogue_C" 0 self))
  (Variables|References|SetWB_UIDialogue _returnvalue)
  (bind _asbp_game_instance (Utilities|Casting|CastToBP_GameInstance (Game|GetGameInstance)))
  (Variables|References|SetBP_Game_Instance _asbp_game_instance))

(event EventTick
  (params (DeltaSeconds :type Float%20%28single-precision%29)))

(fn UpdateTalk
  (params (DialogueIndex :type Integer))
  (bind _datastructdial (Variables|References|GetDataStructDial))
  (bind (_nightindex _speakersname _currentdialogue _opendialogueoptions _reactionchoice _enddialogue_ _needpotion_) (Utilities|Struct|BreakSNPCDialogue _datastructdial))
  ;[0.15 0.15 0.15 0.5] Permet de s'avancer dans les dialogues, s'adapte si le personnage à besoins d'un objet ou qu'il finit de parler
  (if (Variables|State|GetFinishNPCDialogue?)
    (if (Variables|/Game/Widgets/HUD/WB_DataTableDialogue.WB_DataTableDialogue_C|GetTextFinish (Variables|References|GetWB_UIDialogue))
      (Development|PrintString "UpdateDialogue")
      (bind _result (Math|Integer|IncrementInt DialogueIndex)
        (:%20%20
          (Default|UpdateDialogueIndex (Variables|References|GetBP_Game_Instance) _result (Variables|Default|GetCharacter%20Index) false)
          (Default|UpdateCurrentReaction (Variables|References|GetBP_Game_Instance) (Variables|Default|GetCurrentReaction))
          (Default|CallEndQuestPotion)
          (Widget|SetVisibility (Variables|References|GetWB_UIDialogue) "Hidden")))
      (else
        (Default|FinishText (Variables|References|GetWB_UIDialogue))))
    (else
      (CallFunction|GetSDialogueData DialogueIndex)
      (Variables|Default|SetCharacterName _speakersname)
      (if (Variables|/Game/Widgets/HUD/WB_DataTableDialogue.WB_DataTableDialogue_C|GetTextFinish (Variables|References|GetWB_UIDialogue))
        (if (Utilities|Array|IsEmpty _reactionchoice)
          (Default|NextTalk (Variables|References|GetWB_UIDialogue) _currentdialogue (Variables|Default|GetCharacterName))
          (if _enddialogue_
            (Variables|State|SetFinishNPCDialogue? true)
            (else
              (Default|UpdateDialogueIndex (Variables|References|GetBP_Game_Instance) DialogueIndex (Variables|Default|GetCharacter%20Index) (Variables|State|GetNeed%20Potion))
              (Variables|State|SetNeed%20Potion _needpotion_)))
          (else
            (Default|NextTalk (Variables|References|GetWB_UIDialogue) (Utilities|Array|Get(acopy) _reactionchoice (Variables|Default|GetCurrentReaction)) (Variables|Default|GetCharacterName))))
        (else
          (Default|FinishText (Variables|References|GetWB_UIDialogue)))))))

(fn OnInteract
  (bind _bp_my_controller (Variables|References|GetBP_My_Controller))
  (bind _bpc_inventory (Variables|/Game/Blueprints/Managers/BP_GameController.BP_GameController_C|GetBPC_Inventory _bp_my_controller))
  (if (Variables|State|GetNeed%20Potion)
    (Variables|State|SetIsTalking? true)
    (if (Variables|/Game/Blueprints/Components/BPC_Inventory.BPC_Inventory_C|GetNeedObject? _bpc_inventory)
      (Default|AutomaticOpenInventory (Variables|References|GetBP_My_Controller))
      (EventDispatchers|BindEventtoOnUseItem (Variables|/Game/Blueprints/Managers/BP_GameController.BP_GameController_C|GetBPC_Inventory (Variables|References|GetBP_My_Controller)) (EventDispatchers|CreateEvent :!event Custom|ItemDetection))
      (else
        (Variables|/Game/Blueprints/Components/BPC_Inventory.BPC_Inventory_C|SetNeedObject? _bpc_inventory true)
        (CallFunction|UpdateTalk (Variables|Default|GetDialogue%20Index))))
    (else
      (bind _dialogueindex (Default|SetupNPCLine (Variables|References|GetBP_Game_Instance) (Variables|Default|GetCharacter%20Index)))
      (Variables|Default|SetDialogue%20Index _dialogueindex)
      (if (Variables|State|GetIsTalking?)
        (CallFunction|UpdateTalk (Variables|Default|GetDialogue%20Index))
        (return false)
        (else
          (bind _output_get (Variables|State|SetIsTalking? true))
          (CallFunction|UpdateTalk (Variables|Default|GetDialogue%20Index))
          (return _output_get))))))

(fn FindGivenPotion
  (params (IngredientData :type S%20Ingredient%20Structure) (Index :type Integer))
  (bind _id (Utilities|Struct|BreakSIngredient IngredientData))
  (bind _bp_my_controller (Variables|References|GetBP_My_Controller))
  (bind _datastructdial (Variables|References|GetDataStructDial))
  (bind _opendialogueoptions (Utilities|Struct|BreakSNPCDialogue _datastructdial))
  (bind _bpc_inventory (Variables|/Game/Blueprints/Managers/BP_GameController.BP_GameController_C|GetBPC_Inventory _bp_my_controller))
  (bind (_value _returnvalue) (Utilities|Map|Find _opendialogueoptions _id))
  ;[0.15 0.15 0.15 0.5] Adapte la réponse du PNJ en fonction de la potion que le joueur lui a donner, en la comparant aux potions renseigner dans la Data Table
  (if _returnvalue
    (Variables|Default|SetCurrentReaction _value)
    (Variables|State|SetNeed%20Potion false)
    (Variables|/Game/Blueprints/Components/BPC_Inventory.BPC_Inventory_C|SetNeedObject? _bpc_inventory false)
    (EventDispatchers|UnbindEventfromOnUseItem _bpc_inventory (EventDispatchers|CreateEvent :!event Custom|ItemDetection))))

(fn GetSDialogueData
  (params (IndexDialogue :type Integer))
  (bind _getdialoguedata (Variables|References|GetGetDialogueData))
  (bind _outrownames (DataTable|GetDataTableRowNames (.datatable _getdialoguedata)))
  (bind _returnvalue (Utilities|GetDataTableRow (.datatable _getdialoguedata) (Utilities|Array|Get(acopy) _outrownames IndexDialogue))
    (:then
      (Variables|References|SetDataStructDial _returnvalue))))