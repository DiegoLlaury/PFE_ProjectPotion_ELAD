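; BPC_Grimoire is a component for a grimoire book of ingredient pages with page turning.
; On BeginPlay it caches the BP_GameInstance, which holds the current page index list.
; TurnPageRight flags the page as turning and checks whether the first index plus three stays within the DT_PageIngredientData row count, but nothing follows that check yet.
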(event EventBeginPlay
  (bind _asbp_game_instance (Utilities|Casting|CastToBP_GameInstance (Game|GetGameInstance)))
  (Variables|Default|SetRefGameInstance _asbp_game_instance))

(event EventTick
  (params (DeltaSeconds :type Float%20%28single-precision%29)))

(fn TurnPageRight
  (Variables|Default|SetbIsTurningPage true)
  (bind _outrownames (DataTable|GetDataTableRowNames "/Game/Data/Datatables/DT_PageIngredientData.DT_PageIngredientData"))
  (if (< (+ (Utilities|Array|Get(acopy) (Variables|/Game/Blueprints/Managers/BP_GameInstance.BP_GameInstance_C|GetListIndexPage (Variables|Default|GetRefGameInstance))) 3) (Utilities|Array|Length _outrownames))
    _))