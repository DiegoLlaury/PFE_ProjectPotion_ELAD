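; Slot-based inventory component that handles picking up, using, dropping and transferring ingredients and potions between inventories.
; Slots store item IDs resolved through DT_Ingredients, and edits are mirrored into a passed-in save array, with dispatchers signalling changes.
; UseItem branches on category: Brute and Process items require a workbench, while potions require NeedObject and are consumed.
; Full inventories trigger a warning on pickup; drops, blocked at workbenches, spawn in a cone before the player.
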(event Custom|UpdateInventory
  (Default|CallOnInventoryUpdated))

(event EventBeginPlay
  (bind _asbp_player (Utilities|Casting|CastToBP_Player (Game|GetPlayerCharacter 0)))
  (Variables|References|SetAs%20BP%20Player _asbp_player)
  (bind _asbp_game_instance (Utilities|Casting|CastToBP_GameInstance (Game|GetGameInstance)))
  (Variables|References|SetBP_Game_Instance_Ref _asbp_game_instance)
  (bind _asbp_game_controller (Utilities|Casting|CastToBP_GameController (Game|GetPlayerController 0)))
  (Variables|References|SetBP_My_Controller_Ref _asbp_game_controller))

(event EventTick
  (params (DeltaSeconds :type Float%20%28single-precision%29)))

(fn RemoveItemUsed
  (params (Index :type Integer) (InventorySave :type Array%20of%20S%20Item%20Slot%20Structures))
  ;[0.15 0.15 0.15 0.5] Retire un objet de l'inventaire
  (Utilities|Array|SetArrayElem (Variables|Default|Get%20Item%20Slots) Index (Utilities|Struct|MakeSItemSlot "None"))
  (Utilities|Array|SetArrayElem InventorySave Index (Utilities|Struct|MakeSItemSlot "None")))

(fn AddItemtoInventory
  (params (ItemID :type Name%20%28by%20ref%29) (Index :type Integer) (InventorySave :type Array%20of%20S%20Item%20Slot%20Structures))
  ;[0.15 0.15 0.15 0.5] Ajoute un item à la liste de slots dans l'inventaire
  (Utilities|Array|SetArrayElem (Variables|Default|Get%20Item%20Slots) Index (Utilities|Struct|MakeSItemSlot ItemID))
  (Utilities|Array|SetArrayElem InventorySave Index (Utilities|Struct|MakeSItemSlot ItemID))
  ;[0.15 0.15 0.15 0.5] Envoie un message au widget de l'inventaire
  (Default|CallOnInventoryChanged)
  (Default|CallOnInventoryUpdated))

(fn PrintInventory
  ;[0.15 0.15 0.15 0.5] Debug : Permet de print tout l'inventaire
  (for (_array_element _array_index) (Variables|Default|Get%20Item%20Slots)
    (Development|PrintString (Utilities|String|Append (Utilities|String|ToString(Integer) _array_index) ":" (Utilities|String|ToString(Name) (Utilities|Struct|BreakSItemSlot _array_element))))))

(fn Pickup
  (params (ItemID :type Name) (LocalItemQuantity :type Integer) (InventorySave :type Array%20of%20S%20Item%20Slot%20Structures))
  (bind (_success _array_index) (CallFunction|AnySlotAvailable))
  ;[0.15 0.15 0.15 0.5] Systeme de ramasse pour vérifier si tout les slots d'inventaire ne sont pas remplis
  (bind _output_get (Variables|Default|SetItem%20ID ItemID))
  (bind _output_get_2 (LocalVariables|SetLocal_ItemQuantity LocalItemQuantity))
  (while (and (> _output_get_2 0) (not (LocalVariables|GetLocal_IsFull)))
    (if _success
      (CallFunction|AddItemtoInventory _output_get _array_index InventorySave)
      (Math|Integer|DecrementInt (LocalVariables|GetLocal_ItemQuantity)
        (:%20%20
          (return true 0)))
      (else
        (LocalVariables|SetLocal_IsFull true)
        (Default|SetWarningMessage (Variables|/Game/Blueprints/Actors/BP_Player.BP_Player_C|GetWB%20Warning%20Message%20Ref (Variables|References|GetAs%20BP%20Player)) "Pas de place dans l'inventaire"))))
  (return (not (LocalVariables|GetLocal_IsFull)) (LocalVariables|GetLocal_ItemQuantity)))

(fn FindSlot
  (params (ItemID :type Name))
  (for (_array_element _array_index) (Variables|Default|Get%20Item%20Slots)
    (if (== ItemID (Utilities|Struct|BreakSItemSlot _array_element))
      (return true _array_index)))
  (return false -1))

(fn AnySlotAvailable
  (for (_array_element _array_index) (Variables|Default|Get%20Item%20Slots)
    (if (== (Utilities|Struct|BreakSItemSlot _array_element) "")
      (return true _array_index)))
  (return false -1))

(fn UseItem
  (params (Index :type Integer) (InventorySave :type Array%20of%20S%20Item%20Slot%20Structures))
  (bind _bp_my_controller_ref (Variables|References|GetBP_My_Controller_Ref))
  (bind _needobject_ (Variables|State|GetNeedObject?))
  (bind _isonworkbench (Variables|/Game/Blueprints/Managers/BP_GameController.BP_GameController_C|GetIsOnWorkbench _bp_my_controller_ref))
  ;[0.15 0.15 0.15 0.5] Est appeler quand l'on utilise un objet
  (LocalVariables|SetLocal_ItemID (.itemid (Utilities|Array|Get(acopy) (Variables|Default|Get%20Item%20Slots) Index)))
  (switch Utilities|FlowControl|Switch|SwitchonECategory (.category (CallFunction|GetItemData (LocalVariables|GetLocal_ItemID)))
    (:NewEnumerator0
      ;[0.15 0.15 0.15 0.5] Vérifie si le joueur est sur un établis, si oui transforme l'item et envoie un message
      (if _isonworkbench :!label _label
        (Utilities|FlowControl|Sequence
          (:then_0
            (Default|CallOnUseItem (CallFunction|GetItemData (LocalVariables|GetLocal_ItemID)) Index (LocalVariables|GetLocal_ItemID)))
          (:then_1
            (Default|CallOnInventoryUpdated)))
        (else
          (Default|CallOnInventoryUpdated)
          (return (Variables|State|GetNeedObject?) _isonworkbench true))))
    (:NewEnumerator1
      (goto _label))
    (:NewEnumerator2
      ;[0.15 0.15 0.15 0.5] Vérifie si le PNJ a besoin d'une potion, si oui envoir un message pour signifier que l'objet à été utiliser, modifie HUD de l'inventaire et la liste de l'inventaire
      (if _needobject_
        (Utilities|FlowControl|Sequence
          (:then_0
            (Default|CallOnUseItem (CallFunction|GetItemData (LocalVariables|GetLocal_ItemID)) Index (LocalVariables|GetLocal_ItemID)))
          (:then_1
            (Utilities|GetDataTableRow "/Game/Data/Datatables/DT_Ingredients.DT_Ingredients" (Variables|Default|GetItem%20ID)
              (:then
                (Default|RemoveHUDTest (Variables|References|GetBP_My_Controller_Ref)))))
          (:then_2
            (CallFunction|RemoveItemUsed Index InventorySave)
            (Default|CallOnInventoryUpdated)))
        (else
          (Default|CallOnInventoryUpdated)
          (return _needobject_ false true))))))

(fn GetDropLocation
  (bind _returnvalue (Game|Player|GetPlayerPawn 0))
  ;[0.15 0.15 0.15 0.5] Permet de définir la zone de drop de l'item jeter
  (return (+ (Transformation|GetActorLocation _returnvalue) (* (Math|Random|RandomUnitVectorinConeinDegrees (Transformation|GetActorForwardVector _returnvalue) 55.0) 1.2e+02))))

(fn GetItemData
  (params (ItemID :type Name))
  ;[0.15 0.15 0.15 0.5] Lie l'item ID avec les informations dans ça Data Table
  (bind _returnvalue (Utilities|GetDataTableRow "/Game/Data/Datatables/DT_Ingredients.DT_Ingredients" ItemID)
    (:then
      (return _returnvalue))))

(fn DropItem
  (params (Index :type Integer) (InventorySave :type Array%20of%20S%20Item%20Slot%20Structures))
  ;[0.15 0.15 0.15 0.5] Systeme de Drop de l'item gérant les changements dans l'inventaire et l'aparition de l'item
  (if (not (Variables|/Game/Blueprints/Managers/BP_GameController.BP_GameController_C|GetIsOnWorkbench (Variables|References|GetBP_My_Controller_Ref)))
    (bind _output_get (LocalVariables|SetLocal_ItemID_Drop (.itemid (Utilities|Array|Get(acopy) (Variables|Default|Get%20Item%20Slots) Index))))
    (Utilities|FlowControl|Sequence
      (:then_0
        (if (!= (LocalVariables|GetLocal_ItemID_Drop) "")
          (CallFunction|RemoveItemUsed Index InventorySave)
          (Game|SpawnActorfromClass (.Class (Utilities|Struct|BreakSIngredient (CallFunction|GetItemData (LocalVariables|GetLocal_ItemID_Drop)))) (Math|Transform|MakeTransform (CallFunction|GetDropLocation) "0, 0, 0" "1.000000,1.000000,1.000000") "Undefined" "MultiplyWithRoot" 0 (Utilities|String|Append (Utilities|String|ToString(Text) (.Name (Utilities|Struct|BreakSIngredient (CallFunction|GetItemData (LocalVariables|GetLocal_ItemID_Drop))))) (Utilities|String|Append "_" (Utilities|String|ToString(Integer) (Math|Random|RandomInteger 1000)))) 0)
          (else
            (return true))))
      (:then_1
        (Utilities|GetDataTableRow "/Game/Data/Datatables/DT_Ingredients.DT_Ingredients" _output_get
          (:then
            (Default|CallOnInventoryUpdated)))))
    (else
      (return true))))

(fn ResizeInventory
  (params (InventorySave :type Array%20of%20S%20Item%20Slot%20Structures))
  (Utilities|Array|Resize (Variables|Default|Get%20Item%20Slots) (Variables|GameFeelStat|GetSetInventorySize))
  (Utilities|Array|Resize InventorySave (Variables|GameFeelStat|GetSetInventorySize))
  (Variables|Default|Set%20Item%20Slots InventorySave))

(fn SetInventorySave
  (params (NewParam :type Name)))

(fn TransferItemtoInventory
  (params (FromSlotIndex :type Integer) (ItemID :type Name) (TargetInventory :type BPC%20Inventory%20Object%20Reference) (TargetInventorySave :type Array%20of%20S%20Item%20Slot%20Structures) (InventorySave :type Array%20of%20S%20Item%20Slot%20Structures))
  (bind (_success _array_index) (CallFunction|AnySlotAvailable TargetInventory))
  (if _success
    (CallFunction|RemoveItemUsed FromSlotIndex InventorySave)
    (CallFunction|AddItemtoInventory TargetInventory ItemID _array_index TargetInventorySave)
    (CallFunction|UpdateInventory)
    (Default|CallUpdateCupBoard TargetInventory)
    (Default|CallUpdateCupBoard)))

(fn AddItemDemo)