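; BPC_ItemData is an item component that lets its owning actor be picked up into the interactor's inventory.
; On Interact, it passes the item's data row name and the Game Instance's saved inventory slots to the interactor's inventory component.
; A successful pickup records the unique ID as collected in the Game Instance and destroys the owner, while failure prints a no-space message.
; FocusTarget returns an empty string.
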(event EventBeginPlay
  (bind _asbp_game_instance (Utilities|Casting|CastToBP_GameInstance (Game|GetGameInstance)))
  (Variables|Default|SetAs%20BP%20Game%20Instance _asbp_game_instance))

(event EventInteract
  (params (Interactor :type BP%20Game%20Controller%20Object%20Reference))
  ;[0.15 0.15 0.15 0.5] Permet d'intéragir avec un ingrédient pour le ramasser et le mettre dans l'inventaire
  (bind _bpc_inventory (Variables|/Game/Blueprints/Managers/BP_GameController.BP_GameController_C|GetBPC_Inventory Interactor)
    (:then
      (bind _success (Default|Pickup _bpc_inventory (.rowname (Variables|Default|GetGetItemData)) 1 (Variables|/Game/Blueprints/Managers/BP_GameInstance.BP_GameInstance_C|GetInventorySlotsSave (Variables|Default|GetAs%20BP%20Game%20Instance))))
      (if _success
        (Utilities|Set|Add (Variables|/Game/Blueprints/Managers/BP_GameInstance.BP_GameInstance_C|GetCollectedItems (Variables|Default|GetAs%20BP%20Game%20Instance)) (Variables|Default|GetUniqueItemID))
        (Actor|DestroyActor (Components|GetOwner))
        (else
          (Development|PrintString "No Place in Inventory"))))
    (:else)))

(fn FocusTarget
  (return ""))