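; Actor component that launches quick-time-event minigames for cutting, grinding and cauldron potion-making at workbenches.
; LaunchQTE switches on MethodProcess, removes the HUD and shows the matching QTE widget with its workbench reference; Cut and Grind require one specific ingredient category.
; Widget result events are bound on creation, and success and failure functions fire the process or failed dispatchers.
; Separate functions bind and unbind the player controller inventory's OnUseItem event.
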(event EventBeginPlay
  (bind _asbp_game_controller (Utilities|Casting|CastToBP_GameController (Game|GetPlayerController 0)))
  (Variables|Default|SetAs%20BP%20Game%20Controller _asbp_game_controller))

(event EventTick
  (params (DeltaSeconds :type Float%20%28single-precision%29)))

(fn LaunchQTE
  (params (InIngedient :type S%20Ingredient%20Structure) (Index%20Item :type Integer) (ItemID :type Name))
  (bind _refworkbenchcutgrind (Variables|Default|GetRefWorkbenchCutGrind))
  (LocalVariables|SetIngredientCategory (.Category (Utilities|Struct|BreakSIngredient InIngedient)))
  (switch Utilities|FlowControl|Switch|SwitchonEProcessingMethod (Variables|Default|GetMethodProcess)
    (:NewEnumerator0
      (if (Utilities|Enum|Equal(Enum) (LocalVariables|GetIngredientCategory) "NewEnumerator0")
        (Variables|Default|SetbQTEOn true)
        (Default|RemoveHUD (Variables|Default|GetAs%20BP%20Game%20Controller))
        (bind _returnvalue (UserInterface|CreateWidget "/Game/Widgets/HUD/HUDWorkbench/WBP_QTECut.WBP_QTECut_C" 0 _refworkbenchcutgrind))
        (bind _output_get (Variables|Default|SetQTECut _returnvalue))
        (UserInterface|Viewport|AddtoViewport _output_get 0)
        (EventDispatchers|BindEventtoProcessIngredient _output_get (EventDispatchers|CreateEvent :!event CallQTESucess))
        (EventDispatchers|BindEventtoFailQTE _output_get (EventDispatchers|CreateEvent :!event CallQTEFail))
        (return)))
    (:NewEnumerator1
      (if (Utilities|Enum|Equal(Enum) (LocalVariables|GetIngredientCategory) "NewEnumerator0")
        (Variables|Default|SetbQTEOn true)
        (Default|RemoveHUD (Variables|Default|GetAs%20BP%20Game%20Controller))
        (bind _returnvalue_2 (UserInterface|CreateWidget "/Game/Widgets/HUD/HUDWorkbench/WBP_QTEJoystick.WBP_QTEJoystick_C" 0 _refworkbenchcutgrind))
        (bind _output_get_2 (Variables|Default|SetQTEGrind _returnvalue_2))
        (UserInterface|Viewport|AddtoViewport _output_get_2 0)
        (EventDispatchers|BindEventtoProcessIngredient _output_get_2 (EventDispatchers|CreateEvent :!event CallQTESucess))
        (EventDispatchers|BindEventtoFailQTE _output_get_2 (EventDispatchers|CreateEvent :!event CallQTEFail))
        (return)))
    (:NewEnumerator2
      (Variables|Default|SetbQTEOn true)
      (Default|RemoveHUD (Variables|Default|GetAs%20BP%20Game%20Controller))
      (bind _returnvalue_3 (UserInterface|CreateWidget "/Game/Widgets/HUD/HUDWorkbench/WBP_QTEPotion.WBP_QTEPotion_C" 0 (Variables|Default|GetWorkbenchCauldron)))
      (bind _output_get_3 (Variables|Default|SetQTEPotion _returnvalue_3))
      (UserInterface|Viewport|AddtoViewport _output_get_3 0)
      (EventDispatchers|BindEventtoProcessPotion _output_get_3 (EventDispatchers|CreateEvent :!event CallQTESucess))
      (return))))

(fn BindUseItem
  (EventDispatchers|BindEventtoOnUseItem (Variables|/Game/Blueprints/Managers/BP_GameController.BP_GameController_C|GetBPC_Inventory (Variables|Default|GetAs%20BP%20Game%20Controller)) (EventDispatchers|CreateEvent :!event LaunchQTE)))

(fn UnbindUseItem
  (EventDispatchers|UnbindEventfromOnUseItem (Variables|/Game/Blueprints/Managers/BP_GameController.BP_GameController_C|GetBPC_Inventory (Variables|Default|GetAs%20BP%20Game%20Controller)) (EventDispatchers|CreateEvent :!event LaunchQTE)))

(fn CallQTESucess
  (Default|CallLaunchProcessMethod))

(fn CallQTEFail
  (Default|CallFailedMethod))