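; BP_GameController is the player controller that owns the player's inventory component and manages the HUD, inventory screen and workbench displays.
; On BeginPlay it creates the HUD outside menus, sizes the inventory from GameInstance save data and grants a one-time set of demo potions.
; Manual, automatic and workbench open events share one path that removes the default input mapping, hides the info HUD and stops movement.
; Closing restores the mapping and info HUD.
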(event Custom|AutomaticOpenInventory
  (bind _wb_playerhud (Variables|References|GetWB_PlayerHUD))
  (if (not (Variables|States|GetInventoryActive))
    (CallFunction|RemoveInput)
    (Default|CreatePlayerDisplay _wb_playerhud "NewEnumerator3")
    (Default|ChangeUX (Variables|/Game/Widgets/HUD/HUDPlayer/WBP_PlayerHUD.WBP_PlayerHUD_C|GetWB_PlayerDisplay _wb_playerhud) "NewEnumerator3")
    (Variables|States|SetInventoryActive true)
    (Widget|SetVisibility (Variables|References|GetWB_InfoHUD) "Hidden")
    (Audio|PlaySound2D "/Game/SoundEffect/UI/S_OpenInventory_Cue.S_OpenInventory_Cue" 1.0 1.0 0.0 0 0)
    (bind _as_bp_player (Variables|References|GetAs%20BP%20Player)
      (:then
        (Default|StopPlayerMovement _as_bp_player)
        (Default|StopLoopWalk (Variables|References|GetAs%20BP%20Player)))
      (:else))))

(event Custom|CreateHUDPlayer
  (bind _as_bp_game_instance (Variables|References|GetAs%20BP%20Game%20Instance))
  (if (not (Variables|/Game/Blueprints/Managers/BP_GameInstance.BP_GameInstance_C|GetbIsOnMenu _as_bp_game_instance))
    (bind _returnvalue (UserInterface|CreateWidget "/Game/Widgets/HUD/HUDPlayer/WBP_HUDinfo.WBP_HUDinfo_C" 0 _as_bp_game_instance))
    (bind _output_get (Variables|References|SetWB_InfoHUD _returnvalue))
    (Default|SetNightText _output_get)
    (UserInterface|Viewport|AddtoViewport _output_get 0)
    (bind _returnvalue_2 (UserInterface|CreateWidget "/Game/Widgets/HUD/HUDPlayer/WBP_PlayerHUD.WBP_PlayerHUD_C" 0 self))
    (bind _output_get_2 (Variables|References|SetWB_PlayerHUD _returnvalue_2))
    (UserInterface|Viewport|AddtoViewport _output_get_2 0)
    (Input|SetInputModeGameandUI self _output_get_2 "DoNotLock" true false)))

(event Custom|RemoveHUDTest
  (Variables|Default|SetbShowMouseCursor false)
  (Variables|States|SetInventoryActive false)
  (CallFunction|RemoveHUD)
  (Widget|SetVisibility (Variables|References|GetWB_InfoHUD) "Visible")
  (Audio|PlaySound2D "/Game/SoundEffect/UI/S_ShutInventory_Cue.S_ShutInventory_Cue" 1.0 1.0 0.0 0 0))

(event Custom|AutomaticHUDWorkbench
  (params (Method :type EProcessingMethod%20Enum :default "NewEnumerator0") (CupBoard :type BP%20Cupboard%20Object%20Reference))
  (bind _output_get (Variables|Default|SetMethod Method))
  (if (not (Variables|States|GetInventoryActive))
    (CallFunction|RemoveInput)
    (Default|CreatePlayerDisplay (Variables|References|GetWB_PlayerHUD) _output_get CupBoard)
    (Variables|States|SetInventoryActive true)
    (Widget|SetVisibility (Variables|References|GetWB_InfoHUD) "Hidden")
    (Audio|PlaySound2D "/Game/SoundEffect/UI/S_OpenInventory_Cue.S_OpenInventory_Cue" 1.0 1.0 0.0 0 0)
    (bind _as_bp_player (Variables|References|GetAs%20BP%20Player)
      (:then
        (Default|StopPlayerMovement _as_bp_player)
        (Default|StopLoopWalk (Variables|References|GetAs%20BP%20Player)))
      (:else))))

(event Custom|OpenInventory
  (bind _wb_playerhud (Variables|References|GetWB_PlayerHUD))
  (if (not (Variables|States|GetIsOnWorkbench))
    (if (not (Variables|States|GetInventoryActive))
      (Variables|States|SetInventoryManuallyOpen true)
      (Variables|Default|SetMethod "NewEnumerator3")
      (CallFunction|RemoveInput)
      (Default|CreatePlayerDisplay _wb_playerhud "NewEnumerator3")
      (Default|ChangeUX (Variables|/Game/Widgets/HUD/HUDPlayer/WBP_PlayerHUD.WBP_PlayerHUD_C|GetWB_PlayerDisplay _wb_playerhud) "NewEnumerator3")
      (Variables|States|SetInventoryActive true)
      (Widget|SetVisibility (Variables|References|GetWB_InfoHUD) "Hidden")
      (Audio|PlaySound2D "/Game/SoundEffect/UI/S_OpenInventory_Cue.S_OpenInventory_Cue" 1.0 1.0 0.0 0 0)
      (bind _as_bp_player (Variables|References|GetAs%20BP%20Player)
        (:then
          (Default|StopPlayerMovement _as_bp_player)
          (Default|StopLoopWalk (Variables|References|GetAs%20BP%20Player)))
        (:else)))))

(event Input|EnhancedActionEvents|EnhancedInputActionIA_EscapeWorkbench
  (params (ActionValue :type Boolean) (ElapsedSeconds :type Float%20%28double-precision%29) (TriggeredSeconds :type Float%20%28double-precision%29) (InputAction :type Input%20Action%20Object%20Reference :default "/Game/FirstPerson/Input/Actions/IA_EscapeWorkbench.IA_EscapeWorkbench"))
  (:Started
    (if (Variables|States|GetInventoryActive)
      (if (not (Variables|States|GetIsOnWorkbench))
        (Variables|Default|SetbShowMouseCursor false)
        (Variables|States|SetInventoryActive false)
        (CallFunction|RemoveHUD)
        (Widget|SetVisibility (Variables|References|GetWB_InfoHUD) "Visible")
        (Audio|PlaySound2D "/Game/SoundEffect/UI/S_ShutInventory_Cue.S_ShutInventory_Cue" 1.0 1.0 0.0 0 0)))))

(event EventBeginPlay
  (bind _asbp_game_instance (Utilities|Casting|CastToBP_GameInstance (Game|GetGameInstance)))
  (Variables|References|SetAs%20BP%20Game%20Instance _asbp_game_instance)
  (CallFunction|CreateHUDPlayer)
  (bind _asbp_player (Utilities|Casting|CastToBP_Player (Game|Player|GetPlayerPawn 0)))
  (Variables|References|SetAs%20BP%20Player _asbp_player)
  (Variables|/Game/Blueprints/Components/BPC_Inventory.BPC_Inventory_C|SetInventoryType (Variables|Default|GetBPC_Inventory) "NewEnumerator0")
  (Utilities|FlowControl|Delay 0.1)
  (Default|ResizeInventory (Variables|Default|GetBPC_Inventory) (Variables|/Game/Blueprints/Managers/BP_GameInstance.BP_GameInstance_C|GetInventorySlotsSave (Variables|References|GetAs%20BP%20Game%20Instance)))
  (if (not (Variables|/Game/Blueprints/Managers/BP_GameInstance.BP_GameInstance_C|GetDemoItemOnce (Variables|References|GetAs%20BP%20Game%20Instance)))
    (Default|Pickup (Variables|Default|GetBPC_Inventory) "Cough_Potion" 1 (Variables|/Game/Blueprints/Managers/BP_GameInstance.BP_GameInstance_C|GetInventorySlotsSave (Variables|References|GetAs%20BP%20Game%20Instance)))
    (Default|Pickup (Variables|Default|GetBPC_Inventory) "Pest_Control_Potion" 1 (Variables|/Game/Blueprints/Managers/BP_GameInstance.BP_GameInstance_C|GetInventorySlotsSave (Variables|References|GetAs%20BP%20Game%20Instance)))
    (Default|Pickup (Variables|Default|GetBPC_Inventory) "Enlargement_Potion" 1 (Variables|/Game/Blueprints/Managers/BP_GameInstance.BP_GameInstance_C|GetInventorySlotsSave (Variables|References|GetAs%20BP%20Game%20Instance)))
    (Default|Pickup (Variables|Default|GetBPC_Inventory) "Dancing_Potion" 1 (Variables|/Game/Blueprints/Managers/BP_GameInstance.BP_GameInstance_C|GetInventorySlotsSave (Variables|References|GetAs%20BP%20Game%20Instance)))
    (Default|Pickup (Variables|Default|GetBPC_Inventory) "Unlock_Potion" 1 (Variables|/Game/Blueprints/Managers/BP_GameInstance.BP_GameInstance_C|GetInventorySlotsSave (Variables|References|GetAs%20BP%20Game%20Instance)))
    (Default|Pickup (Variables|Default|GetBPC_Inventory) "Potion_Of_Shame" 1 (Variables|/Game/Blueprints/Managers/BP_GameInstance.BP_GameInstance_C|GetInventorySlotsSave (Variables|References|GetAs%20BP%20Game%20Instance)))
    (Variables|/Game/Blueprints/Managers/BP_GameInstance.BP_GameInstance_C|SetDemoItemOnce (Variables|References|GetAs%20BP%20Game%20Instance) true)))

(fn ConstructionScript)

(fn GetPositionCam
  (params (Cam%20Pos :type Vector))
  (Variables|Default|SetCamPosWorkbench_Grind Cam%20Pos)
  (return))

(fn RemoveHUD
  (Variables|States|SetInventoryActive false)
  (Variables|/Game/Blueprints/Components/BPC_Inventory.BPC_Inventory_C|SetNeedObject? (Variables|Default|GetBPC_Inventory) false)
  (bind _wb_playerdisplay (Variables|/Game/Widgets/HUD/HUDPlayer/WBP_PlayerHUD.WBP_PlayerHUD_C|GetWB_PlayerDisplay (Variables|References|GetWB_PlayerHUD))
    (:then
      (Default|RemoveHUD _wb_playerdisplay)
      (Input|AddMappingContext (PlayerController|LocalPlayerSubsystems|GetEnhancedInputLocalPlayerSubsystem self) "/Game/FirstPerson/Input/IMC_Default.IMC_Default" 0 "(bIgnoreAllPressedKeysUntilRelease=True,bForceImmediately=False,bNotifyUserSettings=False)"))
    (:else)))

(fn RemoveInput
  (Input|RemoveMappingContext (PlayerController|LocalPlayerSubsystems|GetEnhancedInputLocalPlayerSubsystem self) "/Game/FirstPerson/Input/IMC_Default.IMC_Default" "(bIgnoreAllPressedKeysUntilRelease=True,bForceImmediately=False,bNotifyUserSettings=False)"))