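; Player controller that creates the player HUD and opens the inventory display on it.
; On BeginPlay it creates a WBP_PlayerHUD widget, stores the reference and adds it to the viewport.
; The IA_Inventory input and the AutomaticOpenInventory event both call CreatePlayerDisplay on that HUD.
; An IsOnWorkbench check that would guard this call is left disconnected, so it never runs.
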(event Custom|AutomaticOpenInventory
  (Default|CreatePlayerDisplay (Variables|Default|GetWB_PlayerHUD)))

(event Custom|CreateHUDPlayer
  (bind _returnvalue (UserInterface|CreateWidget "/Game/Widgets/HUD/HUDPlayer/WBP_PlayerHUD.WBP_PlayerHUD_C"))
  (bind _output_get (Variables|Default|SetWB_PlayerHUD _returnvalue))
  (UserInterface|Viewport|AddtoViewport _output_get 0))

(event Input|EnhancedActionEvents|EnhancedInputActionIA_Inventory
  (params (ActionValue :type Boolean) (ElapsedSeconds :type Float%20%28double-precision%29) (TriggeredSeconds :type Float%20%28double-precision%29) (InputAction :type Input%20Action%20Object%20Reference :default "/Game/FirstPerson/Input/Actions/IA_Inventory.IA_Inventory"))
  (:Started
    (Default|CreatePlayerDisplay (Variables|Default|GetWB_PlayerHUD))))

(event EventBeginPlay
  (CallFunction|CreateHUDPlayer))

(fn ConstructionScript)