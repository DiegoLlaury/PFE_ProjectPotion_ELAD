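; Test grimoire pawn that the player possesses on interaction to flip through ingredient pages, returning to the player pawn on escape.
; Four WBP_PagePatron widgets, refreshed from a sliding page-index array, have their render targets fed every tick into dynamic materials on left, center and right pages.
; A timeline swings the center page forward or backward, with gates controlling re-triggering and DT_PageIngredientData's row count capping forward turns.
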(event Custom|TurnLeft
  (bind _listindexpage (Variables|Default|GetListIndexPage))
  (bind _listindexpage_2 (Variables|Default|GetListIndexPage))
  (if (> (Utilities|Array|Get(acopy) (Variables|Default|GetListIndexPage)) 0)
    (for _index (range 1 3)
      (Utilities|Array|SetArrayElem _listindexpage (- _index 3) (- (Utilities|Array|Get(acopy) _listindexpage 3) _index)))
    (CallFunction|UpdatePage)
    (Utilities|FlowControl|Gate false :!label _label
      (:Exit
        (Utilities|FlowControl|Sequence
          (:then_0
            (goto _label Close))
          (:then_1
            (Utilities|FlowControl|Gate false) ; enters at Close
          )
          (:then_2
            (bind (_direction _alpha) (Timeline|PageTurn ReverseFromEnd)
              (:Update
                (Transformation|SetRelativeTransform (Variables|Default|GetSK_PageCenter) (Math|Transform|Lerp(Transform) (Transformation|GetRelativeTransform (Variables|Default|GetSK_PageRight)) (Transformation|GetRelativeTransform (Variables|Default|GetSK_PageLeft)) _alpha) false false)
                (Transformation|SetRelativeLocationAndRotation (Variables|Default|GetSK_PageCenter) (Math|Vector|Lerp(Vector) "0.000000,0.250000,0.000000" "0.000000,0.250000,0.000000" _alpha) (Math|Rotator|MakeRotator 9e+01 0.0 (Math|Float|Lerp 179.9999 3.6e+02 _alpha)) false false))
              (:Finished
                (Utilities|FlowControl|Sequence
                  (:then_0
                    (Utilities|FlowControl|Gate false) ; enters at Open
                  )
                  (:then_1
                    (goto _label Open))
                  (:then_2
                    (switch Utilities|FlowControl|Switch|SwitchonETimelineDirection _direction
                      (:Forward
                        (Utilities|Array|SetArrayElem _listindexpage_2 0 (Utilities|Array|Get(acopy) _listindexpage_2 2)))
                      (:Backward
                        (Utilities|Array|SetArrayElem _listindexpage_2 3 (Utilities|Array|Get(acopy) _listindexpage_2 1))))
                    (CallFunction|UpdatePage)))))))))))

(event Custom|TurnRight
  (bind _listindexpage (Variables|Default|GetListIndexPage))
  (bind _listindexpage_2 (Variables|Default|GetListIndexPage))
  (bind _outrownames (DataTable|GetDataTableRowNames "/Game/Data/Datatables/DT_PageIngredientData.DT_PageIngredientData"))
  (if (< (+ (Utilities|Array|Get(acopy) (Variables|Default|GetListIndexPage)) 3) (Utilities|Array|Length _outrownames))
    (for _index (range 1 3)
      (Utilities|Array|SetArrayElem _listindexpage _index (+ (Utilities|Array|Get(acopy) _listindexpage) _index)))
    (CallFunction|UpdatePage)
    (Utilities|FlowControl|Gate false :!label _label
      (:Exit
        (Utilities|FlowControl|Sequence
          (:then_0
            (goto _label Close))
          (:then_1
            (Utilities|FlowControl|Gate false) ; enters at Close
          )
          (:then_2
            (bind (_direction _alpha) (Timeline|PageTurn PlayFromStart)
              (:Update
                (Transformation|SetRelativeTransform (Variables|Default|GetSK_PageCenter) (Math|Transform|Lerp(Transform) (Transformation|GetRelativeTransform (Variables|Default|GetSK_PageRight)) (Transformation|GetRelativeTransform (Variables|Default|GetSK_PageLeft)) _alpha) false false)
                (Transformation|SetRelativeLocationAndRotation (Variables|Default|GetSK_PageCenter) (Math|Vector|Lerp(Vector) "0.000000,0.250000,0.000000" "0.000000,0.250000,0.000000" _alpha) (Math|Rotator|MakeRotator 9e+01 0.0 (Math|Float|Lerp 179.9999 3.6e+02 _alpha)) false false))
              (:Finished
                (Utilities|FlowControl|Sequence
                  (:then_0
                    (goto _label Open))
                  (:then_1
                    (Utilities|FlowControl|Gate false) ; enters at Open
                  )
                  (:then_2
                    (switch Utilities|FlowControl|Switch|SwitchonETimelineDirection _direction
                      (:Forward
                        (Utilities|Array|SetArrayElem _listindexpage_2 0 (Utilities|Array|Get(acopy) _listindexpage_2 2)))
                      (:Backward
                        (Utilities|Array|SetArrayElem _listindexpage_2 3 (Utilities|Array|Get(acopy) _listindexpage_2 1))))
                    (CallFunction|UpdatePage)))))))))))

(event Input|EnhancedActionEvents|EnhancedInputActionIA_ChangeGrindWorkbenc
  (params (ActionValue :type Boolean) (ElapsedSeconds :type Float%20%28double-precision%29) (TriggeredSeconds :type Float%20%28double-precision%29) (InputAction :type Input%20Action%20Object%20Reference :default "/Game/FirstPerson/Input/Actions/IA_ChangeGrindWorkbenc.IA_ChangeGrindWorkbenc"))
  (bind _listindexpage (Variables|Default|GetListIndexPage))
  (bind _listindexpage_2 (Variables|Default|GetListIndexPage))
  (:Started
    (bind _outrownames (DataTable|GetDataTableRowNames "/Game/Data/Datatables/DT_PageIngredientData.DT_PageIngredientData"))
    (if (< (+ (Utilities|Array|Get(acopy) (Variables|Default|GetListIndexPage)) 3) (Utilities|Array|Length _outrownames))
      (for _index (range 1 3)
        (Utilities|Array|SetArrayElem _listindexpage _index (+ (Utilities|Array|Get(acopy) _listindexpage) _index)))
      (CallFunction|UpdatePage)
      (Utilities|FlowControl|Gate false :!label _label
        (:Exit
          (Utilities|FlowControl|Sequence
            (:then_0
              (goto _label Close))
            (:then_1
              (Utilities|FlowControl|Gate false) ; enters at Close
            )
            (:then_2
              (bind (_direction _alpha) (Timeline|PageTurn PlayFromStart)
                (:Update
                  (Transformation|SetRelativeTransform (Variables|Default|GetSK_PageCenter) (Math|Transform|Lerp(Transform) (Transformation|GetRelativeTransform (Variables|Default|GetSK_PageRight)) (Transformation|GetRelativeTransform (Variables|Default|GetSK_PageLeft)) _alpha) false false)
                  (Transformation|SetRelativeLocationAndRotation (Variables|Default|GetSK_PageCenter) (Math|Vector|Lerp(Vector) "0.000000,0.250000,0.000000" "0.000000,0.250000,0.000000" _alpha) (Math|Rotator|MakeRotator 9e+01 0.0 (Math|Float|Lerp 179.9999 3.6e+02 _alpha)) false false))
                (:Finished
                  (Utilities|FlowControl|Sequence
                    (:then_0
                      (goto _label Open))
                    (:then_1
                      (Utilities|FlowControl|Gate false) ; enters at Open
                    )
                    (:then_2
                      (switch Utilities|FlowControl|Switch|SwitchonETimelineDirection _direction
                        (:Forward
                          (Utilities|Array|SetArrayElem _listindexpage_2 0 (Utilities|Array|Get(acopy) _listindexpage_2 2)))
                        (:Backward
                          (Utilities|Array|SetArrayElem _listindexpage_2 3 (Utilities|Array|Get(acopy) _listindexpage_2 1))))
                      (CallFunction|UpdatePage))))))))))))

(event Input|EnhancedActionEvents|EnhancedInputActionIA_ChangeCutWorkbench
  (params (ActionValue :type Boolean) (ElapsedSeconds :type Float%20%28double-precision%29) (TriggeredSeconds :type Float%20%28double-precision%29) (InputAction :type Input%20Action%20Object%20Reference :default "/Game/FirstPerson/Input/Actions/IA_ChangeCutWorkbench.IA_ChangeCutWorkbench"))
  (bind _listindexpage (Variables|Default|GetListIndexPage))
  (bind _listindexpage_2 (Variables|Default|GetListIndexPage))
  (:Started
    (if (> (Utilities|Array|Get(acopy) (Variables|Default|GetListIndexPage)) 0)
      (for _index (range 1 3)
        (Utilities|Array|SetArrayElem _listindexpage (- _index 3) (- (Utilities|Array|Get(acopy) _listindexpage 3) _index)))
      (CallFunction|UpdatePage)
      (Utilities|FlowControl|Gate false :!label _label
        (:Exit
          (Utilities|FlowControl|Sequence
            (:then_0
              (goto _label Close))
            (:then_1
              (Utilities|FlowControl|Gate false) ; enters at Close
            )
            (:then_2
              (bind (_direction _alpha) (Timeline|PageTurn ReverseFromEnd)
                (:Update
                  (Transformation|SetRelativeTransform (Variables|Default|GetSK_PageCenter) (Math|Transform|Lerp(Transform) (Transformation|GetRelativeTransform (Variables|Default|GetSK_PageRight)) (Transformation|GetRelativeTransform (Variables|Default|GetSK_PageLeft)) _alpha) false false)
                  (Transformation|SetRelativeLocationAndRotation (Variables|Default|GetSK_PageCenter) (Math|Vector|Lerp(Vector) "0.000000,0.250000,0.000000" "0.000000,0.250000,0.000000" _alpha) (Math|Rotator|MakeRotator 9e+01 0.0 (Math|Float|Lerp 179.9999 3.6e+02 _alpha)) false false))
                (:Finished
                  (Utilities|FlowControl|Sequence
                    (:then_0
                      (Utilities|FlowControl|Gate false) ; enters at Open
                    )
                    (:then_1
                      (goto _label Open))
                    (:then_2
                      (switch Utilities|FlowControl|Switch|SwitchonETimelineDirection _direction
                        (:Forward
                          (Utilities|Array|SetArrayElem _listindexpage_2 0 (Utilities|Array|Get(acopy) _listindexpage_2 2)))
                        (:Backward
                          (Utilities|Array|SetArrayElem _listindexpage_2 3 (Utilities|Array|Get(acopy) _listindexpage_2 1))))
                      (CallFunction|UpdatePage))))))))))))

(event Input|EnhancedActionEvents|EnhancedInputActionIA_EscapeWorkbench
  (params (ActionValue :type Boolean) (ElapsedSeconds :type Float%20%28double-precision%29) (TriggeredSeconds :type Float%20%28double-precision%29) (InputAction :type Input%20Action%20Object%20Reference :default "/Game/FirstPerson/Input/Actions/IA_EscapeWorkbench.IA_EscapeWorkbench"))
  (bind _as_bp_game_controller (Variables|Default|GetAs%20BP%20Game%20Controller))
  (:Started
    (Variables|/Game/Blueprints/Managers/BP_GameController.BP_GameController_C|SetIsOnWorkbench _as_bp_game_controller false)
    (Pawn|Possess _as_bp_game_controller (Variables|Default|GetAs%20BP%20Player))))

(event EventBeginPlay
  (bind _asbp_game_controller (Utilities|Casting|CastToBP_GameController (Game|GetPlayerController 0)))
  (Variables|Default|SetAs%20BP%20Game%20Controller _asbp_game_controller)
  (bind _asbp_player (Utilities|Casting|CastToBP_Player (Game|Player|GetPlayerPawn 0)))
  (Variables|Default|SetAs%20BP%20Player _asbp_player)
  (Utilities|FlowControl|Sequence
    (:then_0
      (bind _returnvalue (Rendering|Material|CreateDynamicMaterialInstance (Variables|Default|GetSK_PageCenter) 0 0 "None" :!class /Script/Engine.PrimitiveComponent))
      (Variables|Default|SetDIM_Center _returnvalue)
      (bind _returnvalue_2 (Rendering|Material|CreateDynamicMaterialInstance (Variables|Default|GetSK_PageLeft) 0 0 "None" :!class /Script/Engine.PrimitiveComponent))
      (Variables|Default|SetDIM_Left _returnvalue_2)
      (bind _returnvalue_3 (Rendering|Material|CreateDynamicMaterialInstance (Variables|Default|GetSK_PageRight) 0 0 "None" :!class /Script/Engine.PrimitiveComponent))
      (Variables|Default|SetDIMRight _returnvalue_3)
      (Variables|Default|SetListWidgetComponent (Utilities|Array|MakeArray (Variables|Default|GetLeft) (Variables|Default|GetMidRight) (Variables|Default|GetMidLeft) (Variables|Default|GetRight)))
      (CallFunction|UpdatePage))))

(event EventOnInteract
  (params (ItemSlots :type Array%20of%20S%20Item%20Slot%20Structures))
  (bind _as_bp_game_controller (Variables|Default|GetAs%20BP%20Game%20Controller))
  (Variables|/Game/Blueprints/Managers/BP_GameController.BP_GameController_C|SetIsOnWorkbench _as_bp_game_controller true)
  (Pawn|Possess _as_bp_game_controller self))

(event EventTick
  (params (DeltaSeconds :type Float%20%28single-precision%29))
  (Rendering|Material|SetTextureParameterValue (Variables|Default|GetDIM_Center) "TextFront" (Class|WidgetComponent|GetRenderTarget (Variables|Default|GetMidLeft)))
  (Rendering|Material|SetTextureParameterValue (Variables|Default|GetDIM_Center) "TextBack" (Class|WidgetComponent|GetRenderTarget (Variables|Default|GetMidRight)))
  (Rendering|Material|SetTextureParameterValue (Variables|Default|GetDIM_Left) "TextFront" (Class|WidgetComponent|GetRenderTarget (Variables|Default|GetLeft)))
  (Rendering|Material|SetTextureParameterValue (Variables|Default|GetDIMRight) "TextBack" (Class|WidgetComponent|GetRenderTarget (Variables|Default|GetRight))))

(fn ConstructionScript)

(fn UpdatePage
  (for (_array_element _array_index) (Variables|Default|GetListIndexPage)
    (CallFunction|CreateWidget _array_element)
    (UserInterface|SetWidget (Utilities|Array|Get(acopy) (Variables|Default|GetListWidgetComponent) _array_index) (Variables|Default|GetTempWidget))))

(fn CreateWidget
  (params (PageIndex :type Integer))
  (bind _returnvalue (UserInterface|CreateWidget "/Game/Widgets/HUD/HUDGrimoire/WBP_PagePatron.WBP_PagePatron_C"))
  (bind _output_get (Variables|Default|SetTempWidget _returnvalue))
  (Default|SetPageData _output_get PageIndex))

(fn FocusTarget
  (return ""))