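; BP_PaperTest is a placeholder test actor that shows two widget components as the front and back of a paper page mesh.
; On BeginPlay it creates a dynamic material instance on the PageSK component.
; Every Tick it feeds the render targets of WidgetFront and WidgetBack into that material's TextFront and TextBack texture parameters.
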(event EventBeginPlay
  (bind _returnvalue (Rendering|Material|CreateDynamicMaterialInstance (Variables|Default|GetPageSK) 0 0 "None" :!class /Script/Engine.PrimitiveComponent))
  (Variables|Default|SetDIM _returnvalue))

(event Collision|EventActorBeginOverlap
  (params (OtherActor :type Actor%20Object%20Reference)))

(event EventTick
  (params (DeltaSeconds :type Float%20%28single-precision%29))
  (Rendering|Material|SetTextureParameterValue (Variables|Default|GetDIM) "TextFront" (Class|WidgetComponent|GetRenderTarget (Variables|Default|GetWidgetFront)))
  (Rendering|Material|SetTextureParameterValue (Variables|Default|GetDIM) "TextBack" (Class|WidgetComponent|GetRenderTarget (Variables|Default|GetWidgetBack))))

(fn ConstructionScript)