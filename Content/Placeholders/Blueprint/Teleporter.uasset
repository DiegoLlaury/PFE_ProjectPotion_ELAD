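; Interactable teleporter placeholder that sends the player to another level.
; While targeted, it outlines its sphere and shows the HUD button, using a short timer and a Tick-updated value to clear both afterwards.
; Interacting plays a portal sound, disables player input and shows a loading screen.
; After a delay it flags NPC dialogue to repeat if unfinished in the game instance, then opens the configured level.
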(event Custom|OutlineDelay
  (if (< (Variables|Default|GetTimer) 0.0)
    (Rendering|Material|SetOverlayMaterial (Variables|Default|GetSphere) "/Game/Materials/MI_ObjectOutlineFalse.MI_ObjectOutlineFalse" :!class /Script/Engine.MeshComponent)
    (Default|ButtonDisappear (Variables|/Game/Blueprints/Managers/BP_GameController.BP_GameController_C|GetWB_InfoHUD (Variables|Default|GetAs%20BP%20Game%20Controller)))))

(event EventBeginPlay
  (bind _asbp_game_controller (Utilities|Casting|CastToBP_GameController (Game|GetPlayerController 0)))
  (Variables|Default|SetAs%20BP%20Game%20Controller _asbp_game_controller)
  (bind _asbp_game_instance (Utilities|Casting|CastToBP_GameInstance (Game|GetGameInstance)))
  (Variables|Default|SetAs%20BP%20Game%20Instance _asbp_game_instance))

(event Collision|EventActorBeginOverlap
  (params (OtherActor :type Actor%20Object%20Reference)))

(event EventTick
  (params (DeltaSeconds :type Float%20%28single-precision%29))
  (Variables|Default|SetDelta%20Seconds DeltaSeconds)
  (Variables|Default|SetTimer (* (Variables|Default|GetDelta%20Seconds) (- (Variables|Default|GetTimer) (Variables|Default|GetDelta%20Seconds)))))

(event EventUIInteract
  (Rendering|Material|SetOverlayMaterial (Variables|Default|GetSphere) "/Game/Materials/MI_ObjectOutline.MI_ObjectOutline" :!class /Script/Engine.MeshComponent)
  (Default|ButtonAppear (Variables|/Game/Blueprints/Managers/BP_GameController.BP_GameController_C|GetWB_InfoHUD (Variables|Default|GetAs%20BP%20Game%20Controller)))
  (Variables|Default|SetTimer 0.1)
  (Utilities|Time|SetTimerbyEvent (delegate Custom|OutlineDelay) 0.2))

(event EventOnInteract
  (params (ItemSlots :type Array%20of%20S%20Item%20Slot%20Structures) (PlayerRef :type BP%20Player%20Object%20Reference))
  (bind _as_bp_game_instance (Variables|Default|GetAs%20BP%20Game%20Instance))
  (bind _as_bp_game_controller (Variables|Default|GetAs%20BP%20Game%20Controller))
  (Audio|PlaySound2D "/Game/SoundEffect/Portal/S_Portal_Cue.S_Portal_Cue" 1.0 1.0 0.0 0 0)
  (bind _returnvalue (UserInterface|CreateWidget "/Game/Widgets/HUD/HUDPlayer/WBP_LoadingScreen.WBP_LoadingScreen_C" _as_bp_game_controller))
  (Input|DisableInput PlayerRef _as_bp_game_controller)
  (UserInterface|Viewport|AddtoViewport _returnvalue 0)
  (Utilities|FlowControl|Delay 2.0)
  (if (not (Variables|/Game/Blueprints/Managers/BP_GameInstance.BP_GameInstance_C|GetFinishNPCDialogue _as_bp_game_instance))
    (Variables|/Game/Blueprints/Managers/BP_GameInstance.BP_GameInstance_C|SetRepeatDialogue _as_bp_game_instance true))
  (Game|OpenLevel(byObjectReference) (Variables|Default|GetLevel)))

(fn ConstructionScript)

(fn FocusTarget
  (return ""))